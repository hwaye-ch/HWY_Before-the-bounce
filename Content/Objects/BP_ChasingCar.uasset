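; BP_ChasingCar is an AI car enemy that sits dark until an enabler activates it, then chases and kills the player.
; Activation shows headlights and Mikey mesh and disables static mesh collision, letting pawn sensing drive AIMoveTo.
; Reaching the target once triggers a camera blend, jumpscare sounds, red spotlight, player death and game over.
; Separate events delay-start engine and horn audio, reset the transform, and show cooldown-guarded dialogue on overlap.
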(event OnSeePawn(PawnSensing)
  (params (Pawn :type Pawn%20Object%20Reference))
  (if (Variables|Default|GetIsStartChasing)
    (Utilities|FlowControl|Sequence
      (:then_0
        (AI|AIMoveTo self "0, 0, 0" Pawn 2e+02 false
          (:OnSuccess
            (Utilities|FlowControl|DoOnce false
              (:Completed
                (Utilities|FlowControl|Sequence
                  (:then_0
                    (bind _asbp_car_camera (Utilities|Casting|CastToBP_CarCamera (Variables|/Script/Engine.ChildActorComponent|GetChildActor (Variables|Default|GetCamera))))
                    (bind _output_get (Variables|Default|SetAs%20BP%20Car%20Camera _asbp_car_camera))
                    (Default|InitializeLevelCamera _output_get (Variables|Default|GetPlayer%20Ref) 0.2)
                    (Audio|SpawnSound2D "/Game/Sounds/sfx_car-collision.sfx_car-collision" 2.0 1.0 0.0 0)
                    (Utilities|FlowControl|Delay 0.5)
                    (Audio|SpawnSound2D "/Game/Sounds/sfx_jumpscare2.sfx_jumpscare2" 2.0 1.0 0.0 0))
                  (:then_1
                    (Audio|Components|Audio|Stop (Variables|Default|GetCar%20Sound))
                    (Rendering|SetVisibility (Variables|Default|GetRed%20Spotlight) true false)
                    (Utilities|FlowControl|Delay 1.0)
                    (CallFunction|CreateRestartWidget))
                  (:then_2
                    (Audio|Components|Audio|Stop (Variables|Default|Getsfx_car-horn))
                    (Audio|Components|Audio|Stop (Variables|Default|GetCar%20Sound))
                    (Default|CallPlayerDead)))))))))))

(event OnComponentBeginOverlap(Sphere)
  (params (OverlappedComponent :type Primitive%20Component%20Object%20Reference) (OtherActor :type Actor%20Object%20Reference) (OtherComp :type Primitive%20Component%20Object%20Reference) (OtherBodyIndex :type Integer) (bFromSweep :type Boolean) (SweepResult :type Hit%20Result%20Structure%20%28by%20ref%29))
  (Utilities|Casting|CastToBP_FirstPersonCharacter OtherActor)
  (Variables|Default|GetIs%20Cooldown%20Dialogue%20of%20Car
    (:then)
    (:else
      (Variables|Default|SetIs%20Cooldown%20Dialogue%20of%20Car true)
      (bind _dialoguecomponent (Default|ConstructDialogue (Variables|Default|GetBP_DialogueComponent) "ch1_car" "/Game/Dialogue/Chapter1_Dialogue.Chapter1_Dialogue" true true))
      (Default|DisplayUpperDialogue _dialoguecomponent)
      (Utilities|FlowControl|Delay 1e+01)
      (Variables|Default|SetIs%20Cooldown%20Dialogue%20of%20Car false))))

(event Custom|Return%20Car%20to%20Original%20Location
  (Transformation|SetActorTransform self (Variables|Default|GetOriginal%20Location) false true))

(event Custom|Activate%20Car!
  (bind _output_get (Variables|Default|SetIsStartChasing true))
  (CallFunction|TurntheLight _output_get)
  (Rendering|SetVisibility (Variables|Default|GetMikeyMesh) true true)
  (Collision|SetCollisionEnabled (Variables|Default|GetStaticMesh) "NoCollision"))

(event Custom|Turn%20the%20Light
  (params (Light%20On? :type Boolean))
  (Rendering|SetVisibility (Variables|Default|GetLampu1) Light%20On? false)
  (Rendering|SetVisibility (Variables|Default|GetLampu2) Light%20On? false))

(event Custom|Start%20Chasing
  (Utilities|FlowControl|Delay 6.0)
  (Components|Activation|Activate (Variables|Default|GetCar%20Sound) false)
  (Components|Activation|Activate (Variables|Default|Getsfx_car-horn) false))

(event Custom|Create%20Restart%20Widget
  (Default|SetGameOver (Variables|Default|GetPlayer%20Ref) 6))

(event EventBeginPlay
  (bind _carstartenabler (Variables|Default|GetCarStartEnabler))
  (Utilities|IsValid _carstartenabler
    (:Is%20Valid
      (EventDispatchers|BindEventtoCarStartChasing _carstartenabler (delegate Custom|Activate%20Car!))
      (CallFunction|TurntheLight false)
      (bind _asbp_first_person_character (Utilities|Casting|CastToBP_FirstPersonCharacter (Game|GetPlayerCharacter 0)))
      (Variables|Default|SetPlayer%20Ref _asbp_first_person_character)
      (Rendering|SetVisibility (Variables|Default|GetMikeyMesh) false true)
      (Collision|SetCollisionEnabled (Variables|Default|GetStaticMesh) "QueryAndPhysics")
      (Variables|Default|SetOriginal%20Location (Transformation|GetActorTransform)))))

(fn ConstructionScript)