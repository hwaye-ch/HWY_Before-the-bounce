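; Component that shows a yes/no choice dialogue to the player and broadcasts the chosen option through ExecuteOption.
; ConstructChoiceDialogue stores the question and option texts and returns itself.
; ShowChoiceDialogue builds WBP_ChoiceDialogue from them, switches to UI-only input with a cursor and disables player movement and look.
; When an option is pressed, OptionListener removes the widget, restores game input and player control, and fires ExecuteOption.
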(event Custom|Show%20Choice%20Dialogue
  (params (Player%20Pref :type BP%20First%20Person%20Character%20Object%20Reference))
  (bind _returnvalue (Game|GetPlayerController 0))
  (Variables|Default|SetPlayer%20Ref Player%20Pref)
  (bind _returnvalue_2 (UserInterface|CreateWidget "/Game/Blueprints/Widgets/WBP_ChoiceDialogue.WBP_ChoiceDialogue_C" 0 (Variables|Default|GetQuestion%20Dialogue) (Variables|Default|GetYes%20Option%20Text) (Variables|Default|GetNo%20Option%20Text)))
  (Variables|Default|SetDialogue%20Widget _returnvalue_2)
  (EventDispatchers|BindEventtoOnOptionPressed (Variables|Default|GetDialogue%20Widget) (delegate Custom|Option%20Listener))
  (UserInterface|Viewport|AddtoViewport (Variables|Default|GetDialogue%20Widget) 0)
  (Input|SetInputModeUIOnly _returnvalue (Variables|Default|GetDialogue%20Widget) "DoNotLock" false)
  (Variables|/Script/Engine.PlayerController|SetbShowMouseCursor _returnvalue true)
  (Default|DisableMovementandLook (Variables|Default|GetPlayer%20Ref)))

(event Custom|Destroy%20Choice%20Dialogue
  (Utilities|IsValid (Variables|Default|GetDialogue%20Widget)
    (:Is%20Valid
      (Widget|RemovefromParent (Variables|Default|GetDialogue%20Widget)))))

(event Custom|Option%20Listener
  (params (ChosenOption :type E_ChoiceDialogue%20Enum :default "NewEnumerator0"))
  (bind _returnvalue (Game|GetPlayerController 0))
  (Utilities|FlowControl|Sequence
    (:then_0
      (CallFunction|DestroyChoiceDialogue)
      (Default|EnableLookandMovement (Variables|Default|GetPlayer%20Ref))
      (Input|SetInputModeGameOnly _returnvalue false)
      (Variables|/Script/Engine.PlayerController|SetbShowMouseCursor _returnvalue false)
      (Utilities|FlowControl|DelayUntilNextTick))
    (:then_1
      (Default|CallExecuteOption ChosenOption))))

(fn ConstructChoiceDialogue
  (params (Question%20Text :type Text) (Yes%20Option%20Text :type Text) (No%20Option%20Text :type Text))
  (Variables|Default|SetQuestion%20Dialogue Question%20Text)
  (Variables|Default|SetYes%20Option%20Text Yes%20Option%20Text)
  (Variables|Default|SetNo%20Option%20Text No%20Option%20Text)
  (return self))