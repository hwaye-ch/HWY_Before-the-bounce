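; Component that adds hold-to-complete progress to a long interaction, displayed through a WBP_ProgressBar widget.
; Start creates the widget if needed and runs a timer for the remaining hold time; Trigger updates the bar and broadcasts progress.
; A short retriggerable delay detects when triggers stop, then pauses the timer and stores held time so filling can resume.
; Update, cancel and one-time finish dispatchers notify listeners, and completion blocks further holds.
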(event Custom|Destroy%20Widget
  (bind _wbp_progressbar (Variables|Default|GetWBP%20ProgressBar))
  (Utilities|IsValid _wbp_progressbar
    (:Is%20Valid
      (Widget|RemovefromParent _wbp_progressbar))))

(event Custom|Start%20Timer
  (bind _returnvalue (Utilities|Time|SetTimerbyEvent (delegate Custom|Finish) (- (Variables|Default|GetMaxHoldTime) (Variables|Default|GetCurrentHoldTime)))))

(event Custom|Stop%20Progress
  (Utilities|Time|PauseTimerbyHandle (stale Custom|Start%20Timer _returnvalue))
  (Default|CallCancelProgressFilling))

(event Custom|Update%20Progress
  (Variables|/Game/Blueprints/Widgets/WBP_ProgressBar.WBP_ProgressBar_C|SetTimeHeld (Variables|Default|GetWBP%20ProgressBar) (+ (Class|KismetSystemLibrary|GetTimerElapsedTimeHandle (stale Custom|Start%20Timer _returnvalue)) (Variables|Default|GetCurrentHoldTime)))
  (bind _progresspercentage (CallFunction|ProgressPercentage))
  (Default|CallUpdateProgressFilling _progresspercentage))

(event Custom|Finish
  (Utilities|FlowControl|DoOnce false
    (:Completed
      (Development|PrintString "Finish Filling" true true "(R=1.000000,G=0.000000,B=0.051657,A=1.000000)")
      (Variables|Default|SetIs%20Progress%20Bar%20Completed true)
      (Default|CallFinishProgressFilling))))

(event EventOnLongInteract
  (params (State :type E_LongInteract%20Enum :default "NewEnumerator0"))
  (if (Variables|Default|GetIs%20Long%20Interact%20Active)
    (Development|PrintString (Utilities|String|EnumtoString State))
    (switch Utilities|FlowControl|Switch|SwitchonE_LongInteract State
      (:NewEnumerator0
        (if (Variables|Default|GetIsTriggeringHoldMechanism)
          (if (not (Variables|Default|GetIs%20Progress%20Bar%20Completed))
            (Variables|Default|SetIsTriggeringHoldMechanism true)
            (CallFunction|UpdateProgress)
            (Utilities|FlowControl|RetriggerableDelay 0.1)
            (Variables|Default|SetIsTriggeringHoldMechanism false)
            (CallFunction|StopProgress)
            (Variables|Default|SetCurrentHoldTime (Variables|/Game/Blueprints/Widgets/WBP_ProgressBar.WBP_ProgressBar_C|GetTimeHeld (Variables|Default|GetWBP%20ProgressBar))))
          (else
            (Utilities|IsValid (Variables|Default|GetWBP%20ProgressBar) :!label _label
              (:Is%20Valid
                _)
              (:Is%20Not%20Valid
                (bind _returnvalue (UserInterface|CreateWidget "/Game/Blueprints/Widgets/WBP_ProgressBar.WBP_ProgressBar_C"))
                (bind _output_get (Variables|Default|SetWBP%20ProgressBar _returnvalue))
                (UserInterface|Viewport|AddtoViewport _output_get 0)
                (Variables|/Game/Blueprints/Widgets/WBP_ProgressBar.WBP_ProgressBar_C|SetMaxTime _output_get (Variables|Default|GetMaxHoldTime))))
            (Variables|Default|SetIsTriggeringHoldMechanism true)
            (CallFunction|StartTimer))))
      (:NewEnumerator1
        (if (not (Variables|Default|GetIs%20Progress%20Bar%20Completed))
          (goto _label)))
      (:NewEnumerator2
        (if (not (Variables|Default|GetIs%20Progress%20Bar%20Completed))
          (Variables|Default|SetIsTriggeringHoldMechanism false))))))

(fn ProgressPercentage
  (return (/ (Variables|/Game/Blueprints/Widgets/WBP_ProgressBar.WBP_ProgressBar_C|GetTimeHeld (Variables|Default|GetWBP%20ProgressBar)) (Variables|Default|GetMaxHoldTime))))

(fn OnProgressFilling
  (return 0.0))