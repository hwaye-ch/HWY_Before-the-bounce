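; Dialogue component that shows localized, DataTable-driven conversations, picking each row's text by the game instance's language.
; ShowDialogue displays one row per call, optionally blocks player movement or look, and fires an event on actionable rows.
; DisplayAutoDialogue advances on a timer until an end row, while DisplayUpperDialogue shows a temporary separate widget with fewer languages.
; Rows chain through next-row and table fields, reusing one dialogue widget until clearing removes it and restores player control.
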(event Custom|Modify%20Movement
  (params (PlayerPref :type BP%20First%20Person%20Character%20Object%20Reference))
  (Utilities|IsValid PlayerPref
    (:Is%20Valid
      (bind _output_get (Variables|Default|SetPlayer%20Pref PlayerPref))
      (if (Variables|PlayerPref.|GetBlockMovement)
        (Default|DisableMovement _output_get))
      (if (Variables|PlayerPref.|GetBlockLook)
        (Default|DisableLook (Variables|Default|GetPlayer%20Pref))))))

(event Custom|Reset%20Movement
  (bind _player_pref (Variables|Default|GetPlayer%20Pref))
  (Utilities|IsValid _player_pref
    (:Is%20Valid
      (Default|EnableLookandMovement _player_pref))))

(event Custom|Display%20Upper%20Dialogue
  (bind _returnvalue (Utilities|GetDataTableRow (Variables|Dialogue|GetDialogueTable) (Variables|Dialogue|GetDialogueCode))
    (:then
      (bind _output_get (CallFunction|GetLanguage))
      (bind _returnvalue_2 (UserInterface|CreateWidget "/Game/Blueprints/Widgets/WBP_UpperDialogue.WBP_UpperDialogue_C" 0 (Utilities|Text|ToText(String) (Utilities|Select :Index _output_get :NewEnumerator0 (.Dialogue (Utilities|Struct|BreakDialogue_Structure _returnvalue)) :NewEnumerator1 (.JP (Utilities|Struct|BreakDialogue_Structure _returnvalue)) :NewEnumerator2 (.EN (Utilities|Struct|BreakDialogue_Structure _returnvalue)) :NewEnumerator3 (.KR (Utilities|Struct|BreakDialogue_Structure _returnvalue)) :NewEnumerator5 (.CH (Utilities|Struct|BreakDialogue_Structure _returnvalue)) :NewEnumerator7 (.DE (Utilities|Struct|BreakDialogue_Structure _returnvalue)) :NewEnumerator8 "" :NewEnumerator9 "" :NewEnumerator10 "" :NewEnumerator11 ""))))
      (UserInterface|Viewport|AddtoViewport _returnvalue_2 0)
      (Utilities|FlowControl|Delay 5.0)
      (Widget|RemovefromParent _returnvalue_2))
    (:RowNotFound
      (Development|PrintString "Wrong Dialogue Code"))))

(event Custom|End%20of%20Dialogue
  (Development|PrintString "End of dialogue"))

(event Custom|Fill%20In%20Dialogue
  (bind _dialoguewidget (Variables|Dialogue|GetDialogueWidget))
  (Utilities|IsValid _dialoguewidget
    (:Is%20Valid
      (Default|FillDialogueText _dialoguewidget))))

(event Custom|Dialogue%20is%20Filled
  (bind _player_pref (Variables|Default|GetPlayer%20Pref))
  (Utilities|IsValid _player_pref
    (:Is%20Valid
      (Variables|/Game/FirstPerson/Blueprints/BP_FirstPersonCharacter.BP_FirstPersonCharacter_C|SetIsDialogueTextComplete _player_pref true))))

(event Custom|Clear%20Dialogue
  (Utilities|IsValid (Variables|Dialogue|GetDialogueWidget)
    (:Is%20Valid
      (Widget|RemovefromParent (Variables|Dialogue|GetDialogueWidget))
      (bind _player_pref (Variables|Default|GetPlayer%20Pref)
        (:then
          (Variables|/Game/FirstPerson/Blueprints/BP_FirstPersonCharacter.BP_FirstPersonCharacter_C|SetDialogueWidget _player_pref 0))
        (:else
          _))
      (Variables|Dialogue|SetDialogueWidget 0))
    (:Is%20Not%20Valid
      _))
  (CallFunction|ResetMovement))

(event Custom|Binds%20Event
  (EventDispatchers|BindEventtoOnClearDialogue (delegate Custom|Clear%20Dialogue))
  (EventDispatchers|BindEventtoOnFillDialogue (delegate Custom|Fill%20In%20Dialogue))
  (EventDispatchers|BindEventtoOnDialogueEnded (delegate Custom|End%20of%20Dialogue)))

(event EventDisplayAutoDialogue
  (CallFunction|BindsEvent)
  (Utilities|FlowControl|Sequence
    (:then_0
      (Variables|Dialogue|SetDialogueTable (Variables|Dialogue|GetDialogueTable)))
    (:then_1
      (Utilities|IsValid (Variables|Dialogue|GetDialogueWidget)
        (:Is%20Valid
          (bind _returnvalue (Utilities|GetDataTableRow (Variables|Dialogue|GetDialogueTable) (Variables|Dialogue|GetDialogueCode))
            (:then
              (bind _output_get (CallFunction|GetLanguage))
              (Default|UpdateDialogue (Variables|Dialogue|GetDialogueWidget) (Utilities|Select :Index _output_get :NewEnumerator0 (.Dialogue (Utilities|Struct|BreakDialogue_Structure _returnvalue)) :NewEnumerator1 (.JP (Utilities|Struct|BreakDialogue_Structure _returnvalue)) :NewEnumerator2 (.EN (Utilities|Struct|BreakDialogue_Structure _returnvalue)) :NewEnumerator3 (.KR (Utilities|Struct|BreakDialogue_Structure _returnvalue)) :NewEnumerator5 (.CH (Utilities|Struct|BreakDialogue_Structure _returnvalue)) :NewEnumerator7 (.DE (Utilities|Struct|BreakDialogue_Structure _returnvalue)) :NewEnumerator8 (.TH (Utilities|Struct|BreakDialogue_Structure _returnvalue)) :NewEnumerator9 (.PH (Utilities|Struct|BreakDialogue_Structure _returnvalue)) :NewEnumerator10 (.PT (Utilities|Struct|BreakDialogue_Structure _returnvalue)) :NewEnumerator11 (.FR (Utilities|Struct|BreakDialogue_Structure _returnvalue))) self (.CharacterName (Utilities|Struct|BreakDialogue_Structure _returnvalue)) false)
              (Variables|Dialogue|SetDialogueCode (.NextRow (Utilities|Struct|BreakDialogue_Structure _returnvalue)))
              (Variables|Dialogue|SetDialogueTable (.Datatable (Utilities|Struct|BreakDialogue_Structure _returnvalue)))
              (Variables|Dialogue|SetIsDialogueEnded (.EndDialogue? (Utilities|Struct|BreakDialogue_Structure _returnvalue)))
              (Utilities|FlowControl|Delay (Variables|Default|GetDisplayDialogueDuration) :!label _label)
              (if (Variables|Dialogue|GetIsDialogueEnded)
                (Default|CallOnClearDialogue)
                (Default|CallOnDialogueEnded)
                (EventDispatchers|UnbindallEventsfromOnDialogueEnded)
                (else
                  (CallFunction|DisplayAutoDialogue))))
            (:RowNotFound
              (Development|PrintString "Wrong Dialogue Code" :!label _label_2))))
        (:Is%20Not%20Valid
          (bind _returnvalue_2 (Utilities|GetDataTableRow (Variables|Dialogue|GetDialogueTable) (Variables|Dialogue|GetDialogueCode))
            (:then
              (bind _output_get_2 (CallFunction|GetLanguage))
              (bind _returnvalue_3 (UserInterface|CreateWidget "/Game/Blueprints/Widgets/WBP_Dialogue.WBP_Dialogue_C" 0 "" (Utilities|Select :Index _output_get_2 :NewEnumerator0 (.Dialogue (Utilities|Struct|BreakDialogue_Structure _returnvalue_2)) :NewEnumerator1 (.JP (Utilities|Struct|BreakDialogue_Structure _returnvalue_2)) :NewEnumerator2 (.EN (Utilities|Struct|BreakDialogue_Structure _returnvalue_2)) :NewEnumerator3 (.KR (Utilities|Struct|BreakDialogue_Structure _returnvalue_2)) :NewEnumerator5 (.CH (Utilities|Struct|BreakDialogue_Structure _returnvalue_2)) :NewEnumerator7 (.DE (Utilities|Struct|BreakDialogue_Structure _returnvalue_2)) :NewEnumerator8 (.TH (Utilities|Struct|BreakDialogue_Structure _returnvalue_2)) :NewEnumerator9 (.PH (Utilities|Struct|BreakDialogue_Structure _returnvalue_2)) :NewEnumerator10 (.PT (Utilities|Struct|BreakDialogue_Structure _returnvalue_2)) :NewEnumerator11 (.FR (Utilities|Struct|BreakDialogue_Structure _returnvalue_2))) self))
              (UserInterface|Viewport|AddtoViewport _returnvalue_3 0)
              (Variables|Dialogue|SetDialogueWidget _returnvalue_3)
              (Variables|Dialogue|SetDialogueCode (.NextRow (Utilities|Struct|BreakDialogue_Structure _returnvalue_2)))
              (Variables|Dialogue|SetDialogueTable (.Datatable (Utilities|Struct|BreakDialogue_Structure _returnvalue_2)))
              (Variables|Dialogue|SetIsDialogueEnded (.EndDialogue? (Utilities|Struct|BreakDialogue_Structure _returnvalue_2)))
              (goto _label))
            (:RowNotFound
              (goto _label_2))))))))

(fn ConstructDialogue
  (params (DialogueCode :type Name) (DialogueTable :type Data%20Table%20Object%20Reference) (BlockMovement :type Boolean) (BlockLook :type Boolean))
  (Variables|Dialogue|SetDialogueCode DialogueCode)
  (Variables|Dialogue|SetDialogueTable DialogueTable)
  (Variables|PlayerPref.|SetBlockMovement BlockMovement)
  (Variables|PlayerPref.|SetBlockLook BlockLook)
  (return self))

(fn GetLanguage
  (bind _ashwy_game_instance (Utilities|Casting|CastToHwyGameInstance (Game|GetGameInstance)))
  (bind _language (Default|GetLanguage _ashwy_game_instance))
  (return _language))

(fn ShowDialogue
  (params (PlayerPref :type BP%20First%20Person%20Character%20Object%20Reference) (DialogueActorTrigger :type Actor%20Object%20Reference))
  (CallFunction|BindsEvent)
  (if (!= (Variables|Dialogue|GetDialogueCode) "")
    (Variables|Default|SetPlayer%20Pref PlayerPref)
    (Utilities|FlowControl|Sequence
      (:then_0
        (CallFunction|ModifyMovement (Variables|Default|GetPlayer%20Pref))
        (Variables|Dialogue|SetDialogueTable (Variables|Dialogue|GetDialogueTable))
        (Variables|/Game/FirstPerson/Blueprints/BP_FirstPersonCharacter.BP_FirstPersonCharacter_C|SetIsDialogueTextComplete (Variables|Default|GetPlayer%20Pref) false)
        (Variables|/Game/FirstPerson/Blueprints/BP_FirstPersonCharacter.BP_FirstPersonCharacter_C|SetIsTriggeringDialogue (Variables|Default|GetPlayer%20Pref) true)
        (Variables|Default|SetDialogueActorTrigger DialogueActorTrigger)
        (Variables|Dialogue|SetDialogueWidget (Variables|/Game/FirstPerson/Blueprints/BP_FirstPersonCharacter.BP_FirstPersonCharacter_C|GetDialogueWidget (Variables|Default|GetPlayer%20Pref))))
      (:then_1
        (Utilities|IsValid (Variables|Dialogue|GetDialogueWidget)
          (:Is%20Valid
            (bind _returnvalue (Utilities|GetDataTableRow (Variables|Dialogue|GetDialogueTable) (Variables|Dialogue|GetDialogueCode))
              (:then
                (bind _output_get (CallFunction|GetLanguage))
                (Default|UpdateDialogue (Variables|Dialogue|GetDialogueWidget) (Utilities|Select :Index _output_get :NewEnumerator0 (.Dialogue (Utilities|Struct|BreakDialogue_Structure _returnvalue)) :NewEnumerator1 (.JP (Utilities|Struct|BreakDialogue_Structure _returnvalue)) :NewEnumerator2 (.EN (Utilities|Struct|BreakDialogue_Structure _returnvalue)) :NewEnumerator3 (.KR (Utilities|Struct|BreakDialogue_Structure _returnvalue)) :NewEnumerator5 (.CH (Utilities|Struct|BreakDialogue_Structure _returnvalue)) :NewEnumerator7 (.DE (Utilities|Struct|BreakDialogue_Structure _returnvalue)) :NewEnumerator8 (.TH (Utilities|Struct|BreakDialogue_Structure _returnvalue)) :NewEnumerator9 (.PH (Utilities|Struct|BreakDialogue_Structure _returnvalue)) :NewEnumerator10 (.PT (Utilities|Struct|BreakDialogue_Structure _returnvalue)) :NewEnumerator11 (.FR (Utilities|Struct|BreakDialogue_Structure _returnvalue))) self (.CharacterName (Utilities|Struct|BreakDialogue_Structure _returnvalue)) true)
                (Variables|/Game/FirstPerson/Blueprints/BP_FirstPersonCharacter.BP_FirstPersonCharacter_C|SetIsDialogueEnded (Variables|Default|GetPlayer%20Pref) (.EndDialogue? (Utilities|Struct|BreakDialogue_Structure _returnvalue)))
                (Variables|Dialogue|SetDialogueCode (.NextRow (Utilities|Struct|BreakDialogue_Structure _returnvalue)))
                (Variables|Dialogue|SetActor%20Name (.CharacterName (Utilities|Struct|BreakDialogue_Structure _returnvalue)))
                (Variables|Dialogue|SetDialogueTable (.Datatable (Utilities|Struct|BreakDialogue_Structure _returnvalue)))
                (Variables|/Game/FirstPerson/Blueprints/BP_FirstPersonCharacter.BP_FirstPersonCharacter_C|SetDialogueComponent (Variables|Default|GetPlayer%20Pref) self)
                (if (.Actionable? (Utilities|Struct|BreakDialogue_Structure _returnvalue))
                  (Default|CallOnActionDuringDialogue :!label _label))
                (return))
              (:RowNotFound
                _)))
          (:Is%20Not%20Valid
            (bind _returnvalue_2 (Utilities|GetDataTableRow (Variables|Dialogue|GetDialogueTable) (Variables|Dialogue|GetDialogueCode))
              (:then
                (bind _output_get_2 (CallFunction|GetLanguage))
                (bind _returnvalue_3 (UserInterface|CreateWidget "/Game/Blueprints/Widgets/WBP_Dialogue.WBP_Dialogue_C" 0 (.CharacterName (Utilities|Struct|BreakDialogue_Structure _returnvalue_2)) (Utilities|Select :Index _output_get_2 :NewEnumerator0 (.Dialogue (Utilities|Struct|BreakDialogue_Structure _returnvalue_2)) :NewEnumerator1 (.JP (Utilities|Struct|BreakDialogue_Structure _returnvalue_2)) :NewEnumerator2 (.EN (Utilities|Struct|BreakDialogue_Structure _returnvalue_2)) :NewEnumerator3 (.KR (Utilities|Struct|BreakDialogue_Structure _returnvalue_2)) :NewEnumerator5 (.CH (Utilities|Struct|BreakDialogue_Structure _returnvalue_2)) :NewEnumerator7 (.DE (Utilities|Struct|BreakDialogue_Structure _returnvalue_2)) :NewEnumerator8 (.TH (Utilities|Struct|BreakDialogue_Structure _returnvalue_2)) :NewEnumerator9 (.PH (Utilities|Struct|BreakDialogue_Structure _returnvalue_2)) :NewEnumerator10 (.PT (Utilities|Struct|BreakDialogue_Structure _returnvalue_2)) :NewEnumerator11 (.FR (Utilities|Struct|BreakDialogue_Structure _returnvalue_2))) self true))
                (UserInterface|Viewport|AddtoViewport _returnvalue_3 0)
                (bind _output_get_3 (Variables|/Game/FirstPerson/Blueprints/BP_FirstPersonCharacter.BP_FirstPersonCharacter_C|SetDialogueWidget (Variables|Default|GetPlayer%20Pref) _returnvalue_3))
                (Variables|Dialogue|SetDialogueWidget _output_get_3)
                (Variables|Dialogue|SetActor%20Name (.CharacterName (Utilities|Struct|BreakDialogue_Structure _returnvalue_2)))
                (Variables|Dialogue|SetDialogueCode (.NextRow (Utilities|Struct|BreakDialogue_Structure _returnvalue_2)))
                (Variables|Dialogue|SetDialogueTable (.Datatable (Utilities|Struct|BreakDialogue_Structure _returnvalue_2)))
                (Variables|/Game/FirstPerson/Blueprints/BP_FirstPersonCharacter.BP_FirstPersonCharacter_C|SetDialogueComponent (Variables|Default|GetPlayer%20Pref) self)
                (Variables|/Game/FirstPerson/Blueprints/BP_FirstPersonCharacter.BP_FirstPersonCharacter_C|SetIsDialogueEnded (Variables|Default|GetPlayer%20Pref) (.EndDialogue? (Utilities|Struct|BreakDialogue_Structure _returnvalue_2)))
                (if (.Actionable? (Utilities|Struct|BreakDialogue_Structure _returnvalue_2))
                  (goto _label)
                  (else
                    (return))))
              (:RowNotFound
                _))))
        (Development|PrintString "Wrong Dialogue Code")))
    (else
      (Development|PrintString "Empty Dialogue Code"))))