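; BP_Chapter1Manager is a child chapter manager that sets up and cleans up Chapter 1.
; InitializeLevel1 binds the chapter-finished event, fades in, starts night ambience and house chatter, shows the frozen food and sets up Mikey's chapter events.
; When the chapter finishes, it stops the house talking sounds.
; StartGame only casts the player character; the InitializeLevel1 call and CurrentChapter assignment are left unwired.
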(event Custom|Initialize%20Level%201
  (EventDispatchers|BindEventtoOnChapterFinished (delegate Custom|On%20Chapter%20Finished_Event))
  (Default|Fadein (Variables|Default|GetBP_FadeScreenComponent) (Variables|Default|GetPlayer%20Ref))
  (Utilities|FlowControl|Sequence
    (:then_0
      (bind _returnvalue (Actor|GetActorOfClass "/Game/Blueprints/Levels/BP_AmbienceSound.BP_AmbienceSound_C"))
      (bind _output_get (Variables|Default|SetAmbience _returnvalue))
      (Default|SpawnNightAmbience _output_get 0.01))
    (:then_1
      (bind _outactors (Actor|GetAllActorsOfClass "/Game/Blueprints/EventItems/BP_HouseTalking.BP_HouseTalking_C"))
      (for _array_element _outactors
        (Default|PlayPeopleTalking _array_element true)))
    (:then_2
      (bind _frozen_food (Variables|Default|GetFrozen%20Food)
        (:then
          (Default|ShowItem _frozen_food))
        (:else)))
    (:then_3
      (bind _mikey (Variables|Default|GetMikey)
        (:then
          (Default|SetupEventforChapter1 _mikey))
        (:else)))))

(event Custom|On%20Chapter%20Finished_Event
  (bind _outactors (Actor|GetAllActorsOfClass "/Game/Blueprints/EventItems/BP_HouseTalking.BP_HouseTalking_C"))
  (for _array_element _outactors
    (bind _sound (Variables|/Game/Blueprints/EventItems/BP_HouseTalking.BP_HouseTalking_C|GetSound _array_element)
      (:then
        (Audio|Components|Audio|Stop _sound))
      (:else))))

(event Custom|Start%20Game
  (Utilities|Casting|CastToBP_FirstPersonCharacter (Game|GetPlayerCharacter 0)))

(event EventBeginPlay
  ;[0.15 0.15 0.15 0.5] Debug
  (|CallParentFunction))

(fn ConstructionScript
  (|CallParentFunction))