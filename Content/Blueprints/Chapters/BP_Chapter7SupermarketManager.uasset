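; Chapter manager that sets up and exits the Chapter 7 supermarket segment.
; Initialization fades in from black, teleports the player to the cashier spawn, unlocks the front door and sets the shop barrier's collision.
; After a short delay it starts the CaseOh customer sequence if that reference is valid.
; TeleporttoTaman fades the screen out, then has the game instance change maps when the fade finishes.
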(event Custom|Teleport%20to%20Taman
  (bind _bp_fadescreencomponent (Variables|Default|GetBP_FadeScreenComponent))
  (Default|FadeOut _bp_fadescreencomponent 1e+01 (Variables|Default|GetPlayer%20Ref))
  (EventDispatchers|BindEventtoOnExactFinish _bp_fadescreencomponent (delegate Custom|OnFadeOut_Event)))

(event Custom|OnFadeOut_Event
  (Default|CallTeleporttoMap (Variables|Default|GetGame%20Instance%20Ref) "NewEnumerator0"))

(event Custom|Initialize%20Chapter%207%20Supermarket
  (bind _player_ref (Variables|Default|GetPlayer%20Ref))
  (Utilities|FlowControl|Sequence
    (:then_0
      (Default|BlackScreenThenFadein (Variables|Default|GetBP_FadeScreenComponent) (Variables|Default|GetPlayer%20Ref) 3.0)
      (bind _returnvalue (Actor|GetActorOfClass "/Game/Blueprints/Levels/SpawnArea_Kasir.SpawnArea_Kasir_C"))
      (Transformation|SetActorTransform _player_ref (Math|Transform|MakeTransform (.location (Transformation|GetActorTransform _returnvalue)) (.rotation (Transformation|GetActorTransform _returnvalue)) (Transformation|GetActorScale3D _player_ref)) false true))
    (:then_1
      (bind _returnvalue_2 (Actor|GetActorOfClass "/Game/Convenience_Store/Blueprints/BP_Front_Door.BP_Front_Door_C"))
      (Variables|/Game/Convenience_Store/Blueprints/BP_Front_Door.BP_Front_Door_C|SetIsLocked _returnvalue_2 false)
      (bind _returnvalue_3 (Actor|GetActorOfClass "/Game/Blueprints/Levels/Barrier_Shop.Barrier_Shop_C"))
      (Default|SetCollisionSetting _returnvalue_3 true))
    (:then_2
      (Utilities|FlowControl|Delay 1e+01)
      (bind _customer_case_oh (Variables|Default|GetCustomer%20Case%20Oh)
        (:then
          (Default|StartSequenceCustomerCaseOh _customer_case_oh))
        (:else)))))

(fn ConstructionScript
  (|CallParentFunction))