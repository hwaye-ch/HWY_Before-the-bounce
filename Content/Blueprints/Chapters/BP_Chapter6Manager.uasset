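; Chapter 6 manager that sets up the level state when InitializeChapter6 is called.
; It teleports the player to the spawn area facing a look target, plays the bus area event, and binds the endless bus's next event to run the bus and set ambience volume.
; It also removes the forbidden collider, activates the story overlap triggers, hides Mikey's mesh and reveals the guarding Mom.
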(event Custom|Initialize%20Chapter%206
  (Utilities|FlowControl|Sequence
    (:then_0
      ;[0.15 0.15 0.15 0.5] Spawn Area
      (bind _spawn_area (Variables|Default|GetSpawn%20Area)
        (:then
          (Transformation|SetActorLocation (Variables|Default|GetPlayer%20Ref) (Transformation|GetActorLocation _spawn_area) false true)
          (bind _look_area (Variables|Default|GetLook%20Area)
            (:then
              (Pawn|SetControlRotation (Game|GetPlayerController 0) (Math|Rotator|FindLookatRotation (Transformation|GetActorLocation (Variables|Default|GetPlayer%20Ref)) (Transformation|GetActorLocation _look_area))))
            (:else)))
        (:else)))
    (:then_1
      ;[0.15 0.15 0.15 0.5] Bus Event
      (bind _area_bus_event (Variables|Default|GetArea%20Bus%20Event)
        (:then
          (Default|PlayEvent _area_bus_event)
          (bind _bus_endless (Variables|Default|GetBus%20Endless)
            (:then
              (EventDispatchers|BindEventtoExecuteNextEvent _bus_endless (delegate Custom|Play%20Sequence%20Level%20on%20Bus)))
            (:else)))
        (:else)))
    (:then_2
      ;[0.15 0.15 0.15 0.5] Activate Triggers
      (bind _collider_forbidden (Variables|Default|GetCollider%20Forbidden)
        (:then
          (Actor|DestroyActor _collider_forbidden)
          (bind _trigger_car_crash (Variables|Default|GetTrigger%20Car%20Crash)
            (:then
              (bind _trigger_intro (Variables|Default|GetTrigger%20Intro)
                (:then
                  (bind _trigger_chasing_car (Variables|Default|GetTrigger%20Chasing%20Car)
                    (:then
                      (bind _trigger_mom (Variables|Default|GetTrigger%20Mom)
                        (:then
                          (Default|ActivateOverlapTrigger _trigger_car_crash))
                        (:else)))
                    (:else)))
                (:else)))
            (:else)))
        (:else)))
    (:then_3
      ;[0.15 0.15 0.15 0.5] NPCs
      (bind _mikey (Variables|Default|GetMikey)
        (:then
          (Rendering|SetVisibility (Variables|/Script/Engine.Character|GetMesh _mikey) false false)
          (bind _mom_guarding (Variables|Default|GetMom%20Guarding)
            (:then
              (Rendering|SetActorHiddenInGame _mom_guarding false))
            (:else)))
        (:else)))))

(event Custom|Play%20Sequence%20Level%20on%20Bus
  ;[0.15 0.15 0.15 0.5] Bus Event
  (bind _bus (Variables|Default|GetBus)
    (:then
      (Default|Execute _bus)
      (bind _ambience_sound (Variables|Default|GetAmbience%20Sound)
        (:then
          (Default|SetAmbienceVolume _ambience_sound 0.2))
        (:else)))
    (:else)))

(event EventBeginPlay
  (|CallParentFunction) ; This node is disabled and will not be called.\nDrag off pins to build functionality.
)

(fn ConstructionScript
  (|CallParentFunction))