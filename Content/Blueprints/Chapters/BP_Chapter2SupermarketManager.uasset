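; Chapter 2 manager for the supermarket level, staging the player, customer sequences and the exit from the map.
; Initialization fades in from black, teleports the player to the cashier spawn area, hides the frozen food, starts Customer 3's sequence, unlocks the front door and sets shop barrier collision.
; Separate events start Customer 2 after a delay, reveal the frozen food as interactable, and fade out before the GameInstance changes maps to go home.
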(event Custom|Show%20Food
  (bind _frozen_food (Variables|Default|GetFrozen%20Food)
    (:then
      (Default|ShowItem _frozen_food)
      (Variables|/Game/Blueprints/ModularItems/BP_Engageable.BP_Engageable_C|SetCanInteract? _frozen_food true))
    (:else)))

(event Custom|Initialize%20Chapter%202%20in%20Supermarket
  (bind _player_ref (Variables|Default|GetPlayer%20Ref))
  (Development|PrintString "Initializing Chapter 2  in Supermarket")
  (Utilities|FlowControl|Sequence
    (:then_0
      (Default|BlackScreenThenFadein (Variables|Default|GetBP_FadeScreenComponent) (Variables|Default|GetPlayer%20Ref) 3.0)
      (bind _returnvalue (Actor|GetActorOfClass "/Game/Blueprints/Levels/SpawnArea_Kasir.SpawnArea_Kasir_C"))
      (Transformation|SetActorTransform _player_ref (Math|Transform|MakeTransform (.location (Transformation|GetActorTransform _returnvalue)) (.rotation (Transformation|GetActorTransform _returnvalue)) (Transformation|GetActorScale3D _player_ref)) false true))
    (:then_1
      (bind _frozen_food (Variables|Default|GetFrozen%20Food)
        (:then
          (Rendering|SetVisibility (Variables|/Game/Blueprints/ModularItems/BP_PickupableItem.BP_PickupableItem_C|GetPickupable _frozen_food) false false))
        (:else)))
    (:then_2
      (bind _returnvalue_2 (Actor|GetActorOfClass "/Game/Blueprints/Characters/BP_Customer3.BP_Customer3_C"))
      (Default|StartSequenceCustomer3 _returnvalue_2))
    (:then_3
      (bind _returnvalue_3 (Actor|GetActorOfClass "/Game/Convenience_Store/Blueprints/BP_Front_Door.BP_Front_Door_C"))
      (Variables|/Game/Convenience_Store/Blueprints/BP_Front_Door.BP_Front_Door_C|SetIsLocked _returnvalue_3 false)
      (bind _returnvalue_4 (Actor|GetActorOfClass "/Game/Blueprints/Levels/Barrier_Shop.Barrier_Shop_C"))
      (Default|SetCollisionSetting _returnvalue_4 true))))

(event Custom|Play%20Customer%202%20Sequence
  (Utilities|FlowControl|Delay 5.0)
  (bind _returnvalue (Actor|GetActorOfClass "/Game/Blueprints/Characters/BP_Customer2.BP_Customer2_C"))
  (Default|StartSequenceCustomer2 _returnvalue))

(event Custom|Proceed%20to%20Go%20Home
  (bind _bp_fadescreencomponent (Variables|Default|GetBP_FadeScreenComponent))
  (Default|FadeOut _bp_fadescreencomponent 5.0 (Variables|Default|GetPlayer%20Ref))
  (EventDispatchers|AssignOnExactFinish _bp_fadescreencomponent (delegate Custom|OnFadeOut_Event)))

(event Custom|OnFadeOut_Event
  (Default|CallTeleporttoMap (Variables|Default|GetGame%20Instance%20Ref) "NewEnumerator0"))

(event EventBeginPlay
  (|CallParentFunction))

(fn ConstructionScript
  (|CallParentFunction))