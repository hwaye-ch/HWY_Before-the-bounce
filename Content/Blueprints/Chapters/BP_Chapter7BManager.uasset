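; Chapter 7B manager Blueprint that sets up and stages the chapter's story beats, including the janitor bad ending.
; Initialization hides Mikey-tagged actors, locks Mikey's door, enables the black box and overlap triggers, then fades in with ambience and bus.
; PlayasJanitor grants the bad-ending achievement, switches to a level camera and reveals cleaning cart, police tape and newspaper.
; PlayDoor opens the door, chains reveal audio, fades out and returns to the main menu.
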(event Custom|Initialize%20Chapter%207B
  (bind _bp_fadescreencomponent (Variables|Default|GetBP_FadeScreenComponent))
  (Utilities|FlowControl|Sequence
    (:then_0
      (bind _outactors (Actor|GetAllActorswithTag "mikey"))
      (for _array_element _outactors
        (Rendering|SetActorHiddenInGame _array_element true)
        (Collision|SetActorEnableCollision _array_element false)))
    (:then_1
      (bind _mikey_s_door (Variables|Default|GetMikey's%20Door)
        (:then
          (Variables|/Game/Blueprints/ModularItems/BP_InteractableDoor.BP_InteractableDoor_C|SetIsLocked _mikey_s_door true)
          (Variables|/Game/Blueprints/EventItems/BP_MikeysDoor.BP_MikeysDoor_C|SetIsIntroChapter7 _mikey_s_door true)
          (bind _returnvalue (Actor|GetActorOfClass "/Game/Blueprints/Levels/Trigger_StartGoodEnding.Trigger_StartGoodEnding_C"))
          (Default|ActivateOverlapTrigger _returnvalue)
          (Default|EnableBlackBox (Variables|Default|GetBlackBoxArea)))
        (:else)))
    (:then_2
      (bind _trigger_intro (Variables|Default|GetTrigger%20Intro)
        (:then
          (bind _trigger_enter_apart (Variables|Default|GetTrigger%20Enter%20Apart)
            (:then
              (bind _trigger_welcome (Variables|Default|GetTrigger%20Welcome)
                (:then
                  (Default|ActivateOverlapTrigger _trigger_intro))
                (:else)))
            (:else)))
        (:else)))
    (:then_3
      (Default|BlackScreenThenFadein _bp_fadescreencomponent (Variables|Default|GetPlayer%20Ref) 5.0)
      (EventDispatchers|AssignOnFadein _bp_fadescreencomponent (delegate Custom|OnFadeIn_Event)))))

(event Custom|Play%20as%20Janitor
  ;[0.15 0.15 0.15 0.5 28] STEAM ACHIEVEMENT - BAD ENDING
  (Default|SetAchievement (Variables|Default|GetGame%20Instance%20Ref) "NewEnumerator1")
  (Default|BlackScreenThenFadein (Variables|Default|GetBP_FadeScreenComponent) (Variables|Default|GetPlayer%20Ref) 8.0)
  (Utilities|FlowControl|Sequence
    (:then_0
      (bind _camera_bangku (Variables|Default|GetCamera%20Bangku)
        (:then
          (Default|InitializeLevelCamera _camera_bangku (Variables|Default|GetPlayer%20Ref) 0.0 false)
          (bind _returnvalue (Audio|SpawnSound2D "/Game/Sounds/sfx_janitor-hum.sfx_janitor-hum" 0.5 1.0 0.0 0))
          (Variables|Default|SetHum _returnvalue))
        (:else)))
    (:then_1
      (bind _cleaning_cart (Variables|Default|GetCleaning%20Cart)
        (:then
          (Default|MoveCleaningCart _cleaning_cart))
        (:else)))
    (:then_2
      (bind _police_line (Variables|Default|GetPolice%20Line)
        (:then
          (Default|ShowTape _police_line))
        (:else)))
    (:then_3
      (bind _koran_baru (Variables|Default|GetKoran%20Baru)
        (:then
          (Default|SetInteraction _koran_baru true true))
        (:else)))
    (:then_4
      (bind _ambience_sound (Variables|Default|GetAmbience%20Sound)
        (:then
          (Default|SetAmbienceVolume _ambience_sound 0.1))
        (:else)))))

(event Custom|OnAudioFinished_Event
  (bind _returnvalue (Audio|SpawnSound2D "/Game/Sounds/BasketballBounce/sfx_basketball_dribbling.sfx_basketball_dribbling" 1.0 1.0 0.0 0))
  (Utilities|FlowControl|Delay 7.0)
  (Audio|Components|Audio|FadeOut _returnvalue 0.0 0.0 "Linear" :!class /Script/Engine.AudioComponent)
  (Utilities|FlowControl|Delay 2.0)
  (Default|BacktoMainMenu (Variables|Default|GetPlayer%20Ref)))

(event Custom|Play%20Door
  (bind _mikey_s_door (Variables|Default|GetMikey's%20Door)
    (:then
      (Default|OpenDoorbyEvent _mikey_s_door)
      (bind _returnvalue (Audio|SpawnSound2D "/Game/Sounds/sfx_reveal.sfx_reveal" 1.0 1.0 0.0 0))
      (EventDispatchers|AssignOnAudioFinished _returnvalue (delegate Custom|OnAudioFinished_Event))
      (Utilities|FlowControl|Delay 1e+01)
      (Default|FadeOut (Variables|Default|GetBP_FadeScreenComponent) 3e+01 (Variables|Default|GetPlayer%20Ref)))
    (:else)))

(event Custom|OnFadeIn_Event
  (bind _ambience_sound (Variables|Default|GetAmbience%20Sound)
    (:then
      (Default|SetAmbienceVolume _ambience_sound 0.1)
      (bind _bus (Variables|Default|GetBus)
        (:then
          (Default|Execute _bus))
        (:else)))
    (:else)))

(event Custom|Turn%20Off%20Ambience%20Sound
  (bind _ambience_sound (Variables|Default|GetAmbience%20Sound)
    (:then
      (Default|SetAmbienceVolume _ambience_sound 0.0))
    (:else)))

(event EventBeginPlay
  (|CallParentFunction))

(fn ConstructionScript
  (|CallParentFunction))