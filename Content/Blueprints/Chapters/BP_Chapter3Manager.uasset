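; BP_Chapter3Manager sets up the third chapter and cleans up when it finishes.
; InitializeLevel3 starts night ambience, sets visibility on "mikey"-tagged actors via HideStuff, stops house talking sounds, activates the laptop and plays the swing.
; It also binds the chapter-finished event, which destroys every BP_BolaBasket actor and fades out the horror ambience.
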(event Custom|Initialize%20Level%203
  (EventDispatchers|BindEventtoOnChapterFinished (delegate Custom|On%20Chapter%20Finished_Event))
  (Utilities|FlowControl|Sequence
    (:then_0
      (bind _returnvalue (Actor|GetActorOfClass "/Game/Blueprints/Levels/BP_AmbienceSound.BP_AmbienceSound_C"))
      (bind _output_get (Variables|Default|SetAmbience _returnvalue))
      (Default|SpawnNightAmbience _output_get 0.01))
    (:then_1
      (bind _outactors (Actor|GetAllActorswithTag "mikey"))
      (for _array_element _outactors
        (Rendering|SetActorHiddenInGame _array_element (Variables|Default|GetHideStuff?))))
    (:then_2
      (bind _outactors_2 (Actor|GetAllActorsOfClass "/Game/Blueprints/EventItems/BP_HouseTalking.BP_HouseTalking_C"))
      (for _array_element_2 _outactors_2
        (bind _sound (Variables|/Game/Blueprints/EventItems/BP_HouseTalking.BP_HouseTalking_C|GetSound _array_element_2)
          (:then
            (Audio|Components|Audio|Stop _sound))
          (:else))))
    (:then_3
      (bind _laptop (Variables|Default|GetLaptop)
        (:then
          (Default|ActivateObject _laptop))
        (:else)))
    (:then_4
      (bind _swing (Variables|Default|GetSwing)
        (:then
          (Default|PlaySwing _swing))
        (:else)))))

(event Custom|On%20Chapter%20Finished_Event
  (Utilities|FlowControl|Sequence
    (:then_0
      (bind _outactors (Actor|GetAllActorsOfClass "/Game/Blueprints/EventItems/BP_BolaBasket.BP_BolaBasket_C"))
      (for _array_element _outactors
        (Actor|DestroyActor _array_element)))
    (:then_1
      (bind _ambience (Variables|Default|GetAmbience)
        (:then
          (Audio|Components|Audio|FadeOut (Variables|/Game/Blueprints/Levels/BP_AmbienceSound.BP_AmbienceSound_C|GetHorrorAmbience _ambience) 2.0 0.0 "Linear" :!class /Script/Engine.AudioComponent))
        (:else)))))

(fn ConstructionScript
  (|CallParentFunction))