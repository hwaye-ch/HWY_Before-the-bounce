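; Manager for Chapter 5, a scripted horror sequence in which the player lies in bed trying to sleep amid disturbances.
; Dialogue-end callbacks and delays chain the scares: creaking door, kitchen sounds, TV, peeping father, disturbance sequence and basketball event.
; Holding LMB closes the eyes and fills a progress bar; completion advances the story according to Status.
; Also saves the chapter on start and provides a tag-based burnt-wall material swap.
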(event FinishProgressFilling(BP_ProgressableComponent)
  ;[0.15 0.15 0.15 0.5 72] Long Interact
  (CallFunction|FinishProgressBarFilling))

(event UpdateProgressFilling(BP_ProgressableComponent)
  (params (ProgressPercentage :type Float%20%28double-precision%29))
  ;[0.15 0.15 0.15 0.5 72] On Progress Hold LMB
  (Variables|Default|SetTemp%20Progress%20Percentage ProgressPercentage)
  (switch Utilities|FlowControl|Switch|SwitchonE_SleepParalysis (Variables|Default|GetStatus)
    (:NewEnumerator0
      _)
    (:NewEnumerator1
      _)
    (:NewEnumerator2
      _)
    (:NewEnumerator3
      _))
  (if (>= (Variables|Default|GetTemp%20Progress%20Percentage) 0.8)
    (Variables|Default|SetIs%20Progress%20Bar%20Ready? false)
    (CallFunction|FinishProgressBarFilling)
    (Utilities|FlowControl|Delay 2.0)
    (Default|RemoveProgressBar (Variables|Default|GetBP_ProgressableComponent))))

(event Custom|Play%20Chapter%205
  (bind _bp_fadescreencomponent (Variables|Default|GetBP_FadeScreenComponent))
  (Utilities|FlowControl|Sequence
    (:then_0
      (Default|BlackScreenThenFadein _bp_fadescreencomponent (Variables|Default|GetPlayer%20Ref) 5.0)
      (EventDispatchers|AssignOnFadein _bp_fadescreencomponent (delegate Custom|OnFadeIn_Event)))
    (:then_1
      (bind _kasur (Variables|Default|GetKasur)
        (:then
          (Variables|/Game/Blueprints/ModularItems/BP_Engageable.BP_Engageable_C|SetHide%20Outline? _kasur true)
          (Utilities|FlowControl|DelayUntilNextTick)
          (bind _bedcamera (Variables|Default|GetBedCamera)
            (:then
              (Default|InitializeLevelCamera _bedcamera (Variables|Default|GetPlayer%20Ref) 0.0)
              (bind _ambiencesound (Variables|Default|GetAmbienceSound)
                (:then
                  (Default|CallTeleporttoMainMapSpawnLocation (Variables|Default|GetPlayer%20Ref))
                  (Default|SetAmbienceVolume _ambiencesound 0.1)
                  (bind _additional_light (Variables|Default|GetAdditional%20Light)
                    (:then
                      (Rendering|SetVisibility (Variables|/Script/Engine.SpotLight|GetSpotLightComponent _additional_light) true false)
                      (bind _cookingsfx (Variables|Default|GetCookingSfx)
                        (:then
                          (Default|SetHorrorAmbience _cookingsfx))
                        (:else)))
                    (:else)))
                (:else)))
            (:else)))
        (:else)))
    (:then_2
      (EventDispatchers|AssignLongInteraction (Variables|Default|GetPlayer%20Ref) (EventDispatchers|CreateEvent :!event Custom|LongInteraction_Event))
      (Variables|Default|SetIs%20Progress%20Bar%20Ready? false))
    (:then_3
      (Default|SaveChapter (Variables|Default|GetGame%20Instance%20Ref) "NewEnumerator4"))))

(event Custom|OnDialogueEnded_Event_2
  ;[0.15 0.15 0.15 0.5] Cooking Sound Effect
  (EventDispatchers|UnbindEventfromOnDialogueEnded (Variables|Default|GetBP_DialogueComponent) (delegate Custom|OnDialogueEnded_Event_2))
  (Utilities|FlowControl|Delay 1e+01)
  (Variables|Default|SetClose%20Timer 0.0)
  (Variables|Default|SetStatus "NewEnumerator0")
  (Variables|Default|SetDuration%20Needed 5.0)
  (CallFunction|ShowMissionWidget)
  (Variables|Default|SetIs%20Progress%20Bar%20Ready? true))

(event Custom|Look%20at%20the%20Poster
  (bind _returnvalue (UserInterface|CreateWidget "/Game/Blueprints/Widgets/WBP_Mission.WBP_Mission_C" 0 "Look at the Poster"))
  (bind _output_get (Variables|Default|SetMission%20Widget _returnvalue))
  (UserInterface|Viewport|AddtoViewport _output_get 0)
  (Utilities|FlowControl|Delay 2.0)
  (Widget|RemovefromParent (Variables|Default|GetMission%20Widget)))

(event Custom|Open%20Eyes%20Event
  (switch Utilities|FlowControl|Switch|SwitchonE_SleepParalysis (Variables|Default|GetStatus)
    (:NewEnumerator1
      (Utilities|FlowControl|DoOnce false
        (:Completed
          (bind _dialoguecomponent (Default|ConstructDialogue (Variables|Default|GetBP_DialogueComponent) "ch5_shocked" "/Game/Dialogue/Chapter5_Dialogue.Chapter5_Dialogue" false false))
          (Default|DisplayAutoDialogue _dialoguecomponent)
          (Default|SetChromaticAbberationtoCamera (Variables|Default|GetBedCamera) true 4.0 false))))))

(event Custom|Finish%20ProgressBar%20Filling
  ;[0.15 0.15 0.15 0.5 72] Event After Closing Eyes
  (Variables|Default|SetIs%20Progress%20Bar%20Ready? false)
  (Widget|RemovefromParent (Variables|Default|GetMission%20Widget))
  (switch Utilities|FlowControl|Switch|SwitchonE_SleepParalysis (Variables|Default|GetStatus)
    (:NewEnumerator0
      (Utilities|FlowControl|DoOnce false
        (:Completed
          (Utilities|FlowControl|Delay 2.0)
          (bind _dialoguecomponent (Default|ConstructDialogue (Variables|Default|GetBP_DialogueComponent) "ch5_wondering" "/Game/Dialogue/Chapter5_Dialogue.Chapter5_Dialogue" true true))
          (Default|ShowDialogue _dialoguecomponent (Variables|Default|GetPlayer%20Ref) self)
          (EventDispatchers|AssignOnDialogueEnded _dialoguecomponent (delegate Custom|OnDialogueEnded_Event_3)))))
    (:NewEnumerator1
      (Utilities|FlowControl|DoOnce false
        (:Completed
          (CallFunction|MoveDad))))
    (:NewEnumerator2
      (Utilities|FlowControl|DoOnce false
        (:Completed
          (CallFunction|ReturnDad))))
    (:NewEnumerator3
      (Utilities|FlowControl|DoOnce false
        (:Completed
          (CallFunction|DialogCannotSleep))))))

(event Custom|OnDialogueEnded_Event_0
  (EventDispatchers|UnbindallEventsfromOnDialogueEnded (Variables|Default|GetBP_DialogueComponent))
  (Utilities|FlowControl|Delay 5.0)
  (Variables|Default|SetClose%20Timer 0.0)
  (Variables|Default|SetStatus "NewEnumerator3")
  (Variables|Default|SetDuration%20Needed 1e+01)
  (Variables|Default|SetIs%20Progress%20Bar%20Ready? true)
  (CallFunction|ShowMissionWidget))

(event Custom|Dialog%20cannot%20sleep
  (bind _bp_dialoguecomponent (Variables|Default|GetBP_DialogueComponent))
  ;[0.15 0.15 0.15 0.5 72] Dialogue Cannot Sleep
  (Utilities|FlowControl|Delay 2.0)
  (EventDispatchers|AssignOnDialogueEnded _bp_dialoguecomponent (delegate Custom|OnDialogueEnded_Event_1))
  (bind _dialoguecomponent (Default|ConstructDialogue _bp_dialoguecomponent "ch5_sulittidur" "/Game/Dialogue/Chapter5_Dialogue.Chapter5_Dialogue" true true))
  (Default|ShowDialogue _dialoguecomponent (Variables|Default|GetPlayer%20Ref) self))

(event Custom|OnDialogueEnded_Event_1
  ;[0.15 0.15 0.15 0.5 72] Dialogue Cannot Sleep
  ;;[0.15 0.15 0.15 0.5 72] ANIMATION
  (EventDispatchers|UnbindEventfromOnDialogueEnded (Variables|Default|GetBP_DialogueComponent) (delegate Custom|OnDialogueEnded_Event_1))
  (Utilities|FlowControl|Delay 1e+01)
  (bind _returnvalue (Sequencer|Player|CreateLevelSequencePlayer "/Game/Animation/Anim_CrazyDisturbance.Anim_CrazyDisturbance"))
  (Sequencer|Player|Play _returnvalue :!class /Script/MovieScene.MovieSceneSequencePlayer)
  (EventDispatchers|BindEventtoOnFinished _returnvalue (delegate Custom|On%20Finished%20Sequence))
  (Utilities|FlowControl|Delay 3e+01)
  (Audio|SpawnSound2D "/Game/Sounds/sfx_tension-build-up.sfx_tension-build-up" 1.0 1.0 0.0 0))

(event Custom|OnFadeIn_Event
  (bind _bp_dialoguecomponent (Variables|Default|GetBP_DialogueComponent))
  (EventDispatchers|UnbindEventfromOnFadein (Variables|Default|GetBP_FadeScreenComponent) (delegate Custom|OnFadeIn_Event))
  (Utilities|FlowControl|Sequence
    (:then_1)
    (:then_2
      (Utilities|FlowControl|Delay 1e+01)
      (EventDispatchers|AssignOnDialogueEnded _bp_dialoguecomponent (delegate Custom|OnDialogueEnded_Event))
      (bind _dialoguecomponent (Default|ConstructDialogue _bp_dialoguecomponent "ch5_sp1" "/Game/Dialogue/Chapter5_Dialogue.Chapter5_Dialogue" true true))
      (Default|ShowDialogue _dialoguecomponent (Variables|Default|GetPlayer%20Ref) self))))

(event Custom|OnDialogueEnded_Event_5
  (EventDispatchers|UnbindEventfromOnDialogueEnded (Variables|Default|GetBP_DialogueComponent) (delegate Custom|OnDialogueEnded_Event_5))
  (Default|SetCollision (Variables|Default|GetBasketBallSound)))

(event Custom|Change%20Wall
  (params (Is%20Burnt? :type Boolean))
  (bind _outactors (Actor|GetAllActorswithTag "wall"))
  (for _array_element _outactors
    (bind _asstatic_mesh_actor (Utilities|Casting|CastToStaticMeshActor _array_element))
    (if Is%20Burnt?
      (Rendering|Material|SetMaterial (Variables|/Script/Engine.StaticMeshActor|GetStaticMeshComponent _asstatic_mesh_actor) 0 "/Game/Materials/M_BurntWall.M_BurntWall")
      (else
        (Rendering|Material|SetMaterial (Variables|/Script/Engine.StaticMeshActor|GetStaticMeshComponent _asstatic_mesh_actor) 0 "/Game/Materials/M_HouseWall1.M_HouseWall1"))))
  (bind _outactors_2 (Actor|GetAllActorswithTag "ceiling"))
  (for _array_element_2 _outactors_2
    (bind _asstatic_mesh_actor_2 (Utilities|Casting|CastToStaticMeshActor _array_element_2))
    (if Is%20Burnt?
      (Rendering|Material|SetMaterial (Variables|/Script/Engine.StaticMeshActor|GetStaticMeshComponent _asstatic_mesh_actor_2) 0 "/Game/Materials/M_BurntWall.M_BurntWall")
      (else
        (Rendering|Material|SetMaterial (Variables|/Script/Engine.StaticMeshActor|GetStaticMeshComponent _asstatic_mesh_actor_2) 0 "/Game/Materials/M_RusunPaint.M_RusunPaint")))))

(event Custom|On%20Finished%20Sequence
  (bind _bp_dialoguecomponent (Variables|Default|GetBP_DialogueComponent))
  ;[0.15 0.15 0.15 0.5 72] Dialogue Cannot Sleep
  ;;[0.15 0.15 0.15 0.5 72] ANIMATION
  (bind _basketballsound (Variables|Default|GetBasketBallSound)
    (:then
      (Default|SetEventReady _basketballsound)
      (bind _posterlight (Variables|Default|GetPosterLight)
        (:then
          (Rendering|SetVisibility (Variables|/Script/Engine.SpotLight|GetSpotLightComponent _posterlight) true false)
          (Utilities|FlowControl|Delay 3.0)
          (bind _dialoguecomponent (Default|ConstructDialogue _bp_dialoguecomponent "ch5_basket" "/Game/Dialogue/Chapter5_Dialogue.Chapter5_Dialogue" true true))
          (Default|ShowDialogue _dialoguecomponent (Variables|Default|GetPlayer%20Ref) self)
          (EventDispatchers|AssignOnDialogueEnded _bp_dialoguecomponent (delegate Custom|OnDialogueEnded_Event_5)))
        (:else)))
    (:else)))

(event Custom|Show%20Mission%20Widget
  ;[0.15 0.15 0.15 0.5] Mission Widget
  (bind _mission_widget (Variables|Default|GetMission%20Widget)
    (:then
      _)
    (:else
      (bind _returnvalue (UserInterface|CreateWidget "/Game/Blueprints/Widgets/WBP_Mission.WBP_Mission_C" 0 "Hold [LMB] to Sleep"))
      (bind _output_get (Variables|Default|SetMission%20Widget _returnvalue))))
  (UserInterface|Viewport|AddtoViewport _mission_widget 0)
  (Utilities|FlowControl|Delay 3.0)
  (Widget|RemovefromParent (Variables|Default|GetMission%20Widget)))

(event Custom|Hide%20Mission%20Widget
  ;[0.15 0.15 0.15 0.5] Mission Widget
  (Widget|RemovefromParent (Variables|Default|GetMission%20Widget)))

(event Custom|OnDialogueEnded_Event_3
  ;[0.15 0.15 0.15 0.5 72] Event After Closing Eyes
  (EventDispatchers|UnbindEventfromOnDialogueEnded (stale Custom|Finish%20ProgressBar%20Filling _dialoguecomponent) (delegate Custom|OnDialogueEnded_Event_3))
  (Utilities|FlowControl|Delay 1e+01)
  (CallFunction|SetTVon)
  (Utilities|FlowControl|Delay 1.0)
  (Audio|SpawnSound2D "/Game/Sounds/sfx_creepy-whossh.sfx_creepy-whossh" 2.0 1.0 0.0 0))

(event Custom|OnDialogueEnded_Event
  (bind _bp_dialoguecomponent (Variables|Default|GetBP_DialogueComponent))
  ;[0.15 0.15 0.15 0.5] Door opened mysteriously
  (EventDispatchers|UnbindallEventsfromOnDialogueEnded (Variables|Default|GetBP_DialogueComponent))
  (bind _ryan_sdoor (Variables|Default|GetRyan'sDoor)
    (:then
      (Default|ClosetheDoor _ryan_sdoor)
      (Utilities|FlowControl|Delay 1e+01)
      (Default|OpenDoorbyEvent _ryan_sdoor)
      (Audio|PlaySoundatLocation "/Game/Sounds/sfx_door-creaking.sfx_door-creaking" (Transformation|GetWorldLocation (Variables|/Game/Blueprints/ModularItems/BP_InteractableDoor.BP_InteractableDoor_C|GetDoor _ryan_sdoor)) "0, 0, 0" 0.4 1.0 0.0 "/Game/Sounds/BasketballBounce/SA_ProximitySoundWithLocation.SA_ProximitySoundWithLocation" 0 0 0)
      (Utilities|FlowControl|Delay 16.0)
      ;[0.15 0.15 0.15 0.5] Cooking Sound Effect
      (bind _cookingsfx (Variables|Default|GetCookingSfx)
        (:then
          (Default|PlayCookingSfx _cookingsfx)
          (bind _dialoguecomponent (Default|ConstructDialogue _bp_dialoguecomponent "ch5_dapur" "/Game/Dialogue/Chapter5_Dialogue.Chapter5_Dialogue" true true))
          (Default|ShowDialogue _dialoguecomponent (Variables|Default|GetPlayer%20Ref) self)
          (EventDispatchers|AssignOnDialogueEnded _bp_dialoguecomponent (delegate Custom|OnDialogueEnded_Event_2)))
        (:else)))
    (:else)))

(event Custom|LongInteraction_Event
  (params (State :type E_LongInteract%20Enum :default "NewEnumerator0"))
  ;[0.15 0.15 0.15 0.5 72] Long Interact
  (Variables|Default|SetLong%20Interact%20State State)
  (Utilities|FlowControl|Sequence
    (:then_0
      _)
    (:then_1
      (Variables|Default|GetIs%20Progress%20Bar%20Ready?
        (:then
          (Default|SetProgressable (Variables|Default|GetBP_ProgressableComponent) (Variables|Default|GetClose%20Timer) (* (Variables|Default|GetDuration%20Needed) 6e+01) (Variables|Default|GetLong%20Interact%20State)))
        (:else))))
  (switch Utilities|FlowControl|Switch|SwitchonE_LongInteract State
    (:NewEnumerator0
      (Math|Float|IncrementFloat (Variables|Default|GetClose%20Timer)
        (:%20%20
          (Utilities|FlowControl|Sequence
            (:then_0
              (bind _result (Math|Float|IncrementFloat (Variables|Default|GetClose%20Eyes%20Counter))
                (:%20%20
                  (Variables|Default|SetIs%20Eyes%20Closing? (>= _result 6e+01)))))
            (:then_1
              (Utilities|FlowControl|DoOnce false :!label _label
                (:Completed
                  (bind _closeeyeswidget (Variables|Default|GetCloseEyesWidget)
                    (:then
                      (UserInterface|Animation|PlayAnimation _closeeyeswidget (Variables|/Game/Blueprints/Widgets/WBP_CloseEyes.WBP_CloseEyes_C|GetCloseEyesAnimation _closeeyeswidget) 0.0 1 "Forward" 1.0 false))
                    (:else)))))))))
    (:NewEnumerator1
      (Variables|Default|GetCloseEyesWidget
        (:then
          _)
        (:else
          (bind _returnvalue (UserInterface|CreateWidget "/Game/Blueprints/Widgets/WBP_CloseEyes.WBP_CloseEyes_C"))
          (bind _output_get (Variables|Default|SetCloseEyesWidget _returnvalue))))
      (UserInterface|Viewport|AddtoViewport _output_get 0)
      (Variables|Default|SetIs%20Eyes%20Closing? false))
    (:NewEnumerator2
      (Variables|Default|SetClose%20Eyes%20Counter 0.0)
      (bind _closeeyeswidget_2 (Variables|Default|GetCloseEyesWidget)
        (:then
          (Class|UserWidget|PlayAnimationReverse _closeeyeswidget_2 (Variables|/Game/Blueprints/Widgets/WBP_CloseEyes.WBP_CloseEyes_C|GetCloseEyesAnimation _closeeyeswidget_2) 1.0 false)
          (Utilities|FlowControl|Sequence
            (:then_0
              (Variables|Default|SetClose%20Timer 0.0)
              (goto _label Reset))
            (:then_1
              (Utilities|FlowControl|Delay 0.3)
              (Variables|Default|GetIs%20Eyes%20Closing?
                (:then
                  (CallFunction|OpenEyesEvent))
                (:else)))))
        (:else)))))

(event Custom|OnDialogueEnded_Event_4
  ;[0.15 0.15 0.15 0.5 72] Television Segment
  (EventDispatchers|UnbindEventfromOnDialogueEnded (stale Custom|Set%20TV%20on _dialoguecomponent) (delegate Custom|OnDialogueEnded_Event_4))
  (Utilities|FlowControl|Delay 2e+01)
  (Variables|Default|SetClose%20Timer 0.0)
  (Variables|Default|SetStatus "NewEnumerator1")
  (Variables|Default|SetDuration%20Needed 5.0)
  (Variables|Default|SetIs%20Progress%20Bar%20Ready? true)
  (CallFunction|ShowMissionWidget))

(event Custom|Set%20TV%20on
  ;[0.15 0.15 0.15 0.5 72] Television Segment
  (bind _television (Variables|Default|GetTelevision)
    (:then
      (Default|TurnonTV _television)
      (Utilities|FlowControl|Delay 5.0)
      (bind _dialoguecomponent (Default|ConstructDialogue (Variables|Default|GetBP_DialogueComponent) "ch5_tv" "/Game/Dialogue/Chapter5_Dialogue.Chapter5_Dialogue" true true))
      (Default|ShowDialogue _dialoguecomponent (Variables|Default|GetPlayer%20Ref) self)
      (EventDispatchers|AssignOnDialogueEnded _dialoguecomponent (delegate Custom|OnDialogueEnded_Event_4)))
    (:else)))

(event Custom|Move%20Dad
  ;[0.15 0.15 0.15 0.5 72] Father Peeping
  (bind _father (Variables|Default|GetFather)
    (:then
      (Default|Peep _father)
      (Utilities|FlowControl|Sequence
        (:then_0
          (Utilities|FlowControl|Delay 2.0)
          (Default|SetChromaticAbberationtoCamera (Variables|Default|GetBedCamera) true 3.0 false)
          (Audio|SpawnSound2D "/Game/Sounds/sfx_creepy-transition.sfx_creepy-transition" 1.0 1.0 0.0 0))
        (:then_1
          (Utilities|FlowControl|Delay 1e+01)
          (Variables|Default|SetClose%20Timer 0.0)
          (Variables|Default|SetStatus "NewEnumerator2")
          (Variables|Default|SetDuration%20Needed 1e+01)
          (Variables|Default|SetIs%20Progress%20Bar%20Ready? true)
          (CallFunction|ShowMissionWidget))))
    (:else)))

(event Custom|Return%20Dad
  (bind _television (Variables|Default|GetTelevision))
  (bind _bp_dialoguecomponent (Variables|Default|GetBP_DialogueComponent))
  ;[0.15 0.15 0.15 0.5 72] Father Peeping
  (Default|SetChromaticAbberationtoCamera (Variables|Default|GetBedCamera) false 3.0 false)
  (Default|ReturnfromPeep (Variables|Default|GetFather))
  (Utilities|FlowControl|Delay 2e+01)
  (Default|TurnOffTV (Variables|Default|GetTelevision))
  (Utilities|FlowControl|Delay 1e+01)
  (Default|PlayCrazyDisturbance (Variables|Default|GetTelevision))
  (Utilities|FlowControl|Delay 2e+01)
  (Default|TurnOffTV _television)
  (Audio|Components|Audio|Stop (Variables|/Game/Blueprints/EventItems/BP_Television.BP_Television_C|GetNbaSound _television))
  (Default|StopAllSounds (Variables|Default|GetCookingSfx))
  (Utilities|FlowControl|Delay 15.0)
  (EventDispatchers|AssignOnDialogueEnded _bp_dialoguecomponent (delegate Custom|OnDialogueEnded_Event_0))
  (bind _dialoguecomponent (Default|ConstructDialogue _bp_dialoguecomponent "ch5_sunyi" "/Game/Dialogue/Chapter5_Dialogue.Chapter5_Dialogue" true true))
  (Default|ShowDialogue _dialoguecomponent (Variables|Default|GetPlayer%20Ref) self))

(event EventBeginPlay
  ;[0.15 0.15 0.15 0.5] Debug
  (|CallParentFunction))

(fn ConstructionScript
  (|CallParentFunction))