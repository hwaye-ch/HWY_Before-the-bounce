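; Chapter 2 manager that sets up and cleans up the level's scripted content.
; InitializeLevel2 fades in the screen, lowers ambience volume, starts house chatter, prepares Mikey and his calling trigger, and makes the laptop interactable.
; It binds a chapter-finished handler that stops house chatter, hides Mikey on the bus and destroys the Mikey actor.
; BeginPlay only calls the parent, and a disconnected debug path can force Chapter 2.
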(event Custom|Initialize%20Level%202
  (Default|Fadein (Variables|Default|GetBP_FadeScreenComponent) (Variables|Default|GetPlayer%20Ref))
  (Development|PrintString "Initializing Chapter 2....")
  (EventDispatchers|BindEventtoOnChapterFinished (delegate Custom|On%20Chapter%20Finished_Event))
  (Utilities|FlowControl|Sequence
    (:then_0
      (bind _returnvalue (Actor|GetActorOfClass "/Game/Blueprints/Levels/BP_AmbienceSound.BP_AmbienceSound_C"))
      (bind _output_get (Variables|Default|SetAmbience _returnvalue))
      (Default|SetAmbienceVolume _output_get 0.4))
    (:then_1
      (bind _outactors (Actor|GetAllActorsOfClass "/Game/Blueprints/EventItems/BP_HouseTalking.BP_HouseTalking_C"))
      (for _array_element _outactors
        (Default|PlayPeopleTalking _array_element true)))
    (:then_2
      (bind _mikey (Variables|Default|GetMikey)
        (:then
          (Default|SetupEventforChapter2 _mikey))
        (:else)))
    (:then_3
      (bind _trigger_mikey_calling (Variables|Default|GetTrigger%20Mikey%20Calling)
        (:then
          (Default|ActivateOverlapTrigger _trigger_mikey_calling))
        (:else)))
    (:then_4
      (bind _laptop (Variables|Default|GetLaptop)
        (:then
          (Variables|/Game/Blueprints/ModularItems/BP_Engageable.BP_Engageable_C|SetCanInteract? _laptop true))
        (:else)))))

(event Custom|On%20Chapter%20Finished_Event
  (Utilities|FlowControl|Sequence
    (:then_0
      (bind _outactors (Actor|GetAllActorsOfClass "/Game/Blueprints/EventItems/BP_HouseTalking.BP_HouseTalking_C"))
      (for _array_element _outactors
        (bind _sound (Variables|/Game/Blueprints/EventItems/BP_HouseTalking.BP_HouseTalking_C|GetSound _array_element)
          (:then
            (Audio|Components|Audio|Stop _sound))
          (:else))))
    (:then_1
      (bind _bus (Variables|Default|GetBus)
        (:then
          (Default|HIdeMikey _bus))
        (:else)))
    (:then_2
      ;[0.15 0.15 0.15 0.5 50] v1.2.1
      (bind _mikey (Variables|Default|GetMikey)
        (:then
          (Actor|DestroyActor _mikey))
        (:else)))))

(event EventBeginPlay
  ;[0.15 0.15 0.15 0.5] Debug
  (|CallParentFunction))

(fn ConstructionScript
  (|CallParentFunction))