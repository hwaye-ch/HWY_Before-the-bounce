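; BP_ChapterNightmare runs the nightmare chapter sequence, staging props and scares across successive blocks.
; InitiateNightmare restricts movement, teleports the player, starts a low hum and hallucination effect, then shows dialogue and a lantern mission prompt.
; SpawnStuff receives new and current blocks, places story items by SpawnCount, then Setups increments it and opens walls.
; Count milestones spawn and later remove crawling Mom, then restore the wall and spawn evil Mikey with mystic audio.
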(event Custom|Initiate%20Nightmare
  (bind _player_ref (Variables|Default|GetPlayer%20Ref))
  (Utilities|FlowControl|Sequence
    (:then_0
      ;[0.15 0.15 0.15 0.5 72] Initialize Player's State
      (Default|BlackScreenThenFadein (Variables|Default|GetBP_FadeScreenComponent) (Variables|Default|GetPlayer%20Ref) 3.0)
      (Variables|/Game/FirstPerson/Blueprints/BP_FirstPersonCharacter.BP_FirstPersonCharacter_C|SetCan%20Jump? _player_ref false)
      (Variables|/Game/FirstPerson/Blueprints/BP_FirstPersonCharacter.BP_FirstPersonCharacter_C|SetCan%20Crouch? _player_ref false)
      (Variables|/Game/FirstPerson/Blueprints/BP_FirstPersonCharacter.BP_FirstPersonCharacter_C|SetCan%20Run? _player_ref false)
      (EventDispatchers|BindEventtoOnChapterFinished (delegate Custom|On%20Chapter%20Finished_Event)))
    (:then_1
      ;[0.15 0.15 0.15 0.5 72] Teleport to Nightmare
      (bind _player_spawn_area (Variables|Default|GetPlayer%20Spawn%20Area)
        (:then
          (Transformation|SetActorLocation (Variables|Default|GetPlayer%20Ref) (.location (Transformation|GetActorTransform _player_spawn_area)) false true)
          (Pawn|SetControlRotation (Game|GetPlayerController 0) (.rotation (Transformation|GetActorTransform _player_spawn_area))))
        (:else)))
    (:then_2
      ;[0.15 0.15 0.15 0.5 72] BG Sound
      (bind _returnvalue (Audio|SpawnSound2D "/Game/Sounds/sfx_low-hum.sfx_low-hum" 3.0 1.0 0.0 0))
      (Variables|Default|SetLow%20Hum%20Sfx _returnvalue))
    (:then_3
      (Utilities|FlowControl|Delay 6.0)
      (bind _dialoguecomponent (Default|ConstructDialogue (Variables|Default|GetBP_DialogueComponent) "ch7_akhir" "/Game/Dialogue/Chapter7_Dialogue.Chapter7_Dialogue" true true))
      (Default|ShowDialogue _dialoguecomponent (Variables|Default|GetPlayer%20Ref) self)
      (EventDispatchers|AssignOnDialogueEnded _dialoguecomponent (delegate Custom|OnDialogueEnded_Event)))
    (:then_4
      (Default|SetHaluEffect (Variables|Default|GetPlayer%20Ref) true))))

(event Custom|Spawn%20Stuff
  (params (New%20Block :type Area%20Endless%20Nightmare%20Object%20Reference) (Current%20Block :type Area%20Endless%20Nightmare%20Object%20Reference))
  ;[0.15 0.15 0.15 0.5 72] Spawn Stuffs
  (Variables|Default|SetCurrentBlock Current%20Block)
  (Variables|Default|SetNewBlock New%20Block)
  (switch int (Variables|Default|GetSpawn%20Count)
    (:Default
      (CallFunction|Setups :!label _label))
    (:0
      (goto _label))
    (:1
      (goto _label))
    (:2
      (bind _returnvalue (Game|SpawnActorfromClass "/Game/Blueprints/EventItems/BP_Koran.BP_Koran_C" (Transformation|GetWorldTransform (Variables|/Game/Blueprints/Items/Area_EndlessNightmare.Area_EndlessNightmare_C|GetSpawnStuffArea (Variables|Default|GetNewBlock))) "Undefined" "MultiplyWithRoot" 0 true 0))
      (Development|PrintString (Utilities|String|Append "Spawning " (Utilities|GetDisplayName _returnvalue)))
      (Rendering|SetVisibility (Variables|/Game/Blueprints/Items/Area_EndlessNightmare.Area_EndlessNightmare_C|GetSpawnStuffArea (Variables|Default|GetNewBlock)) true true :!label _label_2)
      (CallFunction|Setups))
    (:3
      (goto _label))
    (:4
      (bind _returnvalue_2 (Game|SpawnActorfromClass "/Game/Blueprints/EventItems/BP_ConsultationLetterFromSarah.BP_ConsultationLetterFromSarah_C" (Transformation|GetWorldTransform (Variables|/Game/Blueprints/Items/Area_EndlessNightmare.Area_EndlessNightmare_C|GetSpawnStuffArea (Variables|Default|GetNewBlock))) "Undefined" "MultiplyWithRoot" 0 true 0))
      (Variables|/Game/Blueprints/EventItems/BP_ConsultationLetterFromSarah.BP_ConsultationLetterFromSarah_C|SetRunEvent? _returnvalue_2 false)
      (Development|PrintString (Utilities|String|Append (Utilities|GetDisplayName _returnvalue_2) (Utilities|GetDisplayName 0)))
      (goto _label_2))
    (:5
      (goto _label))
    (:6
      (bind _returnvalue_3 (Game|SpawnActorfromClass "/Game/Blueprints/EventItems/BP_Rontgen.BP_Rontgen_C" (Transformation|GetWorldTransform (Variables|/Game/Blueprints/Items/Area_EndlessNightmare.Area_EndlessNightmare_C|GetSpawnStuffArea (Variables|Default|GetNewBlock))) "Undefined" "MultiplyWithRoot" 0 true 0))
      (Variables|/Game/Blueprints/EventItems/BP_Rontgen.BP_Rontgen_C|SetBlock%20Event? _returnvalue_3 true)
      (Development|PrintString (Utilities|String|Append (Utilities|GetDisplayName _returnvalue_3) (Utilities|GetDisplayName 0)))
      (goto _label_2))))

(event Custom|Spawn%20Mom
  ;[0.15 0.15 0.15 0.5 72] Spawn Mom
  (bind _returnvalue (Game|SpawnActorfromClass "/Game/Blueprints/Characters/BP_MomCrawling.BP_MomCrawling_C" (Transformation|GetWorldTransform (Variables|/Game/Blueprints/Items/Area_EndlessNightmare.Area_EndlessNightmare_C|GetSpawnAreaMother (Variables|Default|GetCurrentBlock))) "Undefined" "MultiplyWithRoot" 0 0))
  (bind _output_get (Variables|Default|SetMother _returnvalue))
  (Class|PawnSensingComponent|SetSensingUpdatesEnabled (Variables|/Game/Blueprints/Characters/BP_MomCrawling.BP_MomCrawling_C|GetPawnSensing _output_get) true))

(event Custom|Setups
  (bind _newblock (Variables|Default|GetNewBlock))
  (bind _newblock_2 (Variables|Default|GetNewBlock))
  (bind _wall (Variables|/Game/Blueprints/Items/Area_EndlessNightmare.Area_EndlessNightmare_C|GetWall _newblock_2))
  (bind _wall_2 (Variables|/Game/Blueprints/Items/Area_EndlessNightmare.Area_EndlessNightmare_C|GetWall _newblock))
  (bind _result (Math|Integer|IncrementInt (Variables|Default|GetSpawn%20Count))
    (:%20%20
      (Development|PrintString (Utilities|String|Append "Spawn Count: " (Utilities|String|ToString(Integer) _result)))
      (Rendering|SetVisibility _wall false false)
      (Collision|SetCollisionEnabled _wall "NoCollision")
      (if (== (Variables|Default|GetSpawn%20Count) 10)
        (CallFunction|SpawnMom)
        (elif (== (Variables|Default|GetSpawn%20Count) 24)
          (bind _mother (Variables|Default|GetMother)
            (:then
              (Default|Destroy _mother)
              (Variables|/Game/FirstPerson/Blueprints/BP_FirstPersonCharacter.BP_FirstPersonCharacter_C|SetIsPanic (Variables|Default|GetPlayer%20Ref) false))
            (:else))
          (elif (== (Variables|Default|GetSpawn%20Count) 30)
            (Development|PrintString "Spawning Michael")
            (Rendering|SetVisibility _wall_2 true true)
            (Collision|SetCollisionEnabled _wall_2 "QueryAndPhysics")
            (Game|SpawnActorfromClass "/Game/Blueprints/Characters/BP_MikeyEvilSitting.BP_MikeyEvilSitting_C" (Transformation|GetWorldTransform (Variables|/Game/Blueprints/Items/Area_EndlessNightmare.Area_EndlessNightmare_C|GetMikeyLocation (Variables|Default|GetCurrentBlock))) "Undefined" "MultiplyWithRoot" 0 0)
            (bind _returnvalue (Audio|SpawnSound2D "/Game/Sounds/sfx_mystic.sfx_mystic" 3.0 1.0 0.0 0))
            (Variables|Default|SetMystic%20Sound _returnvalue)))))))

(event Custom|OnDialogueEnded_Event
  (Utilities|FlowControl|Sequence
    (:then_0
      (EventDispatchers|UnbindEventfromOnDialogueEnded (stale Custom|Initiate%20Nightmare _dialoguecomponent) (delegate Custom|OnDialogueEnded_Event))
      (bind _returnvalue (UserInterface|CreateWidget "/Game/Blueprints/Widgets/WBP_Mission.WBP_Mission_C" 0 "Take the Lantern"))
      (UserInterface|Viewport|AddtoViewport _returnvalue 0))
    (:then_1
      (Utilities|FlowControl|Delay 5.0)
      (Widget|RemovefromParent _returnvalue))))

(event Custom|Stop%20Mystic%20Sound
  (Utilities|FlowControl|Sequence
    (:then_0
      (bind _mystic_sound (Variables|Default|GetMystic%20Sound)
        (:then
          _)
        (:else)))
    (:then_1
      (bind _low_hum_sfx (Variables|Default|GetLow%20Hum%20Sfx)
        (:then
          _)
        (:else))))
  (Audio|Components|Audio|FadeOut _mystic_sound 2.0 0.0 "Linear" :!class /Script/Engine.AudioComponent))

(event Custom|On%20Chapter%20Finished_Event
  ;[0.15 0.15 0.15 0.5 72] Initialize Player's State
  (bind _low_hum_sfx (Variables|Default|GetLow%20Hum%20Sfx)
    (:then
      (bind _mystic_sound (Variables|Default|GetMystic%20Sound)
        (:then
          (Audio|Components|Audio|Stop _mystic_sound))
        (:else)))
    (:else)))

(event EventBeginPlay
  ;[0.15 0.15 0.15 0.5 48] DEBUG
  (|CallParentFunction))

(fn ConstructionScript
  (|CallParentFunction))