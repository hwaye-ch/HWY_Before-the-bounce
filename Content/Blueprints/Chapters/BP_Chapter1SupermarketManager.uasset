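; Manager for the supermarket portion of Chapter 1, handling level setup, a customer sequence and the exit home.
; Initialization saves the chapter, moves the player to the supermarket spawn area, starts the toilet camera event and arms the shop start trigger.
; The Customer 2 sequence starts after a short delay.
; Going home fades the screen out, then calls a map teleport through the game instance.
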(event Custom|Initialize%20Level%201%20in%20Supermarket
  (bind _player_ref (Variables|Default|GetPlayer%20Ref))
  ;[0.15 0.15 0.15 0.5 72] Initialize Chapter 1
  (Default|SaveChapter (Variables|Default|GetGame%20Instance%20Ref) "NewEnumerator0")
  (Development|PrintString "Initializing Chapter 1 in Supermarket")
  (Utilities|FlowControl|Sequence
    (:then_0
      (bind _returnvalue (Actor|GetActorOfClass "/Game/Blueprints/Levels/SpawnArea_Chapter1SupermarketSpawn.SpawnArea_Chapter1SupermarketSpawn_C"))
      (Transformation|SetActorTransform _player_ref (Math|Transform|MakeTransform (.location (Transformation|GetActorTransform _returnvalue)) (.rotation (Transformation|GetActorTransform _returnvalue)) (Transformation|GetActorScale3D _player_ref)) false true))
    (:then_1
      (bind _returnvalue_2 (Actor|GetActorOfClass "/Game/Blueprints/LevelCameras/BP_ToiletCamera.BP_ToiletCamera_C"))
      (Default|StartChapter1Event _returnvalue_2))
    (:then_3
      (bind _returnvalue_3 (Actor|GetActorOfClass "/Game/Blueprints/Levels/Trigger_StartShop.Trigger_StartShop_C"))
      (Default|ActivateOverlapTrigger _returnvalue_3))))

(event Custom|Play%20Customer%202%20Sequence
  (Utilities|FlowControl|Delay 5.0)
  (bind _returnvalue (Actor|GetActorOfClass "/Game/Blueprints/Characters/BP_Customer2.BP_Customer2_C"))
  (Default|StartSequenceCustomer2 _returnvalue))

(event Custom|Proceed%20to%20Go%20Home
  (bind _bp_fadescreencomponent (Variables|Default|GetBP_FadeScreenComponent))
  (Default|FadeOut _bp_fadescreencomponent 5.0 (Variables|Default|GetPlayer%20Ref))
  (EventDispatchers|AssignOnExactFinish _bp_fadescreencomponent (delegate Custom|OnFadeOut_Event)))

(event Custom|OnFadeOut_Event
  (Default|CallTeleporttoMap (Variables|Default|GetGame%20Instance%20Ref) "NewEnumerator0"))

(fn ConstructionScript
  (|CallParentFunction))