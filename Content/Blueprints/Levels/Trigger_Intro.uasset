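; Level trigger that starts the intro sequence for the player's current chapter on overlap.
; Chapters 1–3 show auto dialogue with movement and look blocked, while chapter 7 starts rain through BP_Chapter7AManager.
; Chapter 6 shows an intro dialogue with an end-of-dialogue callback, supporting an event chain from Sarah's chat message to a choice about meeting Sarah.
; Choosing yes sets a determination flag on the game instance; no only prints a message.
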(event Custom|Listen%20to%20end%20Dialogue
  (bind _bp_displaychatdialogue (Variables|Default|GetBP_DisplayChatDialogue))
  (Development|PrintString "Tampilkan chat dari Sarah")
  (Utilities|FlowControl|Delay 2.0)
  (Default|ShowChatWidget _bp_displaychatdialogue "/Game/Textures/chat_sarah_2.chat_sarah_2")
  (EventDispatchers|BindEventtoOnAnimationFinished _bp_displaychatdialogue (delegate Custom|After%20Animation%20Finished)))

(event Custom|After%20Animation%20Finished
  (bind _bp_textrelatedcomponent (Variables|Default|GetBP_TextRelatedComponent))
  (bind _bp_choicedialoguecomponent (Variables|Default|GetBP_ChoiceDialogueComponent))
  (Development|PrintString "Animation Finished, Displaying Dialogue Choice")
  (bind _extracted_text (Default|ExtractText _bp_textrelatedcomponent "/Game/Dialogue/Item_Description.Item_Description" "is_attending_sarah"))
  (bind _extracted_text_2 (Default|ExtractText _bp_textrelatedcomponent "/Game/Dialogue/Item_Description.Item_Description" "reply_sarah_1"))
  (bind _extracted_text_3 (Default|ExtractText _bp_textrelatedcomponent "/Game/Dialogue/Item_Description.Item_Description" "reply_sarah_2"))
  (bind _choice_dialogue_component (Default|ConstructChoiceDialogue _bp_choicedialoguecomponent _extracted_text _extracted_text_2 _extracted_text_3))
  (Default|ShowChoiceDialogue _choice_dialogue_component (Variables|Default|GetPlayerRef))
  (EventDispatchers|BindEventtoExecuteOption _bp_choicedialoguecomponent (delegate Custom|Make%20a%20choice)))

(event Custom|Make%20a%20choice
  (params (Chosen%20Option :type E_ChoiceDialogue%20Enum :default "NewEnumerator0"))
  (switch Utilities|FlowControl|Switch|SwitchonE_ChoiceDialogue Chosen%20Option
    (:NewEnumerator0
      (Development|PrintString "You chose to meet Sarah")
      (Default|SetDetermination (Variables|Default|GetGame%20Instance%20Ref) "NewEnumerator1" true))
    (:NewEnumerator1
      (Development|PrintString "You ignore the fuck out of Sarah"))))

(event EventOnOverlapTrigger
  (bind _current_chapter (Default|GetCurrentChapter (Variables|Default|GetPlayerRef)))
  (switch int _current_chapter
    (:1
      (bind _dialoguecomponent (Default|ConstructDialogue (Variables|Default|GetBP_DialogueComponent) "ch1_intro" "/Game/Dialogue/Chapter1_Dialogue.Chapter1_Dialogue" true true))
      (Class|BPIDialogue|DisplayAutoDialogue(Message) _dialoguecomponent))
    (:2
      (bind _dialoguecomponent_2 (Default|ConstructDialogue (Variables|Default|GetBP_DialogueComponent) "ch2_intro" "/Game/Dialogue/Chapter2_Dialogue.Chapter2_Dialogue" true true))
      (Class|BPIDialogue|DisplayAutoDialogue(Message) _dialoguecomponent_2))
    (:3
      (bind _dialoguecomponent_3 (Default|ConstructDialogue (Variables|Default|GetBP_DialogueComponent) "ch3_intro" "/Game/Dialogue/Chapter3_Dialogue.Chapter3_Dialogue" true true))
      (Class|BPIDialogue|DisplayAutoDialogue(Message) _dialoguecomponent_3))
    (:6
      (bind _dialoguecomponent_4 (Default|ConstructDialogue (Variables|Default|GetBP_DialogueComponent) "ch6_intro_0" "/Game/Dialogue/Chapter6_Dialogue.Chapter6_Dialogue" true true))
      (Default|ShowDialogue _dialoguecomponent_4 (Variables|Default|GetPlayerRef) self)
      (EventDispatchers|BindEventtoOnDialogueEnded _dialoguecomponent_4 (EventDispatchers|CreateEvent :!event Custom|Listen%20to%20end%20Dialogue)))
    (:7
      (bind _returnvalue (Actor|GetActorOfClass "/Game/Blueprints/Items/BP_Chapter7AManager.BP_Chapter7AManager_C"))
      (Default|PlayRain _returnvalue))))

(fn ConstructionScript
  (|CallParentFunction))