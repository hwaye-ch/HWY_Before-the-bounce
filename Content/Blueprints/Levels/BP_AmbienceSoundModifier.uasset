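; BP_AmbienceSoundModifier is a box volume that changes the soundscape while the first-person character is inside it.
; Entering, or starting inside, ducks ambience or rain audio and increases footstep sound; leaving reverses this.
; Rain volume fades through a Timeline lerp, spawning the 2D rain sound and muting ambience if none exists.
; On low graphics settings it also switches EasyRain's camera-centric mode off inside and on outside.
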(event OnComponentBeginOverlap(Box)
  (params (OverlappedComponent :type Primitive%20Component%20Object%20Reference) (OtherActor :type Actor%20Object%20Reference) (OtherComp :type Primitive%20Component%20Object%20Reference) (OtherBodyIndex :type Integer) (bFromSweep :type Boolean) (SweepResult :type Hit%20Result%20Structure%20%28by%20ref%29))
  (bind _asbp_first_person_character (Utilities|Casting|CastToBP_FirstPersonCharacter OtherActor))
  (Variables|Default|SetAs%20BP%20First%20Person%20Character _asbp_first_person_character)
  (bind _ambiencesound (Variables|Default|GetAmbienceSound)
    (:then
      (Variables|Rain|GetIsRaining?
        (:then
          (CallFunction|SetRainVolume 0.4))
        (:else
          (Default|SetAmbienceVolume _ambiencesound 0.1)))
      (Default|IncreaseFootstepSound (Variables|Default|GetAs%20BP%20First%20Person%20Character))
      (CallFunction|SetLow-resRainSettings true))
    (:else)))

(event OnComponentEndOverlap(Box)
  (params (OverlappedComponent :type Primitive%20Component%20Object%20Reference) (OtherActor :type Actor%20Object%20Reference) (OtherComp :type Primitive%20Component%20Object%20Reference) (OtherBodyIndex :type Integer))
  (bind _asbp_first_person_character (Utilities|Casting|CastToBP_FirstPersonCharacter OtherActor))
  (Variables|Default|SetAs%20BP%20First%20Person%20Character _asbp_first_person_character)
  (bind _ambiencesound (Variables|Default|GetAmbienceSound)
    (:then
      (Variables|Rain|GetIsRaining?
        (:then
          (CallFunction|SetRainVolume 1.0))
        (:else
          (Default|SetAmbienceVolume _ambiencesound 1.0)))
      (Default|LowerFootstepSound (Variables|Default|GetAs%20BP%20First%20Person%20Character))
      (CallFunction|SetLow-resRainSettings false))
    (:else)))

(event Custom|Start%20Rain
  ;[0.15 0.15 0.15 0.5] Rain
  (bind _returnvalue (Audio|SpawnSound2D "/Game/Sounds/sfx_rain.sfx_rain" (Variables|Default|GetExpectedRainVolume) 1.0 0.0 0))
  (Variables|Default|SetRainSound _returnvalue)
  (CallFunction|SetRainVolume 1.0)
  (Default|SetAmbienceVolume (Variables|Default|GetAmbienceSound) 0.0))

(event Custom|Set%20Rain%20Volume
  (params (Expected%20Volume :type Float%20%28double-precision%29))
  ;[0.15 0.15 0.15 0.5] Rain
  (Variables|Default|SetExpectedRainVolume Expected%20Volume)
  (bind _rainsound (Variables|Default|GetRainSound)
    (:then
      (bind _newtrack_0 (Timeline|Timeline PlayFromStart)
        (:Update
          (Audio|Components|Audio|SetVolumeMultiplier _rainsound (Math|Float|Lerp (Variables|Default|GetCurrentRainVolume) (Variables|Default|GetExpectedRainVolume) _newtrack_0) :!class /Script/Engine.AudioComponent))
        (:Finished
          (Variables|Default|SetCurrentRainVolume (Variables|Default|GetExpectedRainVolume)))))
    (:else
      (CallFunction|StartRain))))

(event Custom|Set%20Low-res%20Rain%20Settings
  (params (In? :type Boolean))
  (bind _graphical_quality (Default|LoadGraphicSettings (Variables|Default|GetGame%20Instance%20Ref)))
  (if (Utilities|Enum|Equal(Enum) _graphical_quality (Variables|Default|GetLOW))
    (bind _easy_rain (Variables|Default|GetEasy%20Rain)
      (:then
        (Default|SetCameraCentric _easy_rain (not In?)))
      (:else))))

(event EventBeginPlay
  (|CallParentFunction)
  (Utilities|FlowControl|DelayUntilNextTick)
  (Utilities|FlowControl|Sequence
    (:then_0
      (bind _ashwy_game_instance (Utilities|Casting|CastToHwyGameInstance (Game|GetGameInstance)))
      (Variables|Default|SetGame%20Instance%20Ref _ashwy_game_instance))
    (:then_1
      (bind _asbp_first_person_character (Utilities|Casting|CastToBP_FirstPersonCharacter (Utilities|Array|Get(acopy) (Collision|GetOverlappingActors (Variables|Default|GetBox) "/Game/FirstPerson/Blueprints/BP_FirstPersonCharacter.BP_FirstPersonCharacter_C" :!class /Script/Engine.PrimitiveComponent))))
      (Default|SetAmbienceVolume (Variables|Default|GetAmbienceSound) 0.1)
      (Default|IncreaseFootstepSound _asbp_first_person_character)
      (CallFunction|SetLow-resRainSettings true))))

(fn ConstructionScript
  (|CallParentFunction))