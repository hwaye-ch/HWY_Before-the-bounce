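; A Chapter 2 level trigger that plays Mikey's calling dialogue and turns the player's view toward him.
; On overlap, it shows the dialogue with movement and look blocked, then starts the look-at after a short delay.
; A timeline interpolates control rotation toward the look-at component's target, feeding its alpha into RInterpTo as delta time.
; When the turn finishes, a temporary "Interact" mission widget appears after a pause.
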(event Custom|Look%20at%20Mikey
  (bind _playerref (Variables|Default|GetPlayerRef))
  (bind _firstpersoncamera (Variables|/Game/FirstPerson/Blueprints/BP_FirstPersonCharacter.BP_FirstPersonCharacter_C|GetFirstPersonCamera _playerref))
  (bind _lookatalpha (Timeline|Timeline Play)
    (:Update
      (Pawn|SetControlRotation (Game|GetPlayerController 0) (Math|Interpolation|RInterpTo (Transformation|GetWorldRotation _firstpersoncamera) (Math|Rotator|FindLookatRotation (Transformation|GetWorldLocation _firstpersoncamera) (Transformation|GetWorldLocation (Variables|/Script/Engine.Actor|GetRootComponent (Variables|/Game/Blueprints/Components/BP_LookAtComponent.BP_LookAtComponent_C|GetObjectToLookAt (Variables|Default|GetBP_LookAtComponent))))) _lookatalpha 5.0)))
    (:Finished
      (Utilities|FlowControl|Delay 2.0)
      (bind _returnvalue (UserInterface|CreateWidget "/Game/Blueprints/Widgets/WBP_Mission.WBP_Mission_C" 0 "Interact"))
      (UserInterface|Viewport|AddtoViewport _returnvalue 0)
      (Utilities|FlowControl|Delay 5.0)
      (Widget|RemovefromParent _returnvalue))))

(event EventOnOverlapTrigger
  (bind _dialoguecomponent (Default|ConstructDialogue (Variables|Default|GetBP_DialogueComponent) "ch2_mikey_calling" "/Game/Dialogue/Chapter2_Dialogue.Chapter2_Dialogue" true true))
  (Class|BPIDialogue|ShowDialogue(Message) _dialoguecomponent (Variables|Default|GetPlayerRef) self)
  (Utilities|FlowControl|Delay 1.0)
  (CallFunction|LookatMikey))

(fn ConstructionScript
  (|CallParentFunction))