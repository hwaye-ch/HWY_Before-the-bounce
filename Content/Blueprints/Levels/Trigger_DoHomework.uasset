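; Level trigger for the Chapter 3 homework beat that shows dialogue when its overlap event fires.
; On BeginPlay it binds to Mikey room events on two referenced actors, Enabler and Trigger.
; The Enabler event arms the overlap and loads the deadline dialogue.
; The Trigger event loads Mikey's dialogue with movement and look blocked, then arms the overlap a tick later.
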(event Custom|Activate%20Trigger
  (Development|PrintString "Trigger Dialogue Deadline Active!")
  (CallFunction|ActivateOverlapTrigger)
  (Default|ConstructDialogue (Variables|Default|GetBP_DialogueComponent) "ch3_deadline" "/Game/Dialogue/Chapter3_Dialogue.Chapter3_Dialogue" false false))

(event Custom|Activate%20Trigger%20Mikey%20Curiosity
  (Development|PrintString "Bounce Curiosity Trigger Activated")
  (Default|ConstructDialogue (Variables|Default|GetBP_DialogueComponent) "ch3_frommike" "/Game/Dialogue/Chapter3_Dialogue.Chapter3_Dialogue" true true)
  (Utilities|FlowControl|DelayUntilNextTick)
  (CallFunction|ActivateOverlapTrigger))

(event EventOnOverlapTrigger
  (Default|ShowDialogue (Variables|Default|GetBP_DialogueComponent) (Variables|Default|GetPlayerRef) self))

(event EventBeginPlay
  (|CallParentFunction)
  (bind _enabler (Variables|Default|GetEnabler)
    (:then
      (EventDispatchers|BindEventtoActivateMikeyRoomEvent _enabler (delegate Custom|Activate%20Trigger)))
    (:else
      _))
  (bind _trigger (Variables|Default|GetTrigger)
    (:then
      (EventDispatchers|BindEventtoTriggerMikeyRoomEvent _trigger (delegate Custom|Activate%20Trigger%20Mikey%20Curiosity)))
    (:else)))

(fn ConstructionScript
  (|CallParentFunction))