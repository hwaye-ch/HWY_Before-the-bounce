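; ColliderForbidden is a level trigger that shows dialogue when its overlap fires, apparently to mark a forbidden area.
; It calls ActivateOverlapTrigger on BeginPlay and again after every trigger, so it re-arms for repeated use.
; On overlap it prints a debug string, then passes the player reference and itself to BPDialogueComponent's ShowDialogue.
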(event EventBeginPlay
  (|CallParentFunction)
  (CallFunction|ActivateOverlapTrigger))

(event EventOnOverlapTrigger
  (Development|PrintString "ColliderForbidden Triggered")
  (Default|ShowDialogue (Variables|Default|GetBP_DialogueComponent) (Variables|Default|GetPlayerRef) self)
  (CallFunction|ActivateOverlapTrigger))

(fn ConstructionScript
  (|CallParentFunction))