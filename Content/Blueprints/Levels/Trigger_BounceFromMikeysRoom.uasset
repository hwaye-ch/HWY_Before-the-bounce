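; Level trigger that stages a scripted scare: a mysterious basketball sound draws the player's gaze while a TV starts playing.
; On overlap it messages the BP_MysteriousBasketballSound actor found at BeginPlay and plays the TV in parallel.
; After a delay it briefly locks movement and look, then a timeline blends control rotation toward the sound's location.
; Movement is re-enabled from the timeline's update.
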(event EventOnOverlapTrigger
  (bind _playerref (Variables|Default|GetPlayerRef))
  (bind _firstpersoncamera (Variables|/Game/FirstPerson/Blueprints/BP_FirstPersonCharacter.BP_FirstPersonCharacter_C|GetFirstPersonCamera _playerref))
  (Utilities|FlowControl|Sequence
    (:then_0
      (bind _basketballsoundtrigger (Variables|Default|GetBasketBallSoundTrigger)
        (:then
          (Class|BPIExecutable|Execute(Message) _basketballsoundtrigger)
          (Utilities|FlowControl|Delay 2.0)
          (Default|DisableMovementandLook (Variables|Default|GetPlayerRef))
          (Utilities|FlowControl|Delay 1.0)
          (Default|EnableLook (Variables|Default|GetPlayerRef))
          (bind _newtrack_0 (Timeline|Timeline Play)
            (:Update
              (Pawn|SetControlRotation (Game|GetPlayerController 0) (Math|Rotator|Lerp(Rotator) (Transformation|GetWorldRotation _firstpersoncamera) (Math|Rotator|FindLookatRotation (Transformation|GetWorldLocation _firstpersoncamera) (Variables|Default|GetSoundLocation)) _newtrack_0))
              (Default|EnableMovement (Variables|Default|GetPlayerRef)))))
        (:else)))
    (:then_1
      (bind _tv (Variables|Default|GetTV)
        (:then
          (Default|PlayTV _tv))
        (:else)))))

(event EventBeginPlay
  (|CallParentFunction)
  (bind _returnvalue (Actor|GetActorOfClass "/Game/Blueprints/EventItems/BP_MysteriousBasketballSound.BP_MysteriousBasketballSound_C"))
  (bind _output_get (Variables|Default|SetBasketBallSoundTrigger _returnvalue))
  (Variables|Default|SetSoundLocation (Transformation|GetActorLocation _output_get)))

(fn ConstructionScript
  (|CallParentFunction))