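; Level trigger for the start of the good ending that shuts the player out of or into Mikey's door and sets a new objective.
; On BeginPlay it caches the BP_MikeysDoor actor found in the level.
; Its overlap event closes and locks that door, then shows a WBP_Mission "Explore the house" prompt and removes it after a short delay.
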(event EventBeginPlay
  (|CallParentFunction)
  (bind _returnvalue (Actor|GetActorOfClass "/Game/Blueprints/EventItems/BP_MikeysDoor.BP_MikeysDoor_C"))
  (Variables|Default|SetMIkey'sDoor _returnvalue))

(event EventOnOverlapTrigger
  (bind _mikey_sdoor (Variables|Default|GetMIkey'sDoor)
    (:then
      (Default|SetDoorClosed _mikey_sdoor)
      (Variables|/Game/Blueprints/ModularItems/BP_InteractableDoor.BP_InteractableDoor_C|SetIsLocked _mikey_sdoor true)
      (bind _returnvalue (UserInterface|CreateWidget "/Game/Blueprints/Widgets/WBP_Mission.WBP_Mission_C" 0 "Explore the house"))
      (UserInterface|Viewport|AddtoViewport _returnvalue 0)
      (Utilities|FlowControl|Delay 5.0)
      (Widget|RemovefromParent _returnvalue))
    (:else)))

(fn ConstructionScript)