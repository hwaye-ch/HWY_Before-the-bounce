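; Level trigger that starts the car chase when its overlap event fires.
; It reveals Mikey's mesh on the car and plays an intro level sequence while player movement and look are disabled.
; When the sequence ends, it turns the player toward the car, starts suspense music and the chase, and enables panic and running with a timed mission hint.
; The car's player-death event fades out and stops the music.
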(event Custom|On%20Finished%20Animation
  (bind _playerref (Variables|Default|GetPlayerRef))
  (Development|PrintString "Animation Finished, Player look at the car! 
")
  (Pawn|SetControlRotation (Game|GetPlayerController 0) (Math|Rotator|FindLookatRotation (Transformation|GetActorLocation (Variables|Default|GetPlayerRef)) (Transformation|GetActorLocation (Variables|Default|GetCarToLookAt))))
  (Audio|Components|Audio|Play (Variables|Default|GetSuspensefulMusic) 0.0)
  (Default|CallCarStartChasing)
  (Default|EnableLookandMovement (Variables|Default|GetPlayerRef))
  (Variables|/Game/FirstPerson/Blueprints/BP_FirstPersonCharacter.BP_FirstPersonCharacter_C|SetIsPanic _playerref true)
  (Variables|/Game/FirstPerson/Blueprints/BP_FirstPersonCharacter.BP_FirstPersonCharacter_C|SetCan%20Run? _playerref true)
  (bind _returnvalue (UserInterface|CreateWidget "/Game/Blueprints/Widgets/WBP_Mission.WBP_Mission_C" 0 "Hold [Shift] to Run"))
  (UserInterface|Viewport|AddtoViewport _returnvalue 0)
  (Utilities|FlowControl|Delay 4.0)
  (Widget|RemovefromParent _returnvalue))

(event Custom|Stop%20Music
  (bind _suspensefulmusic (Variables|Default|GetSuspensefulMusic))
  (Audio|Components|Audio|FadeOut _suspensefulmusic 1.0 0.0 "Linear" :!class /Script/Engine.AudioComponent)
  (Utilities|FlowControl|Delay 1.0)
  (Audio|Components|Audio|Stop _suspensefulmusic))

(event EventBeginPlay
  (|CallParentFunction) ; This node is disabled and will not be called.\nDrag off pins to build functionality.
)

(event EventOnOverlapTrigger
  (bind _returnvalue (Sequencer|Player|CreateLevelSequencePlayer "/Game/Animation/Anim_CarStartedToChase.Anim_CarStartedToChase"))
  (Rendering|SetVisibility (Variables|/Game/Objects/BP_ChasingCar.BP_ChasingCar_C|GetMikeyMesh (Variables|Default|GetCarToLookAt)) true true)
  (Variables|Default|SetSequencePlayer _returnvalue)
  (Sequencer|Player|Play (Variables|Default|GetSequencePlayer) :!class /Script/MovieScene.MovieSceneSequencePlayer)
  (EventDispatchers|BindEventtoOnFinished _returnvalue (delegate Custom|On%20Finished%20Animation))
  (Default|DisableMovementandLook (Variables|Default|GetPlayerRef))
  (EventDispatchers|BindEventtoPlayerDead (Variables|Default|GetCarToLookAt) (delegate Custom|Stop%20Music)))

(fn ConstructionScript
  (|CallParentFunction))