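; Welcome trigger volume that plays an opening dialogue chosen by the player's current chapter when its overlap event fires.
; Chapters 1, 8 and the default (shared with 2) block movement and look, while chapter 3 shows auto dialogue and starts trash counting.
; Chapter 1 also enables the Kulkas, and the default adds an eerie sound.
; Dialogue-end events show timed mission widgets, with chapter 8's also activating the TV and sofa.
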(event Custom|OnDialogueEnded_Event
  (Utilities|FlowControl|Delay 1.0)
  (Utilities|FlowControl|Sequence
    (:then_0
      (bind _returnvalue (UserInterface|CreateWidget "/Game/Blueprints/Widgets/WBP_Mission.WBP_Mission_C" 0 "Relax and Watch TV"))
      (UserInterface|Viewport|AddtoViewport _returnvalue 0)
      (Utilities|FlowControl|Delay 5.0)
      (Widget|RemovefromParent _returnvalue))
    (:then_1
      (bind _tv (Variables|Default|GetTV)
        (:then
          (Variables|/Game/Blueprints/EventItems/BP_Television.BP_Television_C|SetIs%20Enabled? _tv true))
        (:else)))
    (:then_2
      (bind _sofa (Variables|Default|GetSofa)
        (:then
          (Variables|/Game/Blueprints/EventItems/BP_Sofa.BP_Sofa_C|SetIs%20Event%20Ready? _sofa true))
        (:else)))))

(event Custom|OnDialogueEnded_Event_0
  (Utilities|FlowControl|Delay 2.0)
  (bind _returnvalue (UserInterface|CreateWidget "/Game/Blueprints/Widgets/WBP_Mission.WBP_Mission_C" 0 "Eat"))
  (UserInterface|Viewport|AddtoViewport _returnvalue 0)
  (Utilities|FlowControl|Delay 5.0)
  (Widget|RemovefromParent _returnvalue))

(event EventOnOverlapTrigger
  (bind _bp_dialoguecomponent (Variables|Default|GetBP_DialogueComponent))
  (bind _current_chapter (Default|GetCurrentChapter (Variables|Default|GetPlayerRef)))
  (switch int _current_chapter
    (:Default
      (bind _dialoguecomponent (Default|ConstructDialogue (Variables|Default|GetBP_DialogueComponent) "ch2_welcome" "/Game/Dialogue/Chapter2_Dialogue.Chapter2_Dialogue" true true :!label _label))
      (Default|ShowDialogue _dialoguecomponent (Variables|Default|GetPlayerRef) self)
      (Audio|SpawnSound2D "/Game/Sounds/sfx_eerie.sfx_eerie" 2.0 1.0 0.0 0))
    (:1
      (bind _dialoguecomponent_2 (Default|ConstructDialogue (Variables|Default|GetBP_DialogueComponent) "ch1_welcome" "/Game/Dialogue/Chapter1_Dialogue.Chapter1_Dialogue" true true))
      (Default|ShowDialogue _dialoguecomponent_2 (Variables|Default|GetPlayerRef) self)
      (Default|CallEnableKulkas)
      (EventDispatchers|AssignOnDialogueEnded _dialoguecomponent_2 (delegate Custom|OnDialogueEnded_Event_0)))
    (:2
      (goto _label))
    (:3
      (Default|CallStartCountingTrash)
      (bind _dialoguecomponent_3 (Default|ConstructDialogue (Variables|Default|GetBP_DialogueComponent) "ch3_welcome" "/Game/Dialogue/Chapter3_Dialogue.Chapter3_Dialogue" false false))
      (Utilities|FlowControl|DelayUntilNextTick)
      (Class|BPIDialogue|DisplayAutoDialogue(Message) _dialoguecomponent_3))
    (:8
      (bind _dialoguecomponent_4 (Default|ConstructDialogue _bp_dialoguecomponent "ch7_nonton" "/Game/Dialogue/Chapter7_Dialogue.Chapter7_Dialogue" true true))
      (Default|ShowDialogue _dialoguecomponent_4 (Variables|Default|GetPlayerRef) self)
      (EventDispatchers|AssignOnDialogueEnded _bp_dialoguecomponent (delegate Custom|OnDialogueEnded_Event)))))

(fn ConstructionScript)

(fn ShowDialogue
  (params (PlayerPref :type BP%20First%20Person%20Character%20Object%20Reference) (DialogueActorTrigger :type Actor%20Object%20Reference))
  (return))