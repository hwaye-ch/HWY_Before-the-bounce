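; Level trigger that runs the car crash scene, playing a level sequence while moving the player to the basketball court with movement and look disabled.
; When the sequence ends, it restores look, moves the chasing car to the explosion area, silences it and its music, and hides some meshes.
; A delayed fade-out saves and plays one of two chapters by Determination.
; A separate event staggers explosion, fire and sound.
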(event Custom|Activate
  (Components|Activation|SetActive (Variables|/Game/Blueprints/EventItems/Blueprint_Effect_Explosion.Blueprint_Effect_Explosion_C|GetP_Explosion (Variables|Default|GetExplosion)) true false)
  (Utilities|FlowControl|Delay 1.0)
  (Components|Activation|SetActive (Variables|/Game/Blueprints/EventItems/Blueprint_Effect_Fire.Blueprint_Effect_Fire_C|GetP_Fire (Variables|Default|GetFire)) true false))

(event Custom|OnFadeOut_Event
  (bind _returnvalue (Default|GetDetermination (Variables|Default|GetGame%20Instance%20Ref)))
  (if _returnvalue
    (Default|SaveChapter (Variables|Default|GetGame%20Instance%20Ref) "NewEnumerator6")
    (Default|PlayChapter (Variables|Default|GetPlayerRef) 7)
    (else
      (Default|SaveChapter (Variables|Default|GetGame%20Instance%20Ref) "NewEnumerator7")
      (Default|PlayChapter (Variables|Default|GetPlayerRef) 8))))

(event Custom|OnFinishedCutscene
  (bind _the_car (Variables|Default|GetThe%20Car))
  (bind _bp_fadescreencomponent (Variables|Default|GetBP_FadeScreenComponent))
  (Default|EnableLook (Variables|Default|GetPlayerRef))
  (Transformation|SetActorLocation (Variables|Default|GetThe%20Car) (Transformation|GetActorLocation (Variables|Default|GetExplossionArea)) false true)
  (Audio|Components|Audio|Stop (Variables|/Game/Objects/BP_ChasingCar.BP_ChasingCar_C|Getsfx_car-horn _the_car))
  (bind _returnvalue (Actor|GetActorOfClass "/Game/Blueprints/Levels/Trigger_ChasingCar.Trigger_ChasingCar_C"))
  (Default|StopMusic _returnvalue)
  (Rendering|SetVisibility (Variables|/Game/Objects/BP_ChasingCar.BP_ChasingCar_C|GetMikeyMesh _the_car) false true)
  (Utilities|FlowControl|Delay 7.0)
  (Default|FadeOut _bp_fadescreencomponent 1e+01 (Variables|Default|GetPlayerRef))
  (EventDispatchers|AssignOnFadeOut _bp_fadescreencomponent (delegate Custom|OnFadeOut_Event)))

(event Custom|SpawnExplossion
  (CallFunction|Activate)
  (Utilities|FlowControl|Delay 2.0)
  (Components|Activation|Activate (Variables|/Game/Blueprints/Levels/SpawnArea_Explossion.SpawnArea_Explossion_C|Getsfx_explossion (Variables|Default|GetExplossionArea)) false))

(event EventBeginPlay
  (|CallParentFunction)
  (bind _returnvalue (Actor|GetActorOfClass "/Game/Objects/BP_ChasingCar.BP_ChasingCar_C"))
  (Variables|Default|SetThe%20Car _returnvalue)
  (bind _returnvalue_2 (Actor|GetActorOfClass "/Game/Blueprints/Levels/SpawnArea_Explossion.SpawnArea_Explossion_C"))
  (Variables|Default|SetExplossionArea _returnvalue_2)
  (bind _returnvalue_3 (Actor|GetActorOfClass "/Game/Blueprints/EventItems/Blueprint_Effect_Explosion.Blueprint_Effect_Explosion_C"))
  (Variables|Default|SetExplosion _returnvalue_3)
  (bind _returnvalue_4 (Actor|GetActorOfClass "/Game/Blueprints/EventItems/Blueprint_Effect_Fire.Blueprint_Effect_Fire_C"))
  (Variables|Default|SetFire _returnvalue_4))

(event EventOnOverlapTrigger
  (Development|PrintString "Playing Cutscene" true true "(R=1.000000,G=0.000000,B=0.175299,A=1.000000)")
  (Variables|/Game/FirstPerson/Blueprints/BP_FirstPersonCharacter.BP_FirstPersonCharacter_C|SetIsPanic (Variables|Default|GetPlayerRef) false)
  (bind _returnvalue (Sequencer|Player|CreateLevelSequencePlayer "/Game/Animation/Anim_BasketballScene.Anim_BasketballScene"))
  (Sequencer|Player|Play _returnvalue :!class /Script/MovieScene.MovieSceneSequencePlayer)
  (Default|DisableMovementandLook (Variables|Default|GetPlayerRef))
  (EventDispatchers|BindEventtoOnFinished _returnvalue (delegate Custom|OnFinishedCutscene))
  (bind _returnvalue_2 (Actor|GetActorOfClass "/Game/Blueprints/Levels/SpawnArea_BasketballCourt.SpawnArea_BasketballCourt_C"))
  (Transformation|SetActorLocation (Variables|Default|GetPlayerRef) (Transformation|GetActorLocation _returnvalue_2) false false)
  (Pawn|SetControlRotation (Game|GetPlayerController 0) (Math|Rotator|FindLookatRotation (Math|Vector|GetForwardVector (Variables|/Game/FirstPerson/Blueprints/BP_FirstPersonCharacter.BP_FirstPersonCharacter_C|GetFirstPersonCamera (Variables|Default|GetPlayerRef))) (Transformation|GetActorLocation (Variables|Default|GetExplossionArea)))))

(fn ConstructionScript
  (|CallParentFunction))