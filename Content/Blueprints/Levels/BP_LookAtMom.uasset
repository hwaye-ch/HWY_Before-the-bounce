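; BP_LookAtMom is a level event that fires a one-time jumpscare when the player looks at the mom on the bed, then moves on to chapter 6.
; Once ready, Tick checks the player's HitActor for the "Mom" tag behind a DoOnce.
; Timelines turn the bed camera toward BP_MomOnBed, then fade her audio, while scare sounds play and a delayed black screen leads to PlayChapter.
; The father-on-bed call is unconnected.
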(event Custom|FadeOutListener_Event
  (Default|PlayChapter (Variables|Default|GetPlayerRef) 6)
  (Utilities|FlowControl|DelayUntilNextTick)
  (EventDispatchers|UnbindallEventsfromOnFadeOut (Variables|Default|GetBP_FadeScreenComponent)))

(event EventBeginPlay
  (|CallParentFunction))

(event EventTick
  (params (DeltaSeconds :type Float%20%28single-precision%29))
  (bind _bp_fadescreencomponent (Variables|Default|GetBP_FadeScreenComponent))
  (Utilities|FlowControl|DelayUntilNextTick)
  (Variables|Default|GetIsReady?
    (:then
      (bind _hit_actor (Variables|/Game/FirstPerson/Blueprints/BP_FirstPersonCharacter.BP_FirstPersonCharacter_C|GetHit%20Actor (Variables|Default|GetPlayerRef))
        (:then
          (if (Actor|ActorHasTag _hit_actor "Mom")
            (Utilities|FlowControl|DoOnce false
              (:Completed
                (Utilities|FlowControl|Sequence
                  (:then_0
                    (bind _returnvalue (Actor|GetActorOfClass "/Game/Blueprints/EventItems/BP_MomOnBed.BP_MomOnBed_C"))
                    (Variables|Default|SetMom _returnvalue)
                    (bind _returnvalue_2 (Actor|GetActorOfClass "/Game/Blueprints/LevelCameras/BP_BedCamera.BP_BedCamera_C"))
                    (bind _newtrack_0 (Timeline|Timeline PlayFromStart)
                      (:Update
                        (Transformation|SetWorldRotation (Variables|/Game/Blueprints/ModularItems/BP_LevelCamera.BP_LevelCamera_C|GetCamera _returnvalue_2) (Math|Rotator|Lerp(Rotator) (Transformation|GetWorldRotation (Variables|/Game/Blueprints/ModularItems/BP_LevelCamera.BP_LevelCamera_C|GetCamera _returnvalue_2)) (Math|Rotator|FindLookatRotation (Transformation|GetWorldLocation (Variables|/Game/Blueprints/ModularItems/BP_LevelCamera.BP_LevelCamera_C|GetCamera _returnvalue_2)) (Transformation|GetActorLocation (Variables|Default|GetMom))) _newtrack_0) false false))
                      (:Finished
                        (Default|SetLook _returnvalue_2 false)
                        (Utilities|FlowControl|Delay 1.5)
                        (bind _newtrack_0_2 (Timeline|Timeline_0 Play)
                          (:Update
                            (Audio|Components|Audio|SetVolumeMultiplier (Variables|/Game/Blueprints/EventItems/BP_MomOnBed.BP_MomOnBed_C|Getsfx_mom (Variables|Default|GetMom)) (Math|Float|Lerp 1.0 0.0 _newtrack_0_2) :!class /Script/Engine.AudioComponent))))))
                  (:then_1
                    (Audio|SpawnSound2D "/Game/Sounds/sfx_jumpscare-mom.sfx_jumpscare-mom" 3.0 1.0 0.0 0)
                    (Audio|SpawnSound2D "/Game/Sounds/sfx_jumpscare4.sfx_jumpscare4" 1.0 1.0 0.0 0)
                    (Audio|SpawnSound2D "/Game/Sounds/sfx_croak.sfx_croak" 2.0 1.0 0.0 0)
                    (Utilities|FlowControl|Delay 1.5)
                    (Default|ShowBlackScreen _bp_fadescreencomponent 15.0 (Variables|Default|GetPlayerRef))
                    (EventDispatchers|BindEventtoOnBlackScreenFinished _bp_fadescreencomponent (delegate Custom|FadeOutListener_Event))))))))
        (:else)))
    (:else)))

(fn ConstructionScript
  (|CallParentFunction))