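; BP_AmbienceSound is a level actor that controls night and horror background audio.
; It spawns the night ambience at its own location, with timelines fading it to a requested volume or out to silence.
; Setting a volume spawns the ambience if none is valid.
; Horror background plays as a separate 2D sound, instantly setting any active night ambience to a minimum volume.
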(event Custom|Spawn%20Night%20Ambience
  (params (Initial%20Volume :type Float%20%28double-precision%29))
  (bind _output_get (Variables|Default|SetCurrentVolume Initial%20Volume))
  (bind _returnvalue (Audio|SpawnSoundatLocation "/Game/Sounds/sfx_night-ambience.sfx_night-ambience" (Transformation|GetActorLocation) "0, 0, 0" _output_get 1.0 0.0 0 0))
  (Variables|Default|SetNight%20Ambience _returnvalue))

(event Custom|Play%20Horror%20Bg%20Sound
  (bind _returnvalue (Audio|SpawnSound2D "/Game/Sounds/sfx_soundscapehorror.sfx_soundscapehorror" 0.075 1.0 0.0 0))
  (Variables|Default|SetHorrorAmbience _returnvalue)
  (bind _night_ambience (Variables|Default|GetNight%20Ambience)
    (:then
      (Audio|Components|Audio|SetVolumeMultiplier _night_ambience (Variables|Default|GetMinVolume) :!class /Script/Engine.AudioComponent))
    (:else)))

(event Custom|Stop%20the%20Ambience%20Sound
  (bind _night_ambience (Variables|Default|GetNight%20Ambience)
    (:then
      (bind _newtrack_0 (Timeline|Timeline_0 Play)
        (:Update
          (Audio|Components|Audio|SetVolumeMultiplier _night_ambience (Math|Float|Lerp (Variables|Default|GetLowVolume) 0.0 _newtrack_0) :!class /Script/Engine.AudioComponent))))
    (:else)))

(event Custom|Set%20Ambience%20Volume
  (params (Volume :type Float%20%28double-precision%29))
  (bind _output_get (Variables|Default|SetDesiredVolume Volume))
  (bind _night_ambience (Variables|Default|GetNight%20Ambience)
    (:then
      (bind _newtrack_0 (Timeline|Timeline PlayFromStart)
        (:Update
          (Audio|Components|Audio|SetVolumeMultiplier _night_ambience (Math|Float|Lerp (Variables|Default|GetCurrentVolume) (Variables|Default|GetDesiredVolume) _newtrack_0) :!class /Script/Engine.AudioComponent))
        (:Finished
          (Variables|Default|SetCurrentVolume (Variables|Default|GetDesiredVolume) :!label _label))))
    (:else
      (CallFunction|SpawnNightAmbience _output_get)
      (goto _label))))

(fn ConstructionScript
  (|CallParentFunction))