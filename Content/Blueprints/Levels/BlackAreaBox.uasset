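; BlackAreaBox is a level actor that acts as a black enclosure, hidden and non-colliding until enabled.
; BeginPlay hides the root StaticMesh with its children and disables collision on five meshes.
; EnableBlackBox reveals them, restores query and physics collision, and sets IsEventReady.
; The chapter 7B manager lookup is unused, as ChapterManager is set to None, and the Box overlap only casts to the player character.
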(event OnComponentBeginOverlap(Box)
  (params (OverlappedComponent :type Primitive%20Component%20Object%20Reference) (OtherActor :type Actor%20Object%20Reference) (OtherComp :type Primitive%20Component%20Object%20Reference) (OtherBodyIndex :type Integer) (bFromSweep :type Boolean) (SweepResult :type Hit%20Result%20Structure%20%28by%20ref%29))
  (Utilities|Casting|CastToBP_FirstPersonCharacter OtherActor))

(event Custom|Enable%20Black%20Box
  (Rendering|SetVisibility (Variables|Default|GetStaticMesh) true true)
  (Collision|SetCollisionEnabled (Variables|Default|GetStaticMesh) "QueryAndPhysics")
  (Variables|Default|SetIsEventReady? true))

(event EventBeginPlay
  (|CallParentFunction)
  (Rendering|SetVisibility (Variables|Default|GetStaticMesh) false true)
  (Actor|GetActorOfClass "/Game/Blueprints/Chapters/BP_Chapter7BManager.BP_Chapter7BManager_C")
  (Variables|Default|SetChapterManager 0)
  (Collision|SetCollisionEnabled (Variables|Default|GetStaticMesh) "NoCollision"))

(fn ConstructionScript
  (|CallParentFunction))