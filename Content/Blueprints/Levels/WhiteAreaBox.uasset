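; WhiteAreaBox is a Chapter 7A set piece that stays hidden and non-colliding until the chapter manager's MoveNPCs event fires.
; On BeginPlay it finds BP_Chapter7AManager and binds that event, which reveals the meshes, enables their collision and flags the box ready.
; When the first-person character then overlaps the trigger box, it freezes player movement, tells the manager to lock the door after a delay, then restores movement.
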(event OnComponentBeginOverlap(Box)
  (params (OverlappedComponent :type Primitive%20Component%20Object%20Reference) (OtherActor :type Actor%20Object%20Reference) (OtherComp :type Primitive%20Component%20Object%20Reference) (OtherBodyIndex :type Integer) (bFromSweep :type Boolean) (SweepResult :type Hit%20Result%20Structure%20%28by%20ref%29))
  (Utilities|Casting|CastToBP_FirstPersonCharacter OtherActor)
  (Variables|Default|GetIsEventReady?
    (:then
      (Development|PrintString "Closing")
      (Default|DisableMovement (Variables|Default|GetPlayerRef))
      (Utilities|FlowControl|Delay 1e+01)
      (Default|CallLocktheDoor (Variables|Default|GetChapterManager))
      (Utilities|FlowControl|Delay 2.0)
      (Default|EnableMovement (Variables|Default|GetPlayerRef)))
    (:else)))

(event Custom|MoveNPCs_Event
  (Rendering|SetVisibility (Variables|Default|GetStaticMesh) true true)
  (Collision|SetCollisionEnabled (Variables|Default|GetStaticMesh) "QueryAndPhysics")
  (Variables|Default|SetIsEventReady? true))

(event EventBeginPlay
  (|CallParentFunction)
  (Rendering|SetVisibility (Variables|Default|GetStaticMesh) false true)
  (bind _returnvalue (Actor|GetActorOfClass "/Game/Blueprints/Chapters/BP_Chapter7AManager.BP_Chapter7AManager_C"))
  (bind _output_get (Variables|Default|SetChapterManager _returnvalue))
  (EventDispatchers|AssignMoveNPCs _output_get (delegate Custom|MoveNPCs_Event))
  (Collision|SetCollisionEnabled (Variables|Default|GetStaticMesh) "NoCollision"))

(fn ConstructionScript
  (|CallParentFunction))