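; BP_TableCamera is a level camera for the scene where the player wakes from a nightmare at a table.
; A bound enabler event triggers the wake-up: it fades in, activates the camera, teleports the player to the table spawn area and shows Chapter 4 dialogue.
; When dialogue ends, the interact button takes priority to trigger getting up, which fades the screen, plays a chair sound and restores player control.
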(event Custom|Wake%20Up
  (params (PlayerPref :type BP%20First%20Person%20Character%20Object%20Reference))
  (bind _bp_dialoguecomponent (Variables|Default|GetBP_DialogueComponent))
  (Variables|Default|SetPlayer%20Ref PlayerPref)
  (Default|Fadein (Variables|Default|GetBP_FadeScreenComponent) (Variables|Default|GetPlayer%20Ref))
  (CallFunction|InitializeLevelCamera (Variables|Default|GetPlayer%20Ref) 0.0)
  (CallFunction|MoveCharacterNearTable)
  (bind _dialoguecomponent (Default|ConstructDialogue _bp_dialoguecomponent "ch4_waken_0" "/Game/Dialogue/Chapter4_Dialogue.Chapter4_Dialogue" false false))
  (Default|ShowDialogue _dialoguecomponent (Variables|Default|GetPlayer%20Ref) self)
  (EventDispatchers|AssignOnDialogueEnded _bp_dialoguecomponent (delegate Custom|OnDialogueEnded_Event)))

(event Custom|Move%20Character%20near%20Table
  (Transformation|SetActorLocationAndRotation (Variables|Default|GetPlayer%20Ref) (Transformation|GetActorLocation (Variables|Default|GetSpawnAreaTable)) (Transformation|GetActorRotation) false true))

(event Custom|Get%20Up
  (Default|FadeEvent (Variables|Default|GetBP_FadeScreenComponent) 4.0 (Variables|Default|GetPlayer%20Ref) 0.0)
  (Utilities|FlowControl|Delay 2.0)
  (Default|EnableLookandMovement (Variables|Default|GetPlayer%20Ref))
  (CallFunction|EndLevelCamera)
  (Audio|PlaySound2D "/Game/Sounds/sfx_moving-chair.sfx_moving-chair" 1.0 1.0 0.0 0 0)
  (CallFunction|MoveCharacterNearTable)
  (Default|UnsetInteractButtonPriority (Variables|Default|GetPlayer%20Ref)))

(event Custom|OnDialogueEnded_Event
  (Default|SetInteractButtonPriority (Variables|Default|GetPlayer%20Ref))
  (EventDispatchers|BindEventtoInteractButtonPressed (Variables|Default|GetPlayer%20Ref) (delegate Custom|Get%20Up)))

(event EventInitializeLevelCamera
  (params (Player%20Ref :type BP%20First%20Person%20Character%20Object%20Reference) (Blend%20Time :type Float%20%28double-precision%29))
  (|CallParentFunction Player%20Ref Blend%20Time)
  (CallFunction|MoveCharacterNearTable))

(event EventBeginPlay
  (bind _wakeupeventenabler (Variables|Default|GetWakeUpEventEnabler)
    (:then
      (EventDispatchers|BindEventtoWakeUpfromNightmare _wakeupeventenabler (delegate Custom|Wake%20Up))
      (Utilities|FlowControl|Delay 2.0))
    (:else)))

(fn ConstructionScript
  (|CallParentFunction))