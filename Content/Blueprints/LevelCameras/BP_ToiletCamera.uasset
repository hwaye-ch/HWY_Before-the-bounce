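; Level camera Blueprint that plays the Chapter 1 opening sequence from a toilet viewpoint.
; StartChapter1Event starts the camera and fades in from black, then locks player input and shows the first dialogue after a delay.
; When dialogue ends, it triggers the front door's welcome sound, then runs a fade.
; Once that fade finishes, it plays a flush sound, ends the camera and unlocks the door tagged "toilet1", with steps chained through component delegates.
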(event OnDialogueEnded(BP_DialogueComponent)
  (bind _bp_fadescreencomponent (Variables|Default|GetBP_FadeScreenComponent))
  (Default|DisableMovementandLook (Variables|Default|GetPlayer%20Ref))
  (Utilities|FlowControl|Delay 5.0)
  (bind _returnvalue (Actor|GetActorOfClass "/Game/Convenience_Store/Blueprints/BP_Front_Door.BP_Front_Door_C"))
  (Default|PlayWelcomeSound _returnvalue)
  (Utilities|FlowControl|Delay 5.0)
  (EventDispatchers|AssignOnFadeEventFinished _bp_fadescreencomponent (delegate Custom|OnFadeEventFinished_Event))
  (Default|FadeEvent _bp_fadescreencomponent 5.0 (Variables|Default|GetPlayer%20Ref) 2.0))

(event Custom|OnFadeIn_Event
  (Default|DisableMovementandLook (Variables|Default|GetPlayer%20Ref))
  (Utilities|FlowControl|Delay 5.0)
  (bind _dialoguecomponent (Default|ConstructDialogue (Variables|Default|GetBP_DialogueComponent) "ch1_first" "/Game/Dialogue/Chapter1_Dialogue.Chapter1_Dialogue" true true))
  (Default|ShowDialogue _dialoguecomponent (Variables|Default|GetPlayer%20Ref) self))

(event Custom|OnFadeEventFinished_Event
  (Audio|Components|Audio|Play (Variables|Default|Getsfx_flush) 0.0)
  (CallFunction|EndLevelCamera)
  (bind _outactors (Actor|GetAllActorswithTag "toilet1"))
  (bind _asbp_door (Utilities|Casting|CastToBP_Door (Utilities|Array|Get(acopy) _outactors)))
  (Variables|/Game/Convenience_Store/Blueprints/BP_Door.BP_Door_C|SetIsLocked? _asbp_door false))

(event Custom|Start%20Chapter%201%20Event
  (bind _bp_fadescreencomponent (Variables|Default|GetBP_FadeScreenComponent))
  (CallFunction|InitializeLevelCamera (Variables|Default|GetPlayer%20Ref) 0.0 true)
  (Default|BlackScreenThenFadein _bp_fadescreencomponent (Variables|Default|GetPlayer%20Ref) 4.0)
  (EventDispatchers|AssignOnFadein _bp_fadescreencomponent (delegate Custom|OnFadeIn_Event)))

(fn ConstructionScript
  (|CallParentFunction))