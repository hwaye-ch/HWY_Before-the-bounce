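; BP_WindowCamera is an interactable Chapter 7 window viewpoint that blends the player into a child-actor level camera.
; While the story event is ready, interacting once stops the TV, plays window dialogue and has BP_Chapter7AManager move NPCs.
; Exit on the interact button is bound after dialogue ends, or immediately without the event.
; The first event exit triggers sad audio, hides the crutch and briefly shows a "Talk" mission prompt.
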(event Custom|InteractButtonPressed_Event
  (Default|EndLevelCamera (Variables|Default|GetAs%20BP%20Level%20Camera))
  (Variables|/Game/FirstPerson/Blueprints/BP_FirstPersonCharacter.BP_FirstPersonCharacter_C|SetIsInteractButtonPriority? (Variables|Default|GetPlayerRef) false)
  (EventDispatchers|UnbindallEventsfromInteractButtonPressed (Variables|Default|GetPlayerRef))
  (Variables|Default|GetIsEventReady?
    (:then
      (Utilities|FlowControl|DoOnce false
        (:Completed
          (Variables|Default|SetIsEventReady? false)
          (Utilities|FlowControl|Delay 2.0)
          (Utilities|FlowControl|Sequence
            (:then_0
              (Default|PlaySadBacksound (Variables|Default|GetChapterManager))
              (bind _outactors (Actor|GetAllActorswithTag "crutch"))
              (Rendering|SetActorHiddenInGame (Utilities|Array|Get(acopy) _outactors) true))
            (:then_1
              (Utilities|FlowControl|Delay 5.0)
              (bind _returnvalue (UserInterface|CreateWidget "/Game/Blueprints/Widgets/WBP_Mission.WBP_Mission_C" 0 "Talk"))
              (UserInterface|Viewport|AddtoViewport _returnvalue 0)
              (Utilities|FlowControl|Delay 5.0)
              (Widget|RemovefromParent _returnvalue))))))
    (:else)))

(event Custom|OnDialogueEnded_Event
  (bind _playerref (Variables|Default|GetPlayerRef))
  (EventDispatchers|AssignInteractButtonPressed _playerref (delegate Custom|InteractButtonPressed_Event))
  (Variables|/Game/FirstPerson/Blueprints/BP_FirstPersonCharacter.BP_FirstPersonCharacter_C|SetIsInteractButtonPriority? _playerref true)
  (EventDispatchers|UnbindallEventsfromOnDialogueEnded (Variables|Default|GetBP_DialogueComponent))
  (CallFunction|SetCue false))

(event EventBeginPlay
  (|CallParentFunction)
  (bind _returnvalue (Actor|GetActorOfClass "/Game/Blueprints/Chapters/BP_Chapter7AManager.BP_Chapter7AManager_C"))
  (Variables|Default|SetChapterManager _returnvalue))

(event EventInteractObject
  (bind _playerref (Variables|Default|GetPlayerRef))
  (bind _bp_dialoguecomponent (Variables|Default|GetBP_DialogueComponent))
  (bind _asbp_level_camera (Utilities|Casting|CastToBP_LevelCamera (Variables|/Script/Engine.ChildActorComponent|GetChildActor (Variables|Default|GetChildActor))))
  (bind _output_get (Variables|Default|SetAs%20BP%20Level%20Camera _asbp_level_camera))
  (Default|InitializeLevelCamera _output_get (Variables|Default|GetPlayerRef) 0.4 false)
  (Variables|Default|GetIsEventReady?
    (:then
      (Utilities|FlowControl|DoOnce false
        (:Completed
          (Utilities|FlowControl|Sequence
            (:then_0
              (bind _tv (Variables|Default|GetTV)
                (:then
                  (Default|StopTV _tv))
                (:else)))
            (:then_1
              (Utilities|FlowControl|Delay 2.0)
              (bind _dialoguecomponent (Default|ConstructDialogue (Variables|Default|GetBP_DialogueComponent) "ch7_window_1" "/Game/Dialogue/Chapter7_Dialogue.Chapter7_Dialogue" false false))
              (Default|ShowDialogue _dialoguecomponent (Variables|Default|GetPlayerRef) self)
              (EventDispatchers|AssignOnDialogueEnded _bp_dialoguecomponent (delegate Custom|OnDialogueEnded_Event))
              (Default|CallMoveNPCs (Variables|Default|GetChapterManager)))))))
    (:else
      (EventDispatchers|AssignInteractButtonPressed _playerref (delegate Custom|InteractButtonPressed_Event))
      (Variables|/Game/FirstPerson/Blueprints/BP_FirstPersonCharacter.BP_FirstPersonCharacter_C|SetIsInteractButtonPriority? _playerref true)
      (EventDispatchers|UnbindallEventsfromOnDialogueEnded _bp_dialoguecomponent)
      (CallFunction|SetCue false))))

(fn ConstructionScript
  (|CallParentFunction))