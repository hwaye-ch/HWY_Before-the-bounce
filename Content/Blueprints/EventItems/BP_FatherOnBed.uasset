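; BP_FatherOnBed is a scripted horror event that reveals the hidden father mesh on the bed and closes the chapter.
; ShowDadonBed shows the mesh and spotlight, starts audio, then after a delay plays a jumpscare sound while a timeline turns BP_BedCamera toward the father.
; A croak and a long fade-out follow, with a second timeline lowering the father's audio.
; When the fade ends, the player is sent to chapter 6.
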(event Custom|Show%20Dad%20on%20Bed
  (bind _bp_fadescreencomponent (Variables|Default|GetBP_FadeScreenComponent))
  (Rendering|SetVisibility (Variables|Default|GetSkeletalMesh) true false)
  (Rendering|SetVisibility (Variables|Default|GetSpotLight) true false)
  (Audio|Components|Audio|Play (Variables|Default|Getsfx_dad) 0.0)
  (Utilities|FlowControl|Delay 3.0)
  (bind _returnvalue (Actor|GetActorOfClass "/Game/Blueprints/LevelCameras/BP_BedCamera.BP_BedCamera_C"))
  (Audio|SpawnSound2D "/Game/Sounds/sfx_jumpscare-mom.sfx_jumpscare-mom" 2.0 1.0 0.0 0)
  (bind _newtrack_0 (Timeline|Timeline PlayFromStart)
    (:Update
      (Transformation|SetWorldRotation (Variables|/Game/Blueprints/ModularItems/BP_LevelCamera.BP_LevelCamera_C|GetCamera _returnvalue) (Math|Rotator|Lerp(Rotator) (Transformation|GetWorldRotation (Variables|/Game/Blueprints/ModularItems/BP_LevelCamera.BP_LevelCamera_C|GetCamera _returnvalue)) (Math|Rotator|FindLookatRotation (Transformation|GetWorldLocation (Variables|/Game/Blueprints/ModularItems/BP_LevelCamera.BP_LevelCamera_C|GetCamera _returnvalue)) (Transformation|GetActorLocation)) _newtrack_0) false false))
    (:Finished
      (Audio|SpawnSound2D "/Game/Sounds/sfx_croak.sfx_croak" 1.0 1.0 0.0 0)
      (Utilities|FlowControl|Delay 1.5)
      (Default|FadeOut _bp_fadescreencomponent 15.0 (Variables|Default|GetPlayerRef))
      (EventDispatchers|BindEventtoOnFadeOut _bp_fadescreencomponent (delegate Custom|FadeOutListener_Event))
      (bind _newtrack_0_2 (Timeline|Timeline_0 Play)
        (:Update
          (Audio|Components|Audio|SetVolumeMultiplier (Variables|Default|Getsfx_dad) (Math|Float|Lerp 1.0 0.0 _newtrack_0_2) :!class /Script/Engine.AudioComponent))))))

(event Custom|FadeOutListener_Event
  (Default|PlayChapter (Variables|Default|GetPlayerRef) 6)
  (Utilities|FlowControl|DelayUntilNextTick)
  (EventDispatchers|UnbindallEventsfromOnFadeOut (Variables|Default|GetBP_FadeScreenComponent)))

(event EventBeginPlay
  (|CallParentFunction)
  (Rendering|SetVisibility (Variables|Default|GetSkeletalMesh) false false))

(fn ConstructionScript
  (|CallParentFunction))