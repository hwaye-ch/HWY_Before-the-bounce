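; BP_DiningTable is an interactable event item for the Chapter 1 dinner, enabled when an Enabler reports that heated food is ready.
; Combining, handled once, hides the outline, fades the screen with an eating sound and plays a delayed automatic dinner dialogue.
; When the fade finishes, it waits, shows the "ch1_mandi" dialogue and calls CallEnableShower to unlock the shower step.
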(event Custom|Enable%20Dining%20Table
  (params (HeatedFood :type BP%20Heated%20Food%20Object%20Reference))
  (Variables|Default|SetCanInteract? true)
  (Development|PrintString "Food ready to eat")
  (Variables|Default|SetHeated%20Food HeatedFood)
  (EventDispatchers|UnbindallEventsfromEnableDiningTable (Variables|Default|GetEnabler))
  (Variables|Default|SetHide%20Outline? false))

(event Custom|On%20Finished%20Eating
  (Development|PrintString "Eating finished, waiting for dialogue")
  (Utilities|FlowControl|Delay (Variables|Default|GetDurationBeforeDialogue))
  (bind _dialoguecomponent (Default|ConstructDialogue (Variables|Default|GetBP_DialogueComponent) "ch1_mandi" "/Game/Dialogue/Chapter1_Dialogue.Chapter1_Dialogue" false false))
  (Default|ShowDialogue _dialoguecomponent (Variables|Default|GetPlayerRef) self)
  (Default|CallEnableShower)
  (EventDispatchers|UnbindallEventsfromOnFadeEventFinished (Variables|Default|GetBP_FadeScreenComponent)))

(event EventCombineObject
  (Utilities|FlowControl|DoOnce false
    (:Completed
      (Utilities|FlowControl|Sequence
        (:then_0
          (EventDispatchers|BindEventtoOnFadeEventFinished (Variables|Default|GetBP_FadeScreenComponent) (delegate Custom|On%20Finished%20Eating))
          (Default|FadeEvent (Variables|Default|GetBP_FadeScreenComponent) (Variables|Default|GetActionDuration) (Variables|Default|GetPlayerRef) 0.0)
          (Utilities|FlowControl|Delay 2.0)
          (Audio|SpawnSound2D "/Game/Sounds/sfx_eating.sfx_eating" 1.0 1.0 0.0 0)
          (Utilities|FlowControl|Delay 1.0))
        (:then_1
          (Utilities|FlowControl|Delay 7.0)
          (bind _dialoguecomponent (Default|ConstructDialogue (Variables|Default|GetBP_DialogueComponent) "ch1_dinner" "/Game/Dialogue/Chapter1_Dialogue.Chapter1_Dialogue" false false))
          (Default|DisplayAutoDialogue _dialoguecomponent))
        (:then_2
          (Variables|Default|SetHide%20Outline? true))))))

(event EventBeginPlay
  (|CallParentFunction)
  (Variables|/Game/Blueprints/Components/BP_CombinableComponent.BP_CombinableComponent_C|SetCombinableItemCode (Variables|Default|GetBP_CombinableComponent) "NewEnumerator3")
  (bind _enabler (Variables|Default|GetEnabler)
    (:then
      (EventDispatchers|BindEventtoEnableDiningTable _enabler (delegate Custom|Enable%20Dining%20Table)))
    (:else)))

(fn ConstructionScript)