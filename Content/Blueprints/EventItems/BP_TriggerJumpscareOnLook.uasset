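; An event item that triggers a jumpscare when the player's look hit lands on an actor tagged "Jumpscare".
; It stays without collision until a linked enabler calls setup, which enables collision and shows the idle Mom.
; Once ready, Tick checks the player's HitActor and fires once, running a timeline that rotates the camera toward Mom.
; When the timeline finishes, it disables movement and look, calls the jumpscare and turns collision off.
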(event Custom|Setup%20Jumpscare
  (Development|PrintString "Jumpscare is ready")
  (Collision|SetCollisionEnabled (Variables|Default|GetProperty%20Item) "QueryAndPhysics")
  (Variables|Default|SetIsReady true)
  (Rendering|SetVisibility (Variables|/Game/Blueprints/EventItems/BP_JumpscareMom.BP_JumpscareMom_C|GetIdleMom (Variables|Default|GetMom)) true true))

(event EventTick
  (params (DeltaSeconds :type Float%20%28single-precision%29))
  (bind _player_ref (Variables|Default|GetPlayer%20Ref))
  (bind _player_ref_2 (Variables|Default|GetPlayer%20Ref))
  (bind _firstpersoncamera (Variables|/Game/FirstPerson/Blueprints/BP_FirstPersonCharacter.BP_FirstPersonCharacter_C|GetFirstPersonCamera _player_ref))
  (bind _hit_actor (Variables|/Game/FirstPerson/Blueprints/BP_FirstPersonCharacter.BP_FirstPersonCharacter_C|GetHit%20Actor _player_ref_2))
  (if (Variables|Default|GetIsReady)
    (Utilities|IsValid _hit_actor
      (:Is%20Valid
        (if (Actor|ActorHasTag _hit_actor "Jumpscare")
          (Utilities|FlowControl|DoOnce false
            (:Completed
              (bind _mom (Variables|Default|GetMom)
                (:then
                  (Timeline|Timeline Play
                    (:Update
                      (Pawn|SetControlRotation (Game|GetPlayerController 0) (Math|Interpolation|RInterpTo (Math|Rotator|FindLookatRotation (Transformation|GetWorldLocation _firstpersoncamera) (Transformation|GetActorLocation _mom)) (Transformation|GetWorldRotation _firstpersoncamera) 0.0 0.0)))
                    (:Finished
                      (Default|DisableMovementandLook (Variables|Default|GetPlayer%20Ref))
                      (Default|CallCallJumpscare)
                      (Collision|SetCollisionEnabled (Variables|Default|GetProperty%20Item) "NoCollision"))))
                (:else)))))))))

(event EventBeginPlay
  (bind _enabler_jumpscare (Variables|Default|GetEnabler_Jumpscare))
  (|CallParentFunction)
  (Utilities|IsValid _enabler_jumpscare
    (:Is%20Valid
      (EventDispatchers|BindEventtoSetJumpscare _enabler_jumpscare (delegate Custom|Setup%20Jumpscare))
      (Collision|SetCollisionEnabled (Variables|Default|GetProperty%20Item) "NoCollision"))))

(fn ConstructionScript
  (|CallParentFunction))