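; BP_Kulkas is an interactable fridge event item whose door opens and closes on alternate interactions.
; An optional Enabler's event sets CanInteract to true.
; InteractObject uses a FlipFlop to play or reverse one Timeline that swings the door and scales the humming volume, with open and delayed close sounds.
; A frozen-food spawn chain is left unconnected, and ThrowObject is empty.
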(event Custom|Enable%20Kulkas
  (Development|PrintString "Kulas - Enabled")
  (Variables|Default|SetCanInteract? true))

(event EventInteractObject
  (Utilities|FlowControl|FlipFlop
    (:A
      (Audio|PlaySoundatLocation "/Game/Sounds/sfx_fridge-open.sfx_fridge-open" (Transformation|GetWorldLocation (Variables|Default|GetFridge_Door_01)) "0, 0, 0" 1.0 1.0 0.0 "/Game/Sounds/BasketballBounce/SA_ProximitySoundWithLocation.SA_ProximitySoundWithLocation" 0 0 0)
      (bind _newtrack_0 (Timeline|Timeline Play)
        (:Update
          (Audio|Components|Audio|SetVolumeMultiplier (Variables|Default|Getsfx_fridge-humming) (Math|Float|Lerp 0.5 1.5 _newtrack_0) :!class /Script/Engine.AudioComponent)
          (Transformation|SetRelativeRotation (Variables|Default|GetFridge_Door_01) (Math|Rotator|MakeRotator 0.0 0.0 (Math|Float|Lerp 0.0 -9e+01 _newtrack_0)) false false))))
    (:B
      (Utilities|FlowControl|Sequence
        (:then_0
          (Utilities|FlowControl|Delay 0.4)
          (Audio|PlaySoundatLocation "/Game/Sounds/sfx_close-fridge.sfx_close-fridge" (Transformation|GetWorldLocation (Variables|Default|GetFridge_Door_01)) "0, 0, 0" 1.0 1.0 0.0 "/Game/Sounds/BasketballBounce/SA_ProximitySoundWithLocation.SA_ProximitySoundWithLocation" 0 0 0))
        (:then_1
          (Timeline|Timeline Reverse))))))

(event EventBeginPlay
  (bind _enabler (Variables|Default|GetEnabler))
  (Utilities|IsValid _enabler
    (:Is%20Valid
      (EventDispatchers|BindEventtoEnableKulkas _enabler (delegate Custom|Enable%20Kulkas)))))

(fn ConstructionScript)

(fn ThrowObject
  (return))