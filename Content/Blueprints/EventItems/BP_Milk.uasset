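; BP_Milk is a milk event item that is visible only during chapter 2.
; On BeginPlay it runs the parent logic, then reads CurrentChapter from GameInstanceRef and sets its hidden-in-game state accordingly.
; The check happens once, and it toggles only visibility, leaving collision untouched.
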(event EventBeginPlay
  (|CallParentFunction)
  (if (== (Variables|/Game/System/HwyGameInstance.HwyGameInstance_C|GetCurrentChapter (Variables|Default|GetGame%20Instance%20Ref)) 2)
    (Rendering|SetActorHiddenInGame false)
    (else
      (Rendering|SetActorHiddenInGame true))))

(event Collision|EventActorBeginOverlap
  (params (OtherActor :type Actor%20Object%20Reference))
  (|CallParentFunction OtherActor) ; This node is disabled and will not be called.\nDrag off pins to build functionality.
)

(event EventTick
  (params (DeltaSeconds :type Float%20%28single-precision%29))
  (|CallParentFunction DeltaSeconds) ; This node is disabled and will not be called.\nDrag off pins to build functionality.
)

(fn ConstructionScript
  (|CallParentFunction))