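; Chapter 7 event item for an X-ray ("rontgen") that starts a dialogue and story sequence when inspected.
; The first inspection, if no BlockEvent is set, hides the cue and briefly blocks interaction before showing a movement- and look-locking dialogue.
; When dialogue ends, it disables player movement and look, then tells BP_Chapter7AManager, found at BeginPlay, to call the store sequence state.
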(event Custom|OnDialogueEnded_Event
  (Default|DisableMovementandLook (Variables|Default|GetPlayerRef))
  (bind _chapter7manager (Variables|Default|GetChapter7Manager)
    (:then
      (Default|CallStoreSequenceState _chapter7manager))
    (:else)))

(event EventBeginPlay
  (|CallParentFunction)
  (bind _returnvalue (Actor|GetActorOfClass "/Game/Blueprints/Chapters/BP_Chapter7AManager.BP_Chapter7AManager_C"))
  (Variables|Default|SetChapter7Manager _returnvalue))

(event EventInspectObject
  (bind _bp_dialoguecomponent (Variables|Default|GetBP_DialogueComponent))
  (Utilities|FlowControl|DoOnce false
    (:Completed
      (Variables|Default|GetBlock%20Event?
        (:then)
        (:else
          (Variables|/Game/FirstPerson/Blueprints/BP_FirstPersonCharacter.BP_FirstPersonCharacter_C|SetIsInteractionBlocked (Variables|Default|GetPlayerRef) true)
          (CallFunction|SetCue false)
          (Utilities|FlowControl|Delay 2.0)
          (Variables|/Game/FirstPerson/Blueprints/BP_FirstPersonCharacter.BP_FirstPersonCharacter_C|SetIsInteractionBlocked (Variables|Default|GetPlayerRef) false)
          (EventDispatchers|AssignOnDialogueEnded _bp_dialoguecomponent (delegate Custom|OnDialogueEnded_Event))
          (bind _dialoguecomponent (Default|ConstructDialogue _bp_dialoguecomponent "ch7_rontgen_1" "/Game/Dialogue/Chapter7_Dialogue.Chapter7_Dialogue" true true))
          (Default|ShowDialogue _dialoguecomponent (Variables|Default|GetPlayerRef) self))))))

(fn ConstructionScript
  (|CallParentFunction))