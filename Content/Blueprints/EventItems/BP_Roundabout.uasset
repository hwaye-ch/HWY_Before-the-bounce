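; Playground roundabout event item that spins and squeaks during certain story chapters.
; On BeginPlay it waits a tick, then checks the game instance's current chapter to set IsPlaying and spawn a quiet metal squeak with proximity attenuation at its location.
; While IsPlaying is set, Tick yaws the PropertyItem component by the Rotation rate scaled by delta time.
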(event Custom|Play%20Merry%20Go%20Round%20Sound
  (Audio|SpawnSoundatLocation "/Game/Sounds/sfx_metal-squeak.sfx_metal-squeak" (Transformation|GetActorLocation) "0, 0, 0" 0.2 1.0 0.0 "/Game/Sounds/BasketballBounce/SA_ProximitySound.SA_ProximitySound" 0))

(event EventBeginPlay
  (|CallParentFunction)
  (Utilities|FlowControl|DelayUntilNextTick)
  (switch int (Variables|/Game/System/HwyGameInstance.HwyGameInstance_C|GetCurrentChapter (Variables|Default|GetGame%20Instance%20Ref))
    (:1
      _)
    (:2
      _)
    (:3
      _)
    (:7
      _))
  (Variables|Default|SetIsPlaying true)
  (CallFunction|PlayMerryGoRoundSound))

(event EventTick
  (params (DeltaSeconds :type Float%20%28single-precision%29))
  (Variables|Default|GetIsPlaying
    (:then
      (Transformation|AddLocalRotation (Variables|Default|GetProperty%20Item) (Math|Rotator|MakeRotator 0.0 0.0 (* DeltaSeconds (Variables|Default|GetRotation))) false false))
    (:else)))

(fn ConstructionScript
  (|CallParentFunction))