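; BP_PillsActionable is an interactable pills item for Chapter 7 that plays a dialogue and advances the chapter's sequence state.
; On interaction, its dialogue component builds and shows the "ch7_obat" dialogue from the Chapter 7 table, blocking player movement and look.
; When the dialogue ends, a DoOnce-guarded handler tells a valid Chapter7Manager to store the sequence state, then turns off the item's cue.
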(event Custom|OnDialogueEnded_Event
  (Utilities|FlowControl|DoOnce false
    (:Completed
      (bind _chapter7manager (Variables|Default|GetChapter7Manager)
        (:then
          (Default|StoreSequenceStateEvent _chapter7manager)
          (CallFunction|SetCue false))
        (:else)))))

(event EventBeginPlay
  (|CallParentFunction))

(event EventInteractObject
  (bind _bp_dialoguecomponent (Variables|Default|GetBP_DialogueComponent))
  (bind _dialoguecomponent (Default|ConstructDialogue _bp_dialoguecomponent "ch7_obat" "/Game/Dialogue/Chapter7_Dialogue.Chapter7_Dialogue" true true))
  (Default|ShowDialogue _dialoguecomponent (Variables|Default|GetPlayerRef) self)
  (EventDispatchers|AssignOnDialogueEnded _bp_dialoguecomponent (delegate Custom|OnDialogueEnded_Event)))

(fn ConstructionScript
  (|CallParentFunction))