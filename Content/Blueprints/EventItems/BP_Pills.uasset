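; BP_Pills is an interactable pills item that becomes usable once its PillsEnabler fires a wake-up-from-nightmare event.
; Interaction opens a yes/no choice dialogue, with text pulled from the item description data table, behind a DoOnce gate.
; Yes fades the screen, plays a gulping sound and makes Kasur skip its dialogue; No resets the gate so the question can be asked again.
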(event Custom|Listen%20Execution
  (params (Chosen%20Option :type E_ChoiceDialogue%20Enum :default "NewEnumerator0"))
  (bind _bp_textrelatedcomponent (Variables|Default|GetBP_TextRelatedComponent))
  (switch Utilities|FlowControl|Switch|SwitchonE_ChoiceDialogue Chosen%20Option
    (:NewEnumerator0
      (Development|PrintString "You Chose Yes")
      (Utilities|FlowControl|DelayUntilNextTick)
      (Default|FadeEvent (Variables|Default|GetBP_FadeScreenComponent) 7.0 (Variables|Default|GetPlayerRef) 0.0)
      (Utilities|FlowControl|Delay 2.0)
      (Audio|PlaySound2D "/Game/Sounds/sfx_gulping.sfx_gulping" 1.0 1.0 0.0 0 0)
      (bind _kasur (Variables|Default|GetKasur)
        (:then
          (Variables|/Game/Blueprints/EventItems/BP_KasurKecil.BP_KasurKecil_C|SetSkip%20Dialogue? _kasur true))
        (:else)))
    (:NewEnumerator1
      (Development|PrintString "You Chose No")
      (Utilities|FlowControl|DoOnce false) ; enters at Reset
    )))

(event Custom|Enable%20Pills
  (params (PlayerPref :type BP%20First%20Person%20Character%20Object%20Reference))
  (Development|PrintString "Pills are ready to interact")
  (Variables|Default|SetCanInteract? true))

(event EventBeginPlay
  (|CallParentFunction)
  (bind _pillsenabler (Variables|Default|GetPillsEnabler)
    (:then
      (EventDispatchers|BindEventtoWakeUpfromNightmare _pillsenabler (delegate Custom|Enable%20Pills)))
    (:else)))

(event EventInteractObject
  (bind _bp_textrelatedcomponent (Variables|Default|GetBP_TextRelatedComponent))
  (Utilities|FlowControl|DoOnce false
    (:Completed
      (bind _extracted_text (Default|ExtractText _bp_textrelatedcomponent "/Game/Dialogue/Item_Description.Item_Description" "pill_question"))
      (bind _extracted_text_2 (Default|ExtractText _bp_textrelatedcomponent "/Game/Dialogue/Item_Description.Item_Description" "pill_yes"))
      (bind _extracted_text_3 (Default|ExtractText _bp_textrelatedcomponent "/Game/Dialogue/Item_Description.Item_Description" "pill_no"))
      (bind _choice_dialogue_component (Default|ConstructChoiceDialogue (Variables|Default|GetBP_ChoiceDialogueComponent) _extracted_text _extracted_text_2 _extracted_text_3))
      (Default|ShowChoiceDialogue _choice_dialogue_component (Variables|Default|GetPlayerRef))
      (EventDispatchers|BindEventtoExecuteOption _choice_dialogue_component (delegate Custom|Listen%20Execution)))))

(fn ConstructionScript
  (|CallParentFunction))