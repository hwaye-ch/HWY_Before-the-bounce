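; Scripted event actor for the Chapter 6 bus ride, with a bus that drives forward every tick once executed.
; Execute switches to a child-actor bus camera, fades in screen and sound, then shows a dialogue after a delay.
; When the dialogue ends, a delayed screen fade leads to ending the camera, calling the next event, and later destroying the actor.
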(event Custom|Handle%20Finish%20Dialogue
  (bind _bp_fadescreencomponent (Variables|Default|GetBP_FadeScreenComponent))
  (Utilities|FlowControl|Delay 3.0)
  (EventDispatchers|AssignOnFadeEventFinished _bp_fadescreencomponent (delegate Custom|OnFadeEventFinished_Event))
  (Default|FadeEvent _bp_fadescreencomponent 5.0 (Variables|Default|GetPlayer%20Ref) 2.0))

(event Custom|OnFadeEventFinished_Event
  (CallFunction|EndBusCamera)
  (Default|CallExecuteNextEvent)
  (Utilities|FlowControl|DelayUntilNextTick)
  (EventDispatchers|UnbindallEventsfromExecuteNextEvent)
  (Utilities|FlowControl|Delay 1e+01)
  (Actor|DestroyActor))

(event EventBeginPlay
  (|CallParentFunction))

(event EventExecute
  (Utilities|FlowControl|Sequence
    (:then_0
      (bind _asbp_bus_camera (Utilities|Casting|CastToBP_BusCamera (Variables|/Script/Engine.ChildActorComponent|GetChildActor (Variables|Default|GetChildActor))))
      (bind _output_get (Variables|Default|SetAs%20BP%20Bus%20Camera _asbp_bus_camera))
      (Default|InitializeLevelCamera _output_get (Variables|Default|GetPlayer%20Ref) 0.0))
    (:then_1
      (Variables|Default|SetIsMoving true)
      (Audio|Components|Audio|FadeIn (Variables|Default|GetSfx) 2.0 1.0 0.0 "Linear" :!class /Script/Engine.AudioComponent)
      (Default|Fadein (Variables|Default|GetBP_FadeScreenComponent) (Variables|Default|GetPlayer%20Ref)))
    (:then_2
      (Utilities|FlowControl|Delay 1e+01)
      (bind _dialoguecomponent (Default|ConstructDialogue (Variables|Default|GetBP_DialogueComponent) "ch6_bus1" "/Game/Dialogue/Chapter6_Dialogue.Chapter6_Dialogue" false false))
      (EventDispatchers|BindEventtoOnDialogueEnded _dialoguecomponent (delegate Custom|Handle%20Finish%20Dialogue))
      (Default|ShowDialogue _dialoguecomponent (Variables|Default|GetPlayer%20Ref) self))))

(event EventTick
  (params (DeltaSeconds :type Float%20%28single-precision%29))
  (Variables|Default|GetIsMoving
    (:then
      (Transformation|AddActorLocalOffset (* (* (Transformation|GetActorForwardVector) (Variables|Default|GetBusSpeed)) (Utilities|Time|GetWorldDeltaSeconds)) false false))
    (:else)))

(fn ConstructionScript
  (|CallParentFunction))