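; BP_Trash is a trash event item built around a Pickupable component, with interaction switched on by an event.
; BeginPlay runs the parent logic, then leaves the component visible with collision disabled.
; EnableSampah ("sampah" is Indonesian for trash) keeps it visible, enables query and physics collision, and sets CanInteract to true.
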(event Custom|Enable%20Sampah
  (bind _pickupable (Variables|Default|GetPickupable))
  (Rendering|SetVisibility _pickupable true false)
  (Collision|SetCollisionEnabled _pickupable "QueryAndPhysics")
  (Variables|Default|SetCanInteract? true))

(event EventBeginPlay
  (bind _pickupable (Variables|Default|GetPickupable))
  (|CallParentFunction)
  (Rendering|SetVisibility _pickupable true false)
  (Collision|SetCollisionEnabled _pickupable "NoCollision"))

(fn ConstructionScript
  (|CallParentFunction))