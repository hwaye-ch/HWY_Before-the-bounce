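; Frozen food pickup item, built on a parent Blueprint, that can spin its Pickupable component each tick.
; Sphere overlap toggles the first-person character's interact-button priority flag.
; BeginPlay binds to the player's interact-button press, which calls Interact without an overlap check in this graph.
; PickupObject sets the activator component's item code and prints it as debug output.
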(event OnComponentBeginOverlap(Sphere)
  (params (OverlappedComponent :type Primitive%20Component%20Object%20Reference) (OtherActor :type Actor%20Object%20Reference) (OtherComp :type Primitive%20Component%20Object%20Reference) (OtherBodyIndex :type Integer) (bFromSweep :type Boolean) (SweepResult :type Hit%20Result%20Structure%20%28by%20ref%29))
  (bind _asbp_first_person_character (Utilities|Casting|CastToBP_FirstPersonCharacter OtherActor))
  (Variables|/Game/FirstPerson/Blueprints/BP_FirstPersonCharacter.BP_FirstPersonCharacter_C|SetIsInteractButtonPriority? _asbp_first_person_character true))

(event OnComponentEndOverlap(Sphere)
  (params (OverlappedComponent :type Primitive%20Component%20Object%20Reference) (OtherActor :type Actor%20Object%20Reference) (OtherComp :type Primitive%20Component%20Object%20Reference) (OtherBodyIndex :type Integer))
  (bind _asbp_first_person_character (Utilities|Casting|CastToBP_FirstPersonCharacter OtherActor))
  (Variables|/Game/FirstPerson/Blueprints/BP_FirstPersonCharacter.BP_FirstPersonCharacter_C|SetIsInteractButtonPriority? _asbp_first_person_character false))

(event Custom|InteractButtonPressed_Event
  (CallFunction|Interact (stale EventBeginPlay _asbp_first_person_character)))

(event EventPickupObject
  (bind _output_get (Variables|/Game/Blueprints/Components/BP_ActivatorComponent.BP_ActivatorComponent_C|SetActivatorItemCode (Variables|Default|GetBP_ActivatorComponent) "NewEnumerator0"))
  (Development|PrintString (Utilities|String|EnumtoString _output_get)))

(event EventBeginPlay
  (|CallParentFunction)
  (bind _asbp_first_person_character (Utilities|Casting|CastToBP_FirstPersonCharacter (Game|GetPlayerCharacter 0)))
  (EventDispatchers|AssignInteractButtonPressed _asbp_first_person_character (delegate Custom|InteractButtonPressed_Event)))

(event EventTick
  (params (DeltaSeconds :type Float%20%28single-precision%29))
  (if (Variables|Default|GetIsRotating)
    (Transformation|AddLocalRotation (Variables|Default|GetPickupable) (Math|Rotator|MakeRotator 0.0 0.0 (* DeltaSeconds (Variables|Default|GetRotation))) false false)))

(fn ConstructionScript
  (|CallParentFunction))