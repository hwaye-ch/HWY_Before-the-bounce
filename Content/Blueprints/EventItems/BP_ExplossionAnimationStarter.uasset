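; Event item Blueprint that starts an explosion followed by a fire effect when its Activate event fires.
; On BeginPlay it looks up and caches one Blueprint_Effect_Explosion and one BP_FireEffect actor in the level via GetActorOfClass.
; Activate turns on the explosion's particles and audio, then after a short delay turns on the fire's particles and audio.
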(event Custom|Activate
  (bind _explosion (Variables|Default|GetExplosion))
  (bind _fire (Variables|Default|GetFire))
  (Components|Activation|Activate (Variables|/Game/Blueprints/EventItems/Blueprint_Effect_Explosion.Blueprint_Effect_Explosion_C|GetP_Explosion _explosion) false)
  (Components|Activation|Activate (Variables|/Game/Blueprints/EventItems/Blueprint_Effect_Explosion.Blueprint_Effect_Explosion_C|GetExplosion%20Audio _explosion) false)
  (Utilities|FlowControl|Delay 1.0)
  (Components|Activation|Activate (Variables|/Game/Blueprints/EventItems/BP_FireEffect.BP_FireEffect_C|GetP_Fire _fire) false)
  (Components|Activation|Activate (Variables|/Game/Blueprints/EventItems/BP_FireEffect.BP_FireEffect_C|GetFire%20Audio _fire) false))

(event EventBeginPlay
  (|CallParentFunction)
  (bind _returnvalue (Actor|GetActorOfClass "/Game/Blueprints/EventItems/Blueprint_Effect_Explosion.Blueprint_Effect_Explosion_C"))
  (Variables|Default|SetExplosion _returnvalue)
  (bind _returnvalue_2 (Actor|GetActorOfClass "/Game/Blueprints/EventItems/BP_FireEffect.BP_FireEffect_C"))
  (Variables|Default|SetFire _returnvalue_2))

(fn ConstructionScript
  (|CallParentFunction))