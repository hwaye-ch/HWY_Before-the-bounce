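; BP_Motorcycle is an interactable event item that switches the player to a level camera view of the motorcycle.
; On BeginPlay it caches the BP_LevelCamera held in its child actor component.
; InteractObject starts that camera with a short blend and no light dimming, then takes priority over the player's interact button.
; The next interact press ends the camera and releases that priority.
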(event Custom|InteractButtonPressed_Event
  (Default|EndLevelCamera (Variables|Default|GetAs%20BP%20Level%20Camera))
  (Default|UnsetInteractButtonPriority (Variables|Default|GetPlayerRef)))

(event EventBeginPlay
  (|CallParentFunction)
  (bind _asbp_level_camera (Utilities|Casting|CastToBP_LevelCamera (Variables|/Script/Engine.ChildActorComponent|GetChildActor (Variables|Default|GetChildActor))))
  (Variables|Default|SetAs%20BP%20Level%20Camera _asbp_level_camera))

(event Collision|EventActorBeginOverlap
  (params (OtherActor :type Actor%20Object%20Reference)))

(event EventTick
  (params (DeltaSeconds :type Float%20%28single-precision%29)))

(event EventInteractObject
  (bind _playerref (Variables|Default|GetPlayerRef))
  (Default|InitializeLevelCamera (Variables|Default|GetAs%20BP%20Level%20Camera) _playerref 0.5 false)
  (Default|SetInteractButtonPriority _playerref)
  (EventDispatchers|AssignInteractButtonPressed _playerref (delegate Custom|InteractButtonPressed_Event)))

(fn ConstructionScript
  (|CallParentFunction))