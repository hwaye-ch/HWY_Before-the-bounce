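; Ceiling fan event item that spins its PropertyItem component around the yaw axis.
; One tick after BeginPlay it switches on the game instance's CurrentChapter, and every listed chapter and the default branch set IsPlaying to true.
; While IsPlaying passes its check, Tick adds a local rotation scaled by delta time and the Rotation variable, keeping the spin frame-rate independent.
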(event EventBeginPlay
  (|CallParentFunction)
  (Utilities|FlowControl|DelayUntilNextTick)
  (switch int (Variables|/Game/System/HwyGameInstance.HwyGameInstance_C|GetCurrentChapter (Variables|Default|GetGame%20Instance%20Ref))
    (:Default
      _)
    (:1
      _)
    (:2
      _)
    (:3
      _)
    (:4
      _)
    (:7
      _))
  (Variables|Default|SetIsPlaying true))

(event EventTick
  (params (DeltaSeconds :type Float%20%28single-precision%29))
  (Variables|Default|GetIsPlaying
    (:then
      (Transformation|AddLocalRotation (Variables|Default|GetProperty%20Item) (Math|Rotator|MakeRotator 0.0 0.0 (* DeltaSeconds (Variables|Default|GetRotation))) false false))
    (:else)))

(fn ConstructionScript
  (|CallParentFunction))