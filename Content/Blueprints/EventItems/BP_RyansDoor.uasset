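; BP_RyansDoor is an event door that lets the player peek through it using a child-actor level camera.
; StartPeeking blends to that camera; while the event is ready, it triggers a one-time jumpscare, briefly blocks interaction, and plays a Chapter 4 dialogue.
; When the dialogue ends, or if no event is ready, the interact button is prioritized and bound to ExitPeeping, which ends the camera view and releases that priority.
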(event Custom|Exit%20Peeping
  (bind _as_bp_level_camera (Variables|Default|GetAs%20BP%20Level%20Camera)
    (:then
      (Default|EndLevelCamera _as_bp_level_camera)
      (Default|UnsetInteractButtonPriority (Variables|Default|GetPlayer%20Pref)))
    (:else)))

(event Custom|OnDialogueEnded_Event
  (Variables|Default|SetIsEventReady? false)
  (Default|SetInteractButtonPriority (Variables|Default|GetPlayer%20Pref))
  (EventDispatchers|BindEventtoInteractButtonPressed (Variables|Default|GetPlayer%20Pref) (delegate Custom|Exit%20Peeping)))

(event EventStartPeeking
  (bind _bp_dialoguecomponent (Variables|Default|GetBP_DialogueComponent))
  (if (not (Variables|Default|GetIsPeeking))
    (bind _asbp_level_camera (Utilities|Casting|CastToBP_LevelCamera (Variables|/Script/Engine.ChildActorComponent|GetChildActor (Variables|Default|GetLevelCamera))))
    (Variables|Default|SetAs%20BP%20Level%20Camera _asbp_level_camera)
    (Default|InitializeLevelCamera _asbp_level_camera (Variables|Default|GetPlayer%20Pref) 0.3)
    (Variables|Default|GetIsEventReady?
      (:then
        (Utilities|FlowControl|Sequence
          (:then_0
            (Utilities|FlowControl|DoOnce false
              (:Completed
                (Default|CallSetJumpscare))))
          (:then_1
            (Variables|/Game/FirstPerson/Blueprints/BP_FirstPersonCharacter.BP_FirstPersonCharacter_C|SetIsInteractionBlocked (Variables|Default|GetPlayer%20Pref) true)
            (Utilities|FlowControl|Delay 2.0)
            (Variables|/Game/FirstPerson/Blueprints/BP_FirstPersonCharacter.BP_FirstPersonCharacter_C|SetIsInteractionBlocked (Variables|Default|GetPlayer%20Pref) false)
            (bind _dialoguecomponent (Default|ConstructDialogue _bp_dialoguecomponent "ch4_peep_0" "/Game/Dialogue/Chapter4_Dialogue.Chapter4_Dialogue" false false))
            (Default|ShowDialogue _dialoguecomponent (Variables|Default|GetPlayer%20Pref) self)
            (EventDispatchers|AssignOnDialogueEnded _bp_dialoguecomponent (delegate Custom|OnDialogueEnded_Event)))))
      (:else
        (Default|SetInteractButtonPriority (Variables|Default|GetPlayer%20Pref))
        (EventDispatchers|BindEventtoInteractButtonPressed (Variables|Default|GetPlayer%20Pref) (delegate Custom|Exit%20Peeping))))))

(fn ConstructionScript
  (|CallParentFunction))