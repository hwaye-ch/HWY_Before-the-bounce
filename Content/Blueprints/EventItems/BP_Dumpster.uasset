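; BP_Dumpster is an event item that acts as the drop-off point for a trash-collecting mission.
; An Enabler's start-counting event shows a progress widget and turns on a cue.
; Each CombineObject call increments the collectible component's count, plays a dump sound and updates the widget.
; Reaching the maximum removes the widget after a delay and fires the Mikey room event, while earlier drops past a threshold set an achievement.
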(event Custom|Display%20GUI%20Counting%20Trash
  (bind _returnvalue (UserInterface|CreateWidget "/Game/Blueprints/Widgets/WBP_Collectible.WBP_Collectible_C" 0 (Variables|Default|GetTempCollectibleText) (Variables|Default|GetMission%20Text)))
  (Variables|Default|SetMission%20Widget _returnvalue)
  (UserInterface|Viewport|AddtoViewport _returnvalue 0)
  (CallFunction|SetCue true))

(event Custom|Construct%20Collectible
  (bind _bp_collectiblecomponent (Variables|Default|GetBP_CollectibleComponent))
  (Variables|Default|SetTempCollectibleText (Utilities|String|Append (Utilities|String|ToString(Integer) (Variables|/Game/Blueprints/Components/BP_CollectibleComponent.BP_CollectibleComponent_C|GetCurrentCollectedItem _bp_collectiblecomponent)) " / " (Utilities|String|ToString(Integer) (Variables|/Game/Blueprints/Components/BP_CollectibleComponent.BP_CollectibleComponent_C|GetMaxCollectibleItem _bp_collectiblecomponent)))))

(event EventBeginPlay
  (|CallParentFunction)
  (CallFunction|ConstructCollectible)
  (bind _enabler (Variables|Default|GetEnabler)
    (:then
      (EventDispatchers|BindEventtoStartCountingTrash _enabler (delegate Custom|Display%20GUI%20Counting%20Trash)))
    (:else)))

(event EventCombineObject
  (bind _bp_collectiblecomponent (Variables|Default|GetBP_CollectibleComponent))
  (Development|PrintString "Dropped Trash")
  (Math|Integer|IncrementInt (Variables|/Game/Blueprints/Components/BP_CollectibleComponent.BP_CollectibleComponent_C|GetCurrentCollectedItem (Variables|Default|GetBP_CollectibleComponent))
    (:%20%20
      (CallFunction|ConstructCollectible)
      (Audio|SpawnSoundatLocation "/Game/Sounds/sfx_dump_trash.sfx_dump_trash" (Transformation|GetActorLocation) "0, 0, 0" 0.5 1.0 0.0 "/Game/Sounds/BasketballBounce/SA_ProximitySound.SA_ProximitySound" 0)
      (Default|UpdateCollectible (Variables|Default|GetMission%20Widget) (Variables|Default|GetTempCollectibleText) (Variables|Default|GetMission%20Text))
      (if (== (Variables|/Game/Blueprints/Components/BP_CollectibleComponent.BP_CollectibleComponent_C|GetCurrentCollectedItem _bp_collectiblecomponent) (Variables|/Game/Blueprints/Components/BP_CollectibleComponent.BP_CollectibleComponent_C|GetMaxCollectibleItem _bp_collectiblecomponent))
        (Development|PrintString "Mission Completed")
        (Utilities|FlowControl|Delay 2.0)
        (Widget|RemovefromParent (Variables|Default|GetMission%20Widget))
        (Default|CallActivateMikeyRoomEvent)
        (CallFunction|SetCue false)
        (elif (>= (Variables|/Game/Blueprints/Components/BP_CollectibleComponent.BP_CollectibleComponent_C|GetCurrentCollectedItem (Variables|Default|GetBP_CollectibleComponent)) (Variables|Default|GetAchievement%20Trash%20Count))
          (Default|SetAchievement (Variables|Default|GetGame%20Instance%20Ref) "NewEnumerator2"))))))

(fn ConstructionScript
  (|CallParentFunction))