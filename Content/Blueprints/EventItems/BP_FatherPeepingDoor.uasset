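; BP_FatherPeepingDoor is an event item for a horror moment in which the father appears to peep from a door.
; The skeletal mesh starts hidden; Peep shows it and plays a dad horror sound after a two-second delay, while Returnfrompeep hides it again.
; An unconnected timeline that would slide the actor along Y, then stop its sound and destroy it, never runs.
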(event Custom|Return%20from%20peep
  (Rendering|SetVisibility (Variables|Default|GetSkeletalMesh) false false))

(event Custom|Peep
  (Rendering|SetVisibility (Variables|Default|GetSkeletalMesh) true false)
  (Utilities|FlowControl|Delay 2.0)
  (Audio|Components|Audio|Play (Variables|Default|Getsfx_dad-horror) 0.0))

(event EventBeginPlay
  (|CallParentFunction)
  (Rendering|SetVisibility (Variables|Default|GetSkeletalMesh) false false))

(fn ConstructionScript
  (|CallParentFunction))