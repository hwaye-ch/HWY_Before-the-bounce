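; BP_JumpscareMom is a jumpscare actor: a ghost mom flies at the player's face, then a nightmare wake-up follows.
; An enabler's event triggers a delayed swap to the flying mesh, which a Timeline lerps to just before the first-person camera, spawning scare sounds every update.
; It then hides, plays the wake-up Level Sequence, calls the lamp and wake-up events, and destroys itself.
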(event Custom|Listen%20to%20finished%20sequence
  (Default|CallWakeUpfromNightmare (Variables|Default|GetPlayerRef))
  (Utilities|FlowControl|Delay 5.0)
  (EventDispatchers|UnbindallEventsfromWakeUpfromNightmare)
  (Actor|DestroyActor))

(event Custom|Play%20Event
  (bind _playerref (Variables|Default|GetPlayerRef))
  (bind _firstpersoncamera (Variables|/Game/FirstPerson/Blueprints/BP_FirstPersonCharacter.BP_FirstPersonCharacter_C|GetFirstPersonCamera _playerref))
  (Utilities|FlowControl|Delay 1.4)
  (Rendering|SetVisibility (Variables|Default|GetIdleMom) false false)
  (Rendering|SetVisibility (Variables|Default|GetFlyingMom) true false)
  (Variables|Default|SetGhostEndLocation (+ (Transformation|GetWorldLocation _firstpersoncamera) (* (Math|Vector|GetForwardVector _firstpersoncamera) 2e+01)))
  (bind _newtrack_0 (Timeline|Timeline PlayFromStart)
    (:Update
      (Transformation|SetActorLocation (Math|Vector|Lerp(Vector) (Variables|Default|GetGhostStartLocation) (Variables|Default|GetGhostEndLocation) _newtrack_0) false false)
      (Audio|SpawnSound2D "/Game/Sounds/sfx_jumpscare4.sfx_jumpscare4" 1.0 1.0 0.0 0)
      (Audio|SpawnSound2D "/Game/Sounds/sfx_screaming.sfx_screaming" 2.0 1.0 0.0 0)
      (Audio|SpawnSound2D "/Game/Sounds/sfx_tinnitus.sfx_tinnitus" 0.1 1.0 0.0 0))
    (:Finished
      (Utilities|FlowControl|Delay 1.5)
      (Rendering|SetVisibility (Variables|Default|GetFlyingMom) false false)
      (bind _returnvalue (Sequencer|Player|CreateLevelSequencePlayer "/Game/Animation/Anim_ch4-WakeUpFromNightmare.Anim_ch4-WakeUpFromNightmare"))
      (Sequencer|Player|Play _returnvalue :!class /Script/MovieScene.MovieSceneSequencePlayer)
      (EventDispatchers|BindEventtoOnFinished _returnvalue (delegate Custom|Listen%20to%20finished%20sequence))
      (Default|CallTurnAllLamps))))

(event EventBeginPlay
  (|CallParentFunction)
  (bind _jumpscareenabler (Variables|Default|GetJumpscareEnabler)
    (:then
      (EventDispatchers|BindEventtoCallJumpscare _jumpscareenabler (delegate Custom|Play%20Event))
      (Variables|Default|SetGhostStartLocation (Transformation|GetActorLocation self))
      (Rendering|SetVisibility (Variables|Default|GetFlyingMom) false false)
      (Rendering|SetVisibility (Variables|Default|GetIdleMom) false false))
    (:else)))

(fn ConstructionScript
  (|CallParentFunction))