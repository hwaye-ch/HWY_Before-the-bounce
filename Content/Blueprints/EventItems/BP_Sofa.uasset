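; BP_Sofa is an interactable sofa that switches to a child level camera and hosts a scripted Chapter 7 TV event.
; The interact button exits the view unless the TV is on and the event is ready.
; That state triggers a one-time delay-and-callback chain: achievement, TV dialogue, basketball sound with chromatic aberration, second dialogue, then fade.
; The fade's completion ends the camera, unlocks Mikey's door, hides the rope's pickupable and clears the event.
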(event Custom|InteractButtonPressed_Event
  (bind _playerref (Variables|Default|GetPlayerRef))
  (bind _tv (Variables|Default|GetTV)
    (:then
      (if (not (Math|Boolean|ANDBoolean (Variables|/Game/Blueprints/EventItems/BP_Television.BP_Television_C|GetIs%20Enabled? _tv) (Variables|/Game/Blueprints/EventItems/BP_Television.BP_Television_C|GetIs%20TV%20On? _tv) (Variables|Default|GetIs%20Event%20Ready?)))
        (Default|EndLevelCamera (Variables|Default|GetAs%20BP%20Level%20Camera))
        (Variables|/Game/FirstPerson/Blueprints/BP_FirstPersonCharacter.BP_FirstPersonCharacter_C|SetIsInteractButtonPriority? _playerref false)
        (EventDispatchers|UnbindallEventsfromInteractButtonPressed _playerref)))
    (:else)))

(event Custom|OnDialogueEnded_Event
  (bind _bp_fadescreencomponent (Variables|Default|GetBP_FadeScreenComponent))
  (Default|FadeEvent _bp_fadescreencomponent 5.0 (Variables|Default|GetPlayerRef) 2.0)
  (EventDispatchers|AssignOnFadeEventFinished _bp_fadescreencomponent (delegate Custom|OnFadeEventFinished_Event)))

(event Custom|OnFadeEventFinished_Event
  (Default|EndLevelCamera (Variables|Default|GetAs%20BP%20Level%20Camera))
  (bind _mikey_s_door (Variables|Default|Getmikey's%20door)
    (:then
      _)
    (:else
      _))
  (Variables|/Game/Blueprints/ModularItems/BP_InteractableDoor.BP_InteractableDoor_C|SetIsLocked _mikey_s_door false)
  (bind _rope (Variables|Default|GetRope)
    (:then
      _)
    (:else
      _))
  (Rendering|SetVisibility (Variables|/Game/Blueprints/ModularItems/BP_PickupableItem.BP_PickupableItem_C|GetPickupable _rope) false false)
  (Variables|Default|SetIs%20Event%20Ready? false))

(event Custom|OnDialogueEnded_Event_0
  (Utilities|FlowControl|Delay 1e+01)
  (Variables|/Game/FirstPerson/Blueprints/BP_FirstPersonCharacter.BP_FirstPersonCharacter_C|SetIsInteractButtonPriority? (Variables|Default|GetPlayerRef) true)
  (bind _basketball_sound_trigger (Variables|Default|GetBasketball%20Sound%20Trigger)
    (:then
      (Default|Execute _basketball_sound_trigger)
      (Default|SetChromaticAbberationtoCamera (Variables|Default|GetAs%20BP%20Level%20Camera) true 5.0 false)
      (Utilities|FlowControl|Delay 1e+01)
      (Variables|/Game/FirstPerson/Blueprints/BP_FirstPersonCharacter.BP_FirstPersonCharacter_C|SetIsInteractButtonPriority? (Variables|Default|GetPlayerRef) false)
      (bind _dialoguecomponent (Default|ConstructDialogue (Variables|Default|GetBP_DialogueComponent) "ch7_basket" "/Game/Dialogue/Chapter7_Dialogue.Chapter7_Dialogue" true true))
      (Default|ShowDialogue _dialoguecomponent (Variables|Default|GetPlayerRef) self)
      (EventDispatchers|AssignOnDialogueEnded _dialoguecomponent (delegate Custom|OnDialogueEnded_Event)))
    (:else)))

(event EventBeginPlay
  (|CallParentFunction)
  (bind _asbp_level_camera (Utilities|Casting|CastToBP_LevelCamera (Variables|/Script/Engine.ChildActorComponent|GetChildActor (Variables|Default|GetCamera))))
  (Variables|Default|SetAs%20BP%20Level%20Camera _asbp_level_camera))

(event EventInteractObject
  (bind _playerref (Variables|Default|GetPlayerRef))
  (bind _as_bp_level_camera (Variables|Default|GetAs%20BP%20Level%20Camera)
    (:then
      (Default|InitializeLevelCamera _as_bp_level_camera _playerref 0.5 false)
      (Variables|/Game/FirstPerson/Blueprints/BP_FirstPersonCharacter.BP_FirstPersonCharacter_C|SetIsInteractButtonPriority? _playerref true)
      (EventDispatchers|AssignInteractButtonPressed _playerref (delegate Custom|InteractButtonPressed_Event))
      (bind _tv (Variables|Default|GetTV)
        (:then
          (if (Math|Boolean|ANDBoolean (Variables|/Game/Blueprints/EventItems/BP_Television.BP_Television_C|GetIs%20Enabled? _tv) (Variables|/Game/Blueprints/EventItems/BP_Television.BP_Television_C|GetIs%20TV%20On? _tv) (Variables|Default|GetIs%20Event%20Ready?))
            (Utilities|FlowControl|DoOnce false
              (:Completed
                (Utilities|FlowControl|Delay 2.0)
                (Default|SetAchievement (Variables|Default|GetGame%20Instance%20Ref) "NewEnumerator3")
                (Utilities|FlowControl|Delay 1e+01)
                (bind _dialoguecomponent (Default|ConstructDialogue (Variables|Default|GetBP_DialogueComponent) "ch7_tv" "/Game/Dialogue/Chapter7_Dialogue.Chapter7_Dialogue" true true))
                (Default|ShowDialogue _dialoguecomponent (Variables|Default|GetPlayerRef) self)
                (Variables|/Game/FirstPerson/Blueprints/BP_FirstPersonCharacter.BP_FirstPersonCharacter_C|SetIsInteractButtonPriority? (Variables|Default|GetPlayerRef) false)
                (EventDispatchers|AssignOnDialogueEnded _dialoguecomponent (delegate Custom|OnDialogueEnded_Event_0))))))
        (:else)))
    (:else)))

(fn ConstructionScript
  (|CallParentFunction))