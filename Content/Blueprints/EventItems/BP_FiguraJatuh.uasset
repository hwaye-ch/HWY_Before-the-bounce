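; Inspectable photo frame Blueprint that falls as a scripted event and starts a chapter 1 story beat.
; An Enabler's DropPhotoFrame event briefly enables physics, plays a drop sound and arms the sequence.
; Inspecting it then runs one-time dialogue and a chat widget, whose finish triggers more dialogue and fires EnableLaptop.
; Returning it after the fall restores a stored transform once.
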(event Custom|Simulate%20Photo%20Physics
  (Physics|SetSimulatePhysics (Variables|Default|GetInspectableItem) true)
  (Utilities|FlowControl|Delay 0.5)
  (Audio|PlaySoundatLocation "/Game/Sounds/photo_frame_dropped.photo_frame_dropped" (Transformation|GetWorldLocation (Variables|Default|GetInspectableItem)) "0, 0, 0" 3.0 1.0 0.0 "/Game/Sounds/BasketballBounce/SA_ProximitySoundWithLocation.SA_ProximitySoundWithLocation" 0 0 0)
  (Utilities|FlowControl|Delay 1.0)
  (Physics|SetSimulatePhysics (Variables|Default|GetInspectableItem) false)
  (Variables|Default|SetIsSequenceActivated true))

(event Custom|Enable%20Laptop
  (bind _dialoguecomponent (Default|ConstructDialogue (Variables|Default|GetBP_DialogueComponent) "ch1_capek" "/Game/Dialogue/Chapter1_Dialogue.Chapter1_Dialogue" false false))
  (Class|BPIDialogue|DisplayAutoDialogue(Message) _dialoguecomponent)
  (Utilities|FlowControl|Delay 5.0)
  (Default|CallEnableLaptop))

(event EventBeginPlay
  (|CallParentFunction)
  (Variables|Default|SetInitial%20Location (Transformation|GetWorldLocation (Variables|Default|GetInspectableItem)))
  (Variables|Default|SetInitial%20Rotation (Transformation|GetWorldRotation (Variables|Default|GetInspectableItem)))
  (Variables|Default|SetIsLocationChangedInChild true)
  (bind _enabler (Variables|Default|GetEnabler)
    (:then
      (EventDispatchers|BindEventtoDropPhotoFrame _enabler (delegate Custom|Simulate%20Photo%20Physics)))
    (:else)))

(event EventReturnObject
  (Variables|Default|GetIsSequenceActivated
    (:then
      (Utilities|FlowControl|DoOnce false
        (:Completed
          (Transformation|SetWorldLocationAndRotation (Variables|Default|GetInspectableItem) (Variables|Default|GetOriginal%20Location) (Variables|Default|GetOriginal%20Rotation) false false))))
    (:else)))

(event EventInspectObject
  (bind _bp_displaychatdialogue (Variables|Default|GetBP_DisplayChatDialogue))
  (Utilities|FlowControl|Delay (Variables|Default|GetDelayBeforeDialogue))
  (Variables|Default|GetIsSequenceActivated
    (:then
      (Utilities|FlowControl|DoOnce false
        (:Completed
          (bind _dialoguecomponent (Default|ConstructDialogue (Variables|Default|GetBP_DialogueComponent) "ch1_photo" "/Game/Dialogue/Chapter1_Dialogue.Chapter1_Dialogue" false false))
          (Class|BPIDialogue|DisplayAutoDialogue(Message) _dialoguecomponent)
          (Utilities|FlowControl|Delay 15.0)
          (Default|ShowChatWidget _bp_displaychatdialogue "/Game/Textures/sarah1.sarah1")
          (EventDispatchers|BindEventtoOnAnimationFinished _bp_displaychatdialogue (delegate Custom|Enable%20Laptop)))))
    (:else)))

(fn ConstructionScript
  (|CallParentFunction))