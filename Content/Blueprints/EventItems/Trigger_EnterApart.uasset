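; Overlap trigger, named for entering the apartment, that plays story dialogue depending on the player's current chapter.
; On overlap it reads the chapter from the player and has the dialogue component build and show a line that blocks movement and look.
; Only chapters 1 and 8 respond, and chapter 8 draws from the Chapter 7 dialogue table.
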(event EventOnOverlapTrigger
  (bind _current_chapter (Default|GetCurrentChapter (Variables|Default|GetPlayerRef)))
  (switch int _current_chapter
    (:1
      (bind _dialoguecomponent (Default|ConstructDialogue (Variables|Default|GetBP_DialogueComponent) "ch1_roomno" "/Game/Dialogue/Chapter1_Dialogue.Chapter1_Dialogue" true true))
      (Default|ShowDialogue _dialoguecomponent (Variables|Default|GetPlayerRef) self))
    (:8
      (bind _dialoguecomponent_2 (Default|ConstructDialogue (Variables|Default|GetBP_DialogueComponent) "ch7_crazy" "/Game/Dialogue/Chapter7_Dialogue.Chapter7_Dialogue" true true))
      (Default|ShowDialogue _dialoguecomponent_2 (Variables|Default|GetPlayerRef) self))))

(fn ConstructionScript
  (|CallParentFunction))