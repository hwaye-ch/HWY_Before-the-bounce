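; Interactable laptop that advances the story through chapters and hosts a hold-to-work sequence with scares.
; Enabler actors unlock it, then interaction branches on the current chapter to run dialogue, fades, typing audio, saves and chapter switches.
; Its progressable setup pauses or resumes audio with the hold and fires bouncing-ball and peeping-father scares with chromatic aberration at progress thresholds.
; Completion clears the effects, then plays Chapter 4 dialogue and restores the default camera.
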(event Custom|Enable%20Laptop
  (Development|PrintString "Laptop is activated")
  (Variables|Default|SetCanInteract? true))

(event Custom|Activate%20Object
  (bind _bp_fadescreencomponent (Variables|Default|GetBP_FadeScreenComponent))
  (bind _bp_fadescreencomponent_2 (Variables|Default|GetBP_FadeScreenComponent))
  (bind _bp_fadescreencomponent_3 (Variables|Default|GetBP_FadeScreenComponent))
  (Utilities|FlowControl|DoOnce false) ; enters at Reset
)

(event Custom|Play%20Typing%20Sfx
  (bind _returnvalue (Audio|SpawnSound2D "/Game/Sounds/sfx_typing.sfx_typing" 0.7 1.0 0.0 0))
  (Variables|Default|SetTypingSound _returnvalue))

(event Custom|Enable%20Laptop%20Chapter%203
  (CallFunction|EnableLaptop)
  (Variables|Chapter3|SetEndChapter true))

(event Custom|Go%20to%20Chapter%204
  ;[0.15 0.15 0.15 0.5] Chapter 3
  (Default|PlayChapter (Variables|Default|GetPlayerRef) 4))

(event Custom|Go%20to%20Chapter%203
  ;[0.15 0.15 0.15 0.5] Chapter 2
  (bind _typingsound (Variables|Default|GetTypingSound)
    (:then
      (Audio|Components|Audio|Stop _typingsound)
      (Components|DestroyComponent _typingsound)
      (EventDispatchers|UnbindallEventsfromOnFadeEventFinished (Variables|Default|GetBP_FadeScreenComponent))
      (Default|SaveChapter (Variables|Default|GetGame%20Instance%20Ref) "NewEnumerator2")
      (Default|PlayChapter (Variables|Default|GetPlayerRef) 3))
    (:else)))

(event Custom|Go%20to%20Chapter%202
  ;[0.15 0.15 0.15 0.5] Chapter 1
  (bind _typingsound (Variables|Default|GetTypingSound)
    (:then
      (Audio|Components|Audio|Stop _typingsound)
      (Components|DestroyComponent _typingsound)
      (EventDispatchers|UnbindallEventsfromOnFadeEventFinished (Variables|Default|GetBP_FadeScreenComponent))
      (Default|SaveChapter (Variables|Default|GetGame%20Instance%20Ref) "NewEnumerator1")
      (Default|PlayChapter (Variables|Default|GetPlayerRef) 2))
    (:else)))

(event EventInteractObject
  (bind _bp_fadescreencomponent (Variables|Default|GetBP_FadeScreenComponent))
  (bind _bp_fadescreencomponent_2 (Variables|Default|GetBP_FadeScreenComponent))
  (bind _bp_fadescreencomponent_3 (Variables|Default|GetBP_FadeScreenComponent))
  (Utilities|FlowControl|DoOnce false
    (:Completed
      (switch int (Variables|/Game/System/HwyGameInstance.HwyGameInstance_C|GetCurrentChapter (Variables|Default|GetGame%20Instance%20Ref))
        (:1
          ;[0.15 0.15 0.15 0.5] Chapter 1
          (EventDispatchers|BindEventtoOnExactFinish _bp_fadescreencomponent_3 (delegate Custom|Go%20to%20Chapter%202))
          (Default|FadeOut _bp_fadescreencomponent_3 (Variables|Default|GetWorkDuration) (Variables|Default|GetPlayerRef))
          (Utilities|FlowControl|Delay (Variables|Default|GetPreparationDuration))
          (CallFunction|PlayTypingSfx)
          (bind _dialoguecomponent (Default|ConstructDialogue (Variables|Default|GetBP_DialogueComponent) "ch1_belajar" "/Game/Dialogue/Chapter1_Dialogue.Chapter1_Dialogue" false false))
          (Default|DisplayAutoDialogue _dialoguecomponent)
          (bind _ambiencesound (Variables|Default|GetAmbienceSound)
            (:then
              (Default|StoptheAmbienceSound _ambiencesound))
            (:else)))
        (:2
          ;[0.15 0.15 0.15 0.5] Chapter 2
          (EventDispatchers|BindEventtoOnFadeOut _bp_fadescreencomponent (delegate Custom|Go%20to%20Chapter%203))
          (Default|FadeOut _bp_fadescreencomponent 4e+01 (Variables|Default|GetPlayerRef))
          (Utilities|FlowControl|Delay (Variables|Default|GetPreparationDuration))
          (CallFunction|PlayTypingSfx)
          (bind _dialoguecomponent_2 (Default|ConstructDialogue (Variables|Default|GetBP_DialogueComponent) "ch2_tired_1" "/Game/Dialogue/Chapter2_Dialogue.Chapter2_Dialogue" false false))
          (Default|DisplayAutoDialogue _dialoguecomponent_2))
        (:3
          ;[0.15 0.15 0.15 0.5] Chapter 3
          (Variables|Default|GetCanInteract?
            (:then
              (if (Variables|Chapter3|GetEndChapter)
                (Default|SaveChapter (Variables|Default|GetGame%20Instance%20Ref) "NewEnumerator3")
                (EventDispatchers|BindEventtoOnExactFinish _bp_fadescreencomponent_2 (delegate Custom|Go%20to%20Chapter%204))
                (Default|FadeOut _bp_fadescreencomponent_2 1e+01 (Variables|Default|GetPlayerRef))
                (else
                  (bind _dialoguecomponent_3 (Default|ConstructDialogue (Variables|Default|GetBP_DialogueComponent) "ch3_disturbed" "/Game/Dialogue/Chapter3_Dialogue.Chapter3_Dialogue" true true))
                  (Class|BPIDialogue|ShowDialogue(Message) _dialoguecomponent_3 (Variables|Default|GetPlayerRef) self)
                  (CallFunction|ActivateObject))))
            (:else)))))))

(event EventBeginPlay
  (bind _enabler (Variables|Default|GetEnabler))
  (bind _enabler_of_laptop (Variables|Default|GetEnabler%20of%20Laptop))
  (bind _enabler_chapter_3 (Variables|Chapter3|GetEnabler%20Chapter%203))
  (|CallParentFunction)
  (Utilities|IsValid _enabler
    (:Is%20Valid
      (EventDispatchers|BindEventtoEnableLaptop _enabler (delegate Custom|Enable%20Laptop)))
    (:Is%20Not%20Valid
      _))
  (Utilities|IsValid _enabler_chapter_3
    (:Is%20Valid
      (EventDispatchers|BindEventtoActivateLaptop _enabler_chapter_3 (delegate Custom|Enable%20Laptop%20Chapter%203)))
    (:Is%20Not%20Valid
      _))
  (Utilities|IsValid _enabler_of_laptop
    (:Is%20Valid
      (EventDispatchers|BindEventtoTriggerMikeyRoomEvent _enabler_of_laptop (delegate Custom|Enable%20Laptop)))
    (:Is%20Not%20Valid
      _))
  (bind _returnvalue (Actor|GetActorOfClass "/Game/Blueprints/Levels/BP_AmbienceSound.BP_AmbienceSound_C"))
  (Variables|Default|SetAmbienceSound _returnvalue))

(event Custom|SetupProgressableLaptop
  (bind _bp_progressablecomponent (Variables|Default|GetBP_ProgressableComponent))
  (CallFunction|EnableLaptop)
  (Variables|/Game/Blueprints/Components/BP_ProgressableComponent.BP_ProgressableComponent_C|SetIs%20Long%20Interact%20Active _bp_progressablecomponent true)
  (EventDispatchers|BindEventtoUpdateProgressFilling _bp_progressablecomponent (delegate Custom|Call%20Progress%20Filling))
  (EventDispatchers|BindEventtoFinishProgressFilling _bp_progressablecomponent (delegate Custom|Call%20Progress%20Finish))
  (EventDispatchers|AssignCancelProgressFilling _bp_progressablecomponent (delegate Custom|CancelProgressFilling_Event))
  (Utilities|FlowControl|Sequence
    (:then_0
      (Utilities|FlowControl|Delay 2.0)
      (Utilities|FlowControl|DoOnce false
        (:Completed
          (bind _returnvalue (UserInterface|CreateWidget "/Game/Blueprints/Widgets/WBP_Mission.WBP_Mission_C" 0 "Hold [LMB] on Laptop"))
          (UserInterface|Viewport|AddtoViewport _returnvalue 0)
          (bind _output_get (Variables|Default|SetMission%20Widget _returnvalue))
          (Utilities|FlowControl|Delay 3.0)
          (Widget|RemovefromParent _output_get))))
    (:then_1
      (Rendering|Material|SetMaterial (Variables|Default|GetActionableItem) 8 "/Game/Materials/M_Skripsi.M_Skripsi"))))

(event Custom|Call%20Progress%20Filling
  (params (ProgressPercentage :type Float%20%28double-precision%29))
  (bind _audio (Variables|Default|GetAudio))
  (CallFunction|OnProgressUpdateFilling ProgressPercentage)
  (Utilities|FlowControl|DoOnce false
    (:Completed
      (if (Audio|Components|Audio|IsPlaying _audio)
        (Class|AudioComponent|SetPaused (Variables|Default|GetAudio) false)
        (else
          (Audio|Components|Audio|Play _audio 0.0))))))

(event Custom|On%20Finish%20Progress%20Filling
  (bind _bp_progressablecomponent (Variables|Default|GetBP_ProgressableComponent))
  (bind _bp_dialoguecomponent (Variables|Default|GetBP_DialogueComponent))
  ;[0.15 0.15 0.15 0.5] On finished doing with laptop
  (Utilities|FlowControl|Sequence
    (:then_0
      (Development|PrintString "Laptop Progress is completed")
      (Utilities|FlowControl|Delay 2.0)
      (Default|DestroyWidget _bp_progressablecomponent)
      (Variables|/Game/Blueprints/Components/BP_ProgressableComponent.BP_ProgressableComponent_C|SetIs%20Long%20Interact%20Active _bp_progressablecomponent false)
      (Utilities|FlowControl|Delay 3.0)
      (Default|ConstructDialogue _bp_dialoguecomponent "ch4_disturbed" "/Game/Dialogue/Chapter4_Dialogue.Chapter4_Dialogue" false false)
      (Default|DisplayAutoDialogue _bp_dialoguecomponent)
      (Utilities|FlowControl|Delay 6.0)
      (Default|FadeEvent (Variables|Default|GetBP_FadeScreenComponent) 4.0 (Variables|Default|GetPlayerRef) 0.0)
      (Utilities|FlowControl|Delay 2.0)
      (Audio|PlaySound2D "/Game/Sounds/sfx_moving-chair.sfx_moving-chair" 1.0 1.0 0.0 0 0)
      (Default|SwitchtoDefaultCamera (Variables|Default|GetPlayerRef))
      (Utilities|FlowControl|Delay 7.0)
      (bind _dialoguecomponent (Default|ConstructDialogue (Variables|Default|GetBP_DialogueComponent) "ch4_gonnacheck" "/Game/Dialogue/Chapter4_Dialogue.Chapter4_Dialogue" true true))
      (Default|ShowDialogue _dialoguecomponent (Variables|Default|GetPlayerRef) self))
    (:then_1
      (Widget|RemovefromParent (Variables|Default|GetMission%20Widget))
      (Utilities|FlowControl|Delay 3.0)
      (bind _peeking_father (Variables|Default|GetPeeking%20Father)
        (:then
          (Actor|DestroyActor _peeking_father))
        (:else)))
    (:then_2
      (bind _tablecamera (Variables|Default|GetTableCamera)
        (:then
          (Default|SetChromaticAbberationtoCamera _tablecamera false 5.0 false))
        (:else)))))

(event Custom|Call%20Progress%20Finish
  (CallFunction|OnFinishProgressFilling))

(event Custom|CancelProgressFilling_Event
  (bind _audio (Variables|Default|GetAudio))
  (Class|AudioComponent|SetPaused (Variables|Default|GetAudio) true)
  (Utilities|FlowControl|DoOnce false) ; enters at Reset
)

(event Custom|On%20Progress%20Update%20Filling
  (params (Progress%20Percentage :type Float%20%28double-precision%29))
  ;[0.15 0.15 0.15 0.5] Trigger Sound at specific progress percentage
  (if (>= (* Progress%20Percentage 1e+02) (Variables|Chapter4|GetThreshold%20percentage%20to%20trigger%20papa))
    (Utilities|FlowControl|DoOnce false
      (:Completed
        (Development|PrintString "Father is peeping" true true "(R=0.000000,G=1.000000,B=0.047670,A=1.000000)")
        (Default|CallStartFatherPeeping)
        (bind _tablecamera (Variables|Default|GetTableCamera)
          (:then
            (Default|SetChromaticAbberationtoCamera _tablecamera true 5.0 false))
          (:else))))
    (elif (>= (* Progress%20Percentage 1e+02) (Variables|Chapter4|GetThreshold%20percentage%20to%20trigger%20bouncing%20ball))
      (Utilities|FlowControl|DoOnce false
        (:Completed
          (Development|PrintString "Bouncing Ball" true true "(R=0.000000,G=1.000000,B=0.047670,A=1.000000)")
          (Default|CallTriggerMysteriousBasketBallatHall)
          (bind _tablecamera_2 (Variables|Default|GetTableCamera)
            (:then
              (Default|SetChromaticAbberationtoCamera _tablecamera_2 true 2.0 false))
            (:else)))))))

(fn ConstructionScript
  (|CallParentFunction))