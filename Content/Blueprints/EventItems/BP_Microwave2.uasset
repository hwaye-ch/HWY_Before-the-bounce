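; Microwave item that heats frozen food and hands the player a steaming food item when interacted with.
; Combining spawns food on the plate and plays a cooking sound, then after a short delay rotates the food and turns on the light.
; The sound's finish event stops both and marks the food ready.
; Interacting then spawns an interactable food with an activator code, passes it the interaction and destroys the plated food.
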(event Custom|OnFoodReady
  (Development|PrintString "Food Is Ready!")
  (Variables|/Game/Blueprints/EventItems/BP_Food.BP_Food_C|SetIsRotating (Variables|Default|GetFrozenFood) false)
  (Rendering|SetVisibility (Variables|Default|GetLight) false false)
  (Variables|Default|SetIsFoodReady? true))

(event EventInteract
  (params (PlayerRef :type BP%20First%20Person%20Character%20Object%20Reference))
  ;[0.15 0.15 0.15 0.5] Interact with heated food
  (|CallParentFunction PlayerRef)
  (Variables|Default|GetIsFoodReady?
    (:then
      (Development|PrintString "Food is ready to pick up")
      (bind _returnvalue (Game|SpawnActorfromClass "/Game/Blueprints/EventItems/BP_Food.BP_Food_C" (Transformation|GetActorTransform) "Undefined" "MultiplyWithRoot" 0 false 0))
      (Variables|/Game/Blueprints/ModularItems/BP_Engageable.BP_Engageable_C|SetCanInteract? _returnvalue true)
      (Rendering|SetVisibility (Variables|/Game/Blueprints/EventItems/BP_Food.BP_Food_C|GetSteam _returnvalue) true true)
      (Variables|/Game/Blueprints/Components/BP_ActivatorComponent.BP_ActivatorComponent_C|SetActivatorItemCode (Variables|/Game/Blueprints/ModularItems/BP_PickupableItem.BP_PickupableItem_C|GetBP_ActivatorComponent _returnvalue) "NewEnumerator3")
      (Default|Interact _returnvalue (Variables|Default|GetPlayerRef))
      (Variables|Default|SetIsFoodReady? false)
      (Actor|DestroyActor (Variables|Default|GetFrozenFood)))
    (:else
      (Development|PrintString "Food Not Ready"))))

(event EventCombineObject
  ;[0.15 0.15 0.15 0.5] Combine frozen food with microwave
  (bind _returnvalue (Game|SpawnActorfromClass "/Game/Blueprints/EventItems/BP_Food.BP_Food_C" (Transformation|GetWorldTransform (Variables|Default|GetPlate)) "Undefined" "MultiplyWithRoot" 0 false 0))
  (Variables|Default|SetFrozenFood _returnvalue)
  (bind _returnvalue_2 (Audio|SpawnSoundatLocation "/Game/Sounds/sfx_microwave-cooking.sfx_microwave-cooking" (Transformation|GetActorLocation) "0, 0, 0" 1.0 1.0 0.0 "/Game/Sounds/BasketballBounce/SA_ProximitySound.SA_ProximitySound" 0))
  (Utilities|FlowControl|Delay 2.75)
  (Variables|/Game/Blueprints/EventItems/BP_Food.BP_Food_C|SetIsRotating (Variables|Default|GetFrozenFood) true)
  (Rendering|SetVisibility (Variables|Default|GetLight) true false)
  (EventDispatchers|BindEventtoOnAudioFinished _returnvalue_2 (delegate Custom|OnFoodReady)))

(fn ConstructionScript)