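; Scripted scare event item: a dribbling basketball sound that leads the player into a janitor encounter.
; An Enabler's Mikey room trigger is bound at BeginPlay, and Execute spawns the positional sound.
; Once readied, Tick watches for the player targeting a "Mysterious"-tagged actor, then uncrouches them, silences the bounce, shows dialogue and moves the janitor.
; When dialogue ends, a timeline turns the view to the look-at target, playing jumpscare audio and starting janitor talk.
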(event Custom|Dialogue%20Ends
  (bind _player_ref (Variables|Default|GetPlayer%20Ref))
  (bind _bp_lookatcomponent (Variables|Default|GetBP_LookAtComponent))
  (bind _firstpersoncamera (Variables|/Game/FirstPerson/Blueprints/BP_FirstPersonCharacter.BP_FirstPersonCharacter_C|GetFirstPersonCamera _player_ref))
  (bind _objecttolookat (Variables|/Game/Blueprints/Components/BP_LookAtComponent.BP_LookAtComponent_C|GetObjectToLookAt _bp_lookatcomponent))
  (bind _returnvalue (Transformation|GetWorldLocation _firstpersoncamera))
  (bind _rootcomponent (Variables|/Script/Engine.Actor|GetRootComponent _objecttolookat))
  (bind _returnvalue_2 (Transformation|GetWorldLocation _rootcomponent))
  (bind _returnvalue_3 (Math|Rotator|FindLookatRotation (Math|Vector|MakeVector (.x _returnvalue) (.y _returnvalue) (.z _returnvalue)) _returnvalue_2))
  (Development|PrintString "I'm done")
  (bind _lookatalpha (Timeline|Timeline_0 Play)
    (:Update
      (Pawn|SetControlRotation (Game|GetPlayerController 0) (Math|Interpolation|RInterpTo (Transformation|GetWorldRotation _firstpersoncamera) (Math|Rotator|MakeRotator (.roll _returnvalue_3) 0.0 (.yaw _returnvalue_3)) _lookatalpha 5.0))
      (Utilities|FlowControl|DoOnce false
        (:Completed
          (Utilities|FlowControl|Delay 0.2)
          (Audio|PlaySound2D "/Game/Sounds/sfx_gasp.sfx_gasp" 1.0 1.0 0.0 0 0)
          (Audio|PlaySound2D "/Game/Sounds/sfx_piano_jumpscare.sfx_piano_jumpscare" 1.0 1.0 0.0 0 0)
          (Default|CallTalktoJanitor (Variables|Default|GetPlayer%20Ref))
          (Utilities|FlowControl|Delay 5.0))))))

(event Custom|Set%20Event%20Ready
  (Variables|Default|SetIs%20Event%20Ready? true)
  (Collision|SetCollisionEnabled (Variables|Default|GetProperty%20Item) "QueryAndPhysics"))

(event EventTick
  (params (DeltaSeconds :type Float%20%28single-precision%29))
  (bind _player_ref (Variables|Default|GetPlayer%20Ref))
  (bind _player_ref_2 (Variables|Default|GetPlayer%20Ref))
  (bind _bouncesound (Variables|Default|GetBounceSound))
  (bind _hit_actor (Variables|/Game/FirstPerson/Blueprints/BP_FirstPersonCharacter.BP_FirstPersonCharacter_C|GetHit%20Actor _player_ref_2))
  (Variables|Default|GetIs%20Event%20Ready?
    (:then
      (Utilities|IsValid _hit_actor
        (:Is%20Valid
          (if (Actor|ActorHasTag _hit_actor "Mysterious")
            (Utilities|FlowControl|DoOnce false
              (:Completed
                (if (Variables|/Game/FirstPerson/Blueprints/BP_FirstPersonCharacter.BP_FirstPersonCharacter_C|GetIsCrouch _player_ref)
                  (Default|ToggleCrouch _player_ref)
                  (Utilities|FlowControl|Delay 0.2))
                (Utilities|IsValid _bouncesound
                  (:Is%20Valid
                    (Audio|Components|Audio|Stop _bouncesound))
                  (:Is%20Not%20Valid
                    _))
                (Utilities|FlowControl|Delay 0.05)
                (Class|BPIDialogue|ShowDialogue(Message) (Variables|Default|GetBP_DialogueComponent) (Variables|Default|GetPlayer%20Ref) self)
                (Default|CallMoveJanitor)))))))
    (:else)))

(event EventExecute
  (bind _returnvalue (Audio|SpawnSoundatLocation "/Game/Sounds/BasketballBounce/sfx_basketball_dribbling.sfx_basketball_dribbling" (Transformation|GetSocketLocation (Variables|Default|GetProperty%20Item) "None") "0, 0, 0" 1.0 1.0 0.0 "/Game/Sounds/BasketballBounce/SA_ProximitySound.SA_ProximitySound" 0))
  (Variables|Default|SetBounceSound _returnvalue))

(event EventBeginPlay
  (bind _enabler (Variables|Default|GetEnabler))
  (|CallParentFunction)
  (Utilities|IsValid _enabler
    (:Is%20Valid
      (EventDispatchers|BindEventtoTriggerMikeyRoomEvent _enabler (delegate EventExecute))
      (EventDispatchers|BindEventtoOnDialogueEnded (Variables|Default|GetBP_DialogueComponent) (delegate Custom|Dialogue%20Ends))
      (Collision|SetCollisionEnabled (Variables|Default|GetProperty%20Item) "NoCollision"))))

(fn ConstructionScript
  (|CallParentFunction))