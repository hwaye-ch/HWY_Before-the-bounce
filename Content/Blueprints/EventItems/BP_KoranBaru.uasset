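; BP_KoranBaru is a readable newspaper event item that triggers a Chapter 7 event after it is read.
; It starts hidden and non-interactable, and plays a newspaper sound when read.
; The first time it is put down, a DoOnce waits ten seconds, then has the Chapter7Manager play its door event and stop its hum.
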(event EventBeginPlay
  (|CallParentFunction)
  (CallFunction|SetInteraction false false))

(event EventUnreadObject
  (Utilities|FlowControl|DoOnce false
    (:Completed
      (Utilities|FlowControl|Delay 1e+01)
      (bind _chapter7manager (Variables|Default|GetChapter7Manager)
        (:then
          (Default|PlayDoor _chapter7manager)
          (Audio|Components|Audio|Stop (Variables|/Game/Blueprints/Chapters/BP_Chapter7BManager.BP_Chapter7BManager_C|GetHum _chapter7manager)))
        (:else)))))

(event EventReadObject
  (Audio|Components|Audio|Play (Variables|Default|GetNewspaperSound) 0.0))

(fn ConstructionScript
  (|CallParentFunction))