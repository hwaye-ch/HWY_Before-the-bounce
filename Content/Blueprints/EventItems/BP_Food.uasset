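; BP_Food is a food event item with a Pickupable component and a child-actor steam effect.
; On BeginPlay it runs the parent logic, caches the steam effect, deactivates its audio, and hides both the lit steam particles and Pickupable.
; While IsRotating is set, Tick yaws Pickupable at the Rotation rate, scaled by delta time.
; Nothing in this graph reveals the hidden parts again.
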(event EventBeginPlay
  (|CallParentFunction)
  (bind _asblueprint_effect_steam (Utilities|Casting|CastToBlueprint_Effect_Steam (Variables|/Script/Engine.ChildActorComponent|GetChildActor (Variables|Default|GetSteam))))
  (bind _output_get (Variables|Default|SetAs%20Blueprint%20Effect%20Steam _asblueprint_effect_steam))
  (Components|Activation|SetActive (Variables|/Game/StarterContent/Blueprints/Blueprint_Effect_Steam.Blueprint_Effect_Steam_C|GetSteam%20AUdio _output_get) false false)
  (Rendering|SetVisibility (Variables|/Game/StarterContent/Blueprints/Blueprint_Effect_Steam.Blueprint_Effect_Steam_C|GetP_Steam_Lit (Variables|Default|GetAs%20Blueprint%20Effect%20Steam)) false false))

(event Collision|EventActorBeginOverlap
  (params (OtherActor :type Actor%20Object%20Reference)))

(event EventTick
  (params (DeltaSeconds :type Float%20%28single-precision%29))
  (if (Variables|Default|GetIsRotating)
    (Transformation|AddLocalRotation (Variables|Default|GetPickupable) (Math|Rotator|MakeRotator 0.0 0.0 (* DeltaSeconds (Variables|Default|GetRotation))) false false)))

(fn ConstructionScript
  (|CallParentFunction))