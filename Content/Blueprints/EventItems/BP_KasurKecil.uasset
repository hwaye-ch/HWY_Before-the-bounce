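; Small bed (kasur) event item that lets the player sleep to advance to chapter 5.
; It becomes interactable when its KasurEnabler fires the wake-up-from-nightmare event.
; Interaction shows a sleep choice dialogue with data-table text, unless a valid SkipDialogue reference bypasses it.
; Yes sets a Determination flag and joins the one-shot sleep path (save, fade out, play chapter), while No re-arms the prompt.
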(event ExecuteOption(BP_ChoiceDialogueComponent)
  (params (Chosen%20Option :type E_ChoiceDialogue%20Enum :default "NewEnumerator0"))
  (bind _bp_fadescreencomponent (Variables|Default|GetBP_FadeScreenComponent))
  (switch Utilities|FlowControl|Switch|SwitchonE_ChoiceDialogue Chosen%20Option
    (:NewEnumerator0
      (Default|SetDetermination (Variables|Default|GetGame%20Instance%20Ref) "NewEnumerator0" false)
      (Utilities|FlowControl|DoOnce false
        (:Completed
          (Development|PrintString "Executing Sleep and Go to Next Chapter")
          (Default|SaveChapter (Variables|Default|GetGame%20Instance%20Ref) "NewEnumerator4")
          (Default|FadeOut _bp_fadescreencomponent 1e+01 (Variables|Default|GetPlayerRef))
          (EventDispatchers|AssignOnFadeOut _bp_fadescreencomponent (delegate Custom|OnFadeOut_Event))
          (Variables|Default|SetHide%20Outline? true)
          (EventDispatchers|UnbindallEventsfromExecuteOption (Variables|Default|GetBP_ChoiceDialogueComponent)))))
    (:NewEnumerator1
      (Utilities|FlowControl|DoOnce false) ; enters at Reset
    )))

(event Custom|Enable%20Kasur
  (params (PlayerPref :type BP%20First%20Person%20Character%20Object%20Reference))
  (Development|PrintString "Kasur is ready to interact")
  (Variables|Default|SetCanInteract? true))

(event Custom|OnFadeOut_Event
  (Default|PlayChapter (Variables|Default|GetPlayerRef) 5))

(event EventBeginPlay
  (|CallParentFunction)
  (bind _kasurenabler (Variables|Default|GetKasurEnabler)
    (:then
      (EventDispatchers|BindEventtoWakeUpfromNightmare _kasurenabler (delegate Custom|Enable%20Kasur)))
    (:else)))

(event EventInteractObject
  (bind _bp_fadescreencomponent (Variables|Default|GetBP_FadeScreenComponent))
  (Variables|Default|GetSkip%20Dialogue?
    (:then
      (Utilities|FlowControl|DoOnce false
        (:Completed
          (Development|PrintString "Executing Sleep and Go to Next Chapter")
          (Default|SaveChapter (Variables|Default|GetGame%20Instance%20Ref) "NewEnumerator4")
          (Default|FadeOut _bp_fadescreencomponent 1e+01 (Variables|Default|GetPlayerRef))
          (EventDispatchers|AssignOnFadeOut _bp_fadescreencomponent (delegate Custom|OnFadeOut_Event))
          (Variables|Default|SetHide%20Outline? true)
          (EventDispatchers|UnbindallEventsfromExecuteOption (Variables|Default|GetBP_ChoiceDialogueComponent)))))
    (:else
      (Utilities|FlowControl|DoOnce false
        (:Completed
          (bind (_extracted_text _extracted_text2 _extracted_text3) (|ExtractText))
          (bind _choice_dialogue_component (Default|ConstructChoiceDialogue (Variables|Default|GetBP_ChoiceDialogueComponent) _extracted_text _extracted_text2 _extracted_text3))
          (Default|ShowChoiceDialogue _choice_dialogue_component (Variables|Default|GetPlayerRef)))))))

(fn ConstructionScript
  (|CallParentFunction))