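; BP_MomOnBed is an event item actor that reveals a hidden mom figure, presumably on a bed.
; BeginPlay hides the skeletal mesh.
; The DisplayMom event, triggered from outside this graph, shows the mesh and a spotlight and plays the SfxMom sound.
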(event Custom|Display%20Mom
  (Rendering|SetVisibility (Variables|Default|GetSkeletalMesh) true false)
  (Rendering|SetVisibility (Variables|Default|GetSpotLight) true false)
  (Audio|Components|Audio|Play (Variables|Default|Getsfx_mom) 0.0))

(event EventBeginPlay
  (|CallParentFunction)
  (Rendering|SetVisibility (Variables|Default|GetSkeletalMesh) false false))

(fn ConstructionScript
  (|CallParentFunction))