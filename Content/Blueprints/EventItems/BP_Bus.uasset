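; BP_Bus is an event item that stages a bus cutscene for the player, showing the Michael component in chapters 1 and 2.
; Execute resets the bus to its starting location, activates its child-actor BP_BusCamera and plays the Anim_Bus level sequence.
; TakeOffBus fades the screen, then ends the camera and restores ambience volume when the fade finishes.
; A separate event hides Michael.
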(event Custom|Take%20Off%20Bus
  (bind _bp_fadescreencomponent (Variables|Default|GetBP_FadeScreenComponent))
  (Default|FadeEvent _bp_fadescreencomponent 3.0 (Variables|Default|GetPlayer%20Ref) 0.0)
  (EventDispatchers|BindEventtoOnFadeEventFinished _bp_fadescreencomponent (delegate Custom|End%20Bus%20Camera)))

(event Custom|End%20Bus%20Camera
  (bind _as_bp_bus_camera (Variables|Default|GetAs%20BP%20Bus%20Camera)
    (:then
      (Default|EndLevelCamera _as_bp_bus_camera)
      (bind _ambience (Variables|Default|GetAmbience)
        (:then
          (Default|SetAmbienceVolume _ambience 1.0))
        (:else)))
    (:else)))

(event Custom|HIde%20Mikey
  (Rendering|SetVisibility (Variables|Default|GetMichael) false false))

(event EventBeginPlay
  (|CallParentFunction)
  (Variables|Default|SetInitial%20Location (Transformation|GetActorLocation))
  (Utilities|FlowControl|DelayUntilNextTick)
  (bind _returnvalue (Actor|GetActorOfClass "/Game/Blueprints/Levels/BP_AmbienceSound.BP_AmbienceSound_C"))
  (Variables|Default|SetAmbience _returnvalue)
  (bind _current_chapter (Default|GetCurrentChapter (Variables|Default|GetPlayer%20Ref)))
  (switch int _current_chapter
    (:1
      _)
    (:2
      _))
  (Rendering|SetVisibility (Variables|Default|GetMichael) true false))

(event EventExecute
  (Transformation|SetActorLocation (Variables|Default|GetInitial%20Location) false true)
  (bind _asbp_bus_camera (Utilities|Casting|CastToBP_BusCamera (Variables|/Script/Engine.ChildActorComponent|GetChildActor (Variables|Default|GetChildActor))))
  (bind _output_get (Variables|Default|SetAs%20BP%20Bus%20Camera _asbp_bus_camera))
  (Default|InitializeLevelCamera _output_get (Variables|Default|GetPlayer%20Ref) 0.0 false)
  (bind _returnvalue (Sequencer|Player|CreateLevelSequencePlayer "/Game/Animation/Anim_Bus.Anim_Bus"))
  (Sequencer|Player|Play _returnvalue :!class /Script/MovieScene.MovieSceneSequencePlayer)
  (Variables|Default|GetAmbience
    (:then)
    (:else)))

(fn ConstructionScript
  (|CallParentFunction))