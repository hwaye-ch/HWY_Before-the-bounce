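; BP_Koran is a readable event item, apparently a newspaper, used in Chapter 7A.
; On BeginPlay it finds and caches the BP_Chapter7AManager actor.
; Reading it plays a newspaper sound.
; The first time it is put down, it turns off its cue and, if the manager is valid, tells it to store the sequence state.
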(event EventBeginPlay
  (|CallParentFunction)
  (bind _returnvalue (Actor|GetActorOfClass "/Game/Blueprints/Chapters/BP_Chapter7AManager.BP_Chapter7AManager_C"))
  (Variables|Default|SetChapter7Manager _returnvalue))

(event EventUnreadObject
  (Utilities|FlowControl|DoOnce false
    (:Completed
      (CallFunction|SetCue false)
      (bind _chapter7manager (Variables|Default|GetChapter7Manager)
        (:then
          (Default|StoreSequenceStateEvent _chapter7manager))
        (:else)))))

(event EventReadObject
  (Audio|Components|Audio|Play (Variables|Default|GetNewspaperSound) 0.0))

(fn ConstructionScript
  (|CallParentFunction))