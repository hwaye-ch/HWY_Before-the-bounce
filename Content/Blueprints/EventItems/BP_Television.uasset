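; BP_Television is an interactive TV prop that plays video with sound and a flickering screen light.
; Scripted events start and stop an NBA broadcast, while Interact, when enabled, toggles a separate footage screen through a FlipFlop.
; Timelines animate light intensity and fade the basketball audio when StopTV runs.
; PlayCrazyDisturbance recursively cycles power with shrinking delays, then sets a stop flag intended to leave the TV on.
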(event Custom|Turn%20On%20TV
  (bind _mediaplayer (Variables|Default|GetMediaPlayer))
  (Rendering|SetVisibility (Variables|Default|GetLight) true false)
  (Rendering|SetVisibility (Variables|Default|GetScreen%20TV) true false)
  (Audio|SpawnSoundatLocation "/Game/Sounds/sfx_tv-turn.sfx_tv-turn" (Transformation|GetWorldLocation (Variables|Default|GetProperty%20Item)) "0, 0, 0" 1.0 0.9 0.0 "/Game/Sounds/BasketballBounce/SA_ProximitySound.SA_ProximitySound" 0)
  (Media|MediaPlayer|OpenSource _mediaplayer "/Game/Media/nba.nba")
  (Media|MediaPlayer|Play _mediaplayer :!class /Script/MediaAssets.MediaPlayer)
  (bind _nbasound (Variables|Default|GetNbaSound)
    (:then
      (Audio|Components|Audio|SetVolumeMultiplier _nbasound 0.3 :!class /Script/Engine.AudioComponent)
      (bind _light_intensity (Timeline|FlashingLightTime Play)
        (:Update
          (Rendering|Components|Light|SetIntensity (Variables|Default|GetLight) (* _light_intensity 2e+02)))))
    (:else
      (bind _returnvalue (Audio|SpawnSoundatLocation "/Game/Sounds/sfx_basketball-match.sfx_basketball-match" (Transformation|GetWorldLocation (Variables|Default|GetProperty%20Item)) "0, 0, 0" 0.3 1.0 0.0 "/Game/Sounds/BasketballBounce/SA_ProximitySound.SA_ProximitySound" 0 false))
      (Variables|Default|SetNbaSound _returnvalue)
      (Timeline|FlashingLightTime Play))))

(event Custom|Turn%20Off%20TV
  (Audio|SpawnSoundatLocation "/Game/Sounds/sfx_tv-turn.sfx_tv-turn" (Transformation|GetWorldLocation (Variables|Default|GetProperty%20Item)) "0, 0, 0" 1.0 1.0 0.0 "/Game/Sounds/BasketballBounce/SA_ProximitySound.SA_ProximitySound" 0)
  (Rendering|SetVisibility (Variables|Default|GetLight) false false)
  (Rendering|SetVisibility (Variables|Default|GetScreen%20TV) false false)
  (Audio|Components|Audio|SetVolumeMultiplier (Variables|Default|GetNbaSound) 0.001 :!class /Script/Engine.AudioComponent)
  (bind _light_intensity (Timeline|FlashingLightTime Stop)
    (:Update
      (Rendering|Components|Light|SetIntensity (Variables|Default|GetLight) (* _light_intensity 2e+02)))))

(event Custom|Play%20Crazy%20Disturbance
  (Utilities|FlowControl|Delay (Variables|Default|GetDuration))
  (CallFunction|TurnonTV)
  (Utilities|FlowControl|Delay (Variables|Default|GetDuration))
  (CallFunction|TurnOffTV)
  (Variables|Default|GetShouldStop?
    (:then
      (CallFunction|TurnonTV))
    (:else
      (CallFunction|PlayCrazyDisturbance)
      (if (>= (Variables|Default|GetDuration) 0.3)
        (Variables|Default|SetDuration (- (Variables|Default|GetDuration) 0.1))
        (else
          (Utilities|FlowControl|Delay 5.0)
          (Variables|Default|SetShouldStop? true))))))

(event Custom|Play%20TV
  (bind _mediaplayer (Variables|Default|GetMediaPlayer))
  (Rendering|SetVisibility (Variables|Default|GetLight) true false)
  (Rendering|SetVisibility (Variables|Default|GetScreen%20TV) true false)
  (Media|MediaPlayer|OpenSource _mediaplayer "/Game/Media/nba.nba")
  (Media|MediaPlayer|Play _mediaplayer :!class /Script/MediaAssets.MediaPlayer)
  (Components|Activation|Activate (Variables|Default|Getbasketball%20sound) false)
  (bind _light_intensity (Timeline|Timeline Play)
    (:Update
      (Rendering|Components|Light|SetIntensity (Variables|Default|GetLight) (* _light_intensity 2e+02)))))

(event Custom|Stop%20TV
  (Rendering|SetVisibility (Variables|Default|GetLight) false false)
  (Rendering|SetVisibility (Variables|Default|GetScreen%20TV) false false)
  (Sequencer|Player|Pause (Variables|Default|GetMediaPlayer))
  (bind _newtrack_0 (Timeline|Timeline_0 Play)
    (:Update
      (Audio|Components|Audio|SetVolumeMultiplier (Variables|Default|Getbasketball%20sound) (Math|Float|Lerp 1.0 0.0 _newtrack_0) :!class /Script/Engine.AudioComponent))))

(event EventBeginPlay
  (|CallParentFunction)
  (Rendering|SetVisibility (Variables|Default|GetLight) false false))

(event EventInteract
  (params (PlayerRef :type BP%20First%20Person%20Character%20Object%20Reference))
  (bind _mediaplayer (Variables|Default|GetMediaPlayer))
  (bind _sfx_footage_hwaye (Variables|Default|Getsfx_footage-hwaye))
  (Variables|Default|GetIs%20Enabled?
    (:then
      (Audio|SpawnSoundatLocation "/Game/Sounds/sfx_tv-turn.sfx_tv-turn" (Transformation|GetWorldLocation (Variables|Default|GetProperty%20Item)) "0, 0, 0" 1.0 1.0 0.0 "/Game/Sounds/BasketballBounce/SA_ProximitySound.SA_ProximitySound" 0)
      (bind _isa (Utilities|FlowControl|FlipFlop)
        (:A
          _)
        (:B
          _))
      (Rendering|SetVisibility (Variables|Default|GetLight) _isa false)
      (Variables|Default|SetIs%20TV%20On? _isa)
      (if _isa
        (Media|MediaPlayer|OpenSource _mediaplayer "/Game/Media/footage.footage")
        (Media|MediaPlayer|Play _mediaplayer :!class /Script/MediaAssets.MediaPlayer)
        (Components|Activation|Activate _sfx_footage_hwaye false)
        (Audio|Components|Audio|SetVolumeMultiplier _sfx_footage_hwaye 0.3 :!class /Script/Engine.AudioComponent)
        (bind _light_intensity (Timeline|Timeline_1 Play)
          (:Update
            (Rendering|Components|Light|SetIntensity (Variables|Default|GetLight) (* _light_intensity 2e+02))))
        (else
          (Sequencer|Player|Pause _mediaplayer)
          (Audio|Components|Audio|SetVolumeMultiplier (Variables|Default|Getsfx_footage-hwaye) 0.001 :!class /Script/Engine.AudioComponent)
          (Timeline|Timeline_1 Play))))
    (:else)))

(fn ConstructionScript
  (|CallParentFunction))