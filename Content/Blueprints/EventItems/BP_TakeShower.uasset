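; Interactable event item for taking a shower, locked until its Enabler's EnableShower event sets CanInteract.
; Interacting works once: it runs a timed screen fade through the fade component, plays the shower sound and shows an auto dialogue from the Chapter 1 table, then hides its outline.
; When the fade finishes, it calls the enable-frame event to trigger what follows and unbinds from the fade callback.
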(event Custom|OnFadeEventFinished_Event
  (Development|PrintString "Showering Finished: Executing Frame Event")
  (Default|CallEnableFrameEvent)
  (EventDispatchers|UnbindallEventsfromOnFadeEventFinished (Variables|Default|GetBP_FadeScreenComponent)))

(event Custom|Set%20Shower%20Active
  (Variables|Default|SetCanInteract? true))

(event EventBeginPlay
  (bind _enabler (Variables|Default|GetEnabler)
    (:then
      (EventDispatchers|BindEventtoEnableShower _enabler (delegate Custom|Set%20Shower%20Active)))
    (:else)))

(event EventInteractObject
  (Utilities|FlowControl|DoOnce false
    (:Completed
      (EventDispatchers|AssignOnFadeEventFinished (Variables|Default|GetBP_FadeScreenComponent) (delegate Custom|OnFadeEventFinished_Event))
      (Default|FadeEvent (Variables|Default|GetBP_FadeScreenComponent) (Variables|Default|GetShowerDuration) (Variables|Default|GetPlayerRef) 0.0)
      (Utilities|FlowControl|Delay 1.0)
      (Audio|PlaySound2D "/Game/Sounds/sfx_shower.sfx_shower" 1.0 1.0 0.0 0 0)
      (Utilities|FlowControl|Delay 3.0)
      (bind _dialoguecomponent (Default|ConstructDialogue (Variables|Default|GetBP_DialogueComponent) "ch1_shower" "/Game/Dialogue/Chapter1_Dialogue.Chapter1_Dialogue" false false))
      (Default|DisplayAutoDialogue _dialoguecomponent)
      (Variables|Default|SetHide%20Outline? true))))

(fn ConstructionScript
  (|CallParentFunction))