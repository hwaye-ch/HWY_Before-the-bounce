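; Interactable consultation letter from Sarah in Chapter 7, examined through a level camera.
; While RunEvent is set, the first interaction clears the cue and, after a short delay, plays the letter dialogue with movement and look blocked.
; When dialogue ends, or directly without the event, the interact button is bound to exit the camera.
; Exiting with the event pending tells BP_Chapter7AManager to store sequence state and clears RunEvent.
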(event Custom|InteractButtonPressed_Event
  (Default|EndLevelCamera (Variables|Default|GetAs%20BP%20Level%20Camera))
  (Variables|/Game/FirstPerson/Blueprints/BP_FirstPersonCharacter.BP_FirstPersonCharacter_C|SetIsInteractButtonPriority? (Variables|Default|GetPlayerRef) false)
  (EventDispatchers|UnbindallEventsfromInteractButtonPressed (Variables|Default|GetPlayerRef))
  (Variables|Default|GetRunEvent?
    (:then
      (Utilities|FlowControl|DelayUntilNextTick)
      (EventDispatchers|UnbindallEventsfromOnDialogueEnded (Variables|Default|GetBP_DialogueComponent))
      (bind _chapter7manager (Variables|Default|GetChapter7Manager)
        (:then
          (Default|StoreSequenceStateEvent _chapter7manager)
          (Variables|Default|SetRunEvent? false))
        (:else)))
    (:else)))

(event Custom|OnDialogueEnded_Event
  (Variables|/Game/FirstPerson/Blueprints/BP_FirstPersonCharacter.BP_FirstPersonCharacter_C|SetIsInteractButtonPriority? (Variables|Default|GetPlayerRef) true)
  (EventDispatchers|AssignInteractButtonPressed (Variables|Default|GetPlayerRef) (delegate Custom|InteractButtonPressed_Event)))

(event EventBeginPlay
  (|CallParentFunction)
  (bind _returnvalue (Actor|GetActorOfClass "/Game/Blueprints/Chapters/BP_Chapter7AManager.BP_Chapter7AManager_C"))
  (Variables|Default|SetChapter7Manager _returnvalue))

(event EventInteractObject
  (bind _bp_dialoguecomponent (Variables|Default|GetBP_DialogueComponent))
  (bind _asbp_level_camera (Utilities|Casting|CastToBP_LevelCamera (Variables|/Script/Engine.ChildActorComponent|GetChildActor (Variables|Default|GetChildActor))))
  (bind _output_get (Variables|Default|SetAs%20BP%20Level%20Camera _asbp_level_camera))
  (Default|InitializeLevelCamera _output_get (Variables|Default|GetPlayerRef) 0.0 false)
  (Variables|Default|GetRunEvent?
    (:then
      (Utilities|FlowControl|DoOnce false
        (:Completed
          (CallFunction|SetCue false)
          (Utilities|FlowControl|Delay 3.0)
          (EventDispatchers|AssignOnDialogueEnded _bp_dialoguecomponent (delegate Custom|OnDialogueEnded_Event))
          (bind _dialoguecomponent (Default|ConstructDialogue _bp_dialoguecomponent "ch7_letter_1" "/Game/Dialogue/Chapter7_Dialogue.Chapter7_Dialogue" true true))
          (Default|ShowDialogue _dialoguecomponent (Variables|Default|GetPlayerRef) self))))
    (:else
      (Variables|/Game/FirstPerson/Blueprints/BP_FirstPersonCharacter.BP_FirstPersonCharacter_C|SetIsInteractButtonPriority? (Variables|Default|GetPlayerRef) true)
      (EventDispatchers|AssignInteractButtonPressed (Variables|Default|GetPlayerRef) (delegate Custom|InteractButtonPressed_Event)))))

(fn ConstructionScript
  (|CallParentFunction))