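; Mom jumpscare actor that ends in game over, starting hidden with its spotlight off and armed through a Trigger binding.
; When fired, a timeline locks player input and rotates the view using a look-at toward the mother.
; After a delay, it switches to a child-actor BP_MomCamera, lights the spotlight, plays the scare sound, then sets game over.
; RunMother, uncalled here, slides the actor horizontally to in front of the player's camera.
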(event Custom|Initiate%20Jumpscare
  (CallFunction|LookatMother)
  (Utilities|FlowControl|Delay 1.0)
  (bind _asbp_mom_camera (Utilities|Casting|CastToBP_MomCamera (Variables|/Script/Engine.ChildActorComponent|GetChildActor (Variables|Default|GetChildActor))))
  (Variables|Default|SetAs%20BP%20Mom%20Camera _asbp_mom_camera)
  (Default|InitializeLevelCamera _asbp_mom_camera (Variables|Default|GetPlayerRef) 0.1)
  (Rendering|SetVisibility (Variables|Default|GetSpotLight) true false)
  (Audio|SpawnSound2D "/Game/Sounds/sfx_jumpscare.sfx_jumpscare" 0.5 1.0 0.0 0)
  (Default|SetLook (Variables|Default|GetAs%20BP%20Mom%20Camera) false)
  (Utilities|FlowControl|Delay 5.0)
  (Default|SetGameOver (Variables|Default|GetPlayerRef) 6))

(event Custom|Run%20Mother
  (bind _playerref (Variables|Default|GetPlayerRef))
  (bind _firstpersoncamera (Variables|/Game/FirstPerson/Blueprints/BP_FirstPersonCharacter.BP_FirstPersonCharacter_C|GetFirstPersonCamera _playerref))
  (Variables|Default|SetEnd%20Location (+ (Transformation|GetWorldLocation _firstpersoncamera) (* (Math|Vector|GetForwardVector _firstpersoncamera) 2e+02)))
  (bind _newtrack_0 (Timeline|Timeline PlayFromStart)
    (:Update
      (Transformation|SetActorLocation (Math|Vector|MakeVector (.x (Math|Vector|Lerp(Vector) (Variables|Default|GetStart%20Location) (Variables|Default|GetEnd%20Location) _newtrack_0)) (.y (Math|Vector|Lerp(Vector) (Variables|Default|GetStart%20Location) (Variables|Default|GetEnd%20Location) _newtrack_0)) (.z (Variables|Default|GetStart%20Location))) false false))))

(event Custom|Look%20at%20Mother
  (bind _playerref (Variables|Default|GetPlayerRef))
  (bind _firstpersoncamera (Variables|/Game/FirstPerson/Blueprints/BP_FirstPersonCharacter.BP_FirstPersonCharacter_C|GetFirstPersonCamera _playerref))
  (Timeline|Timeline_0 Play
    (:Update
      (Pawn|SetControlRotation (Game|GetPlayerController 0) (Math|Interpolation|RInterpTo (Math|Rotator|FindLookatRotation (Transformation|GetWorldLocation _firstpersoncamera) (Transformation|GetActorLocation)) (Transformation|GetWorldRotation _firstpersoncamera) 0.0 0.0))
      (Default|DisableMovementandLook (Variables|Default|GetPlayerRef)))))

(event EventBeginPlay
  (|CallParentFunction)
  (bind _trigger (Variables|Default|GetTrigger)
    (:then
      (EventDispatchers|BindEventtoSetMomJumpscare _trigger (delegate Custom|Initiate%20Jumpscare))
      (Variables|Default|SetStart%20Location (Transformation|GetActorLocation))
      (Rendering|SetVisibility (Variables|Default|GetSpotLight) false false)
      (Rendering|SetActorHiddenInGame true))
    (:else)))

(fn ConstructionScript
  (|CallParentFunction))