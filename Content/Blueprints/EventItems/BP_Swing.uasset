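; BP_Swing is an interactable swing event item that shows a level camera view and grants an achievement on first use.
; InteractObject blends to the BP_LevelCamera cached from its child actor, with dimmed light, then binds the interact button to end that view.
; A separate PlaySwing event plays a proximity-attenuated sound and rocks a component in roll through a timeline.
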(event Custom|Play%20Swing
  (bind _object_6 (Variables|Default|GetObject_6))
  (bind _relativerotation (Variables|/Script/Engine.SceneComponent|GetRelativeRotation _object_6))
  (Audio|SpawnSoundatLocation "/Game/Sounds/sfx_swing.sfx_swing" (Transformation|GetActorLocation) "0, 0, 0" 0.2 1.0 0.0 "/Game/Sounds/BasketballBounce/SA_ProximitySound.SA_ProximitySound" 0)
  (bind _newtrack_0 (Timeline|Timeline Play)
    (:Update
      (Transformation|SetRelativeRotation _object_6 (Math|Rotator|MakeRotator (Math|Float|MapRangeClamped _newtrack_0 -1.0 1.0 -5.0 5.0) (.pitch _relativerotation) (.yaw _relativerotation)) false false))))

(event Custom|InteractButtonPressed_Event
  (Default|UnsetInteractButtonPriority (Variables|Default|GetPlayerRef))
  (Default|EndLevelCamera (Variables|Default|GetAs%20BP%20Level%20Camera)))

(event EventInteractObject
  (bind _playerref (Variables|Default|GetPlayerRef))
  (bind _as_bp_level_camera (Variables|Default|GetAs%20BP%20Level%20Camera)
    (:then
      (Default|InitializeLevelCamera _as_bp_level_camera _playerref 0.3 true)
      (Default|SetInteractButtonPriority _playerref)
      (Utilities|FlowControl|Delay 0.3)
      (EventDispatchers|AssignInteractButtonPressed _playerref (delegate Custom|InteractButtonPressed_Event))
      (Utilities|FlowControl|DoOnce false
        (:Completed
          (Default|SetAchievement (Variables|Default|GetGame%20Instance%20Ref) "NewEnumerator4"))))
    (:else)))

(event EventBeginPlay
  (|CallParentFunction)
  (bind _asbp_level_camera (Utilities|Casting|CastToBP_LevelCamera (Variables|/Script/Engine.ChildActorComponent|GetChildActor (Variables|Default|GetChildActor))))
  (Variables|Default|SetAs%20BP%20Level%20Camera _asbp_level_camera))

(fn ConstructionScript
  (|CallParentFunction))