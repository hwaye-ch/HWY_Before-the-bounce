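; Mom NPC for Chapter 7A, repositioned and given dialogue as story events fire on BP_Chapter7AManager.
; On the move event she snaps to SpawnArea_Mom, stands, stops her cooking sound, builds her dialogue and awaits the manager's enable event.
; Once ready, talking shows the dialogue, triggers the door unlock and binds the goodbye move.
; That move snaps her to SpawnArea_Mom2, keeping her current height.
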(event Custom|MoveNPCs_Event
  (Utilities|FlowControl|Sequence
    (:then_0
      (bind _returnvalue (Actor|GetActorOfClass "/Game/Blueprints/Levels/SpawnArea_Mom.SpawnArea_Mom_C"))
      (Transformation|SetActorLocationAndRotation (Transformation|GetActorLocation _returnvalue) (Transformation|GetActorRotation _returnvalue))
      (Variables|Default|SetIsStanding true)
      (Default|ConstructDialogue (Variables|Default|GetBP_DialogueComponent) "ch7_mother_0" "/Game/Dialogue/Chapter7_Dialogue.Chapter7_Dialogue" true true)
      (EventDispatchers|AssignEnableDialogue (Variables|Default|GetChapterManager) (delegate Custom|EnableDialogue_Event)))
    (:then_1
      (Audio|Components|Audio|Stop (Variables|Default|GetCooking%20Sfx)))))

(event Custom|MoveNPCsToSayGoodbye_Event
  (bind _returnvalue (Actor|GetActorOfClass "/Game/Blueprints/Levels/SpawnArea_Mom2.SpawnArea_Mom2_C"))
  (Transformation|SetActorLocationAndRotation (Math|Vector|MakeVector (.x (Transformation|GetActorLocation _returnvalue)) (.y (Transformation|GetActorLocation _returnvalue)) (.z (Transformation|GetActorLocation))) (Transformation|GetActorRotation _returnvalue)))

(event Custom|EnableDialogue_Event
  (params (NPC :type E_NPC%20Enum :default "NewEnumerator0"))
  (if (Utilities|Enum|Equal(Enum) NPC "NewEnumerator0")
    (Variables|Default|SetIsEventReady true)
    (Utilities|FlowControl|DelayUntilNextTick)
    (EventDispatchers|UnbindallEventsfromEnableDialogue (Variables|Default|GetChapterManager))))

(event EventTalkwithObject
  (Variables|Default|GetIsEventReady
    (:then
      (Default|ShowDialogue (Variables|Default|GetBP_DialogueComponent) (Variables|Default|GetPlayerRef) self)
      (Default|CallUnlockDoor (Variables|Default|GetChapterManager))
      (EventDispatchers|AssignMoveNPCstoSayGoodbye (Variables|Default|GetChapterManager) (delegate Custom|MoveNPCsToSayGoodbye_Event)))
    (:else)))

(event EventBeginPlay
  (|CallParentFunction)
  (bind _returnvalue (Actor|GetActorOfClass "/Game/Blueprints/Items/BP_Chapter7AManager.BP_Chapter7AManager_C"))
  (bind _output_get (Variables|Default|SetChapterManager _returnvalue))
  (EventDispatchers|AssignMoveNPCs _output_get (delegate Custom|MoveNPCs_Event)))

(fn ConstructionScript
  (|CallParentFunction))