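; BP_Customer2 is the second supermarket customer in Chapter 1, whose mesh is visible only in that chapter.
; A buying level sequence ends by attaching the beer to the drop area.
; Its one-time, input-blocking dialogue plays a ka-ching sound on its action event.
; When dialogue ends, the customer takes the beer in hand and plays a go-home sequence, then notifies the chapter manager and destroys the beer.
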(event Custom|Start%20Sequence%20Customer%202
  (bind _returnvalue (Sequencer|Player|CreateLevelSequencePlayer "/Game/Animation/Anim_Customer2Buying.Anim_Customer2Buying"))
  (EventDispatchers|AssignOnFinished _returnvalue (delegate Custom|OnFinished_Event))
  (Sequencer|Player|Play _returnvalue :!class /Script/MovieScene.MovieSceneSequencePlayer))

(event Custom|OnAction_Event
  (Audio|PlaySound2D "/Game/Sounds/sfx_kaching.sfx_kaching" 1.0 1.0 0.0 0 0))

(event Custom|OnFinished_Event
  (bind _returnvalue (Actor|GetActorOfClass "/Game/Blueprints/Levels/Area_DropStuff.Area_DropStuff_C"))
  (bind _output_get (Variables|Default|SetArea_Drop _returnvalue))
  (Transformation|AttachComponentToComponent (Variables|Default|GetBeer) (Variables|/Game/Blueprints/ModularItems/BP_SpawnLocation.BP_SpawnLocation_C|GetDefaultSceneRoot _output_get) "" "SnapToTarget" "SnapToTarget" "KeepWorld" true))

(event Custom|OnDialogueEnded_Event
  (Utilities|FlowControl|Delay 2.0)
  (Transformation|DetachFromActor (Variables|Default|GetBeer) "KeepWorld" "KeepWorld" "KeepWorld")
  (CallFunction|TakeBeer)
  (Utilities|FlowControl|DelayUntilNextTick)
  (CallFunction|PlayGoHomeSequence)
  (Utilities|FlowControl|Delay 15.0)
  (Utilities|FlowControl|Sequence
    (:then_0
      (Default|ProceedtoGoHome (Variables|Default|GetChapter1Manager)))
    (:then_1
      (bind _beer (Variables|Default|GetBeer)
        (:then
          (Actor|DestroyActor _beer))
        (:else)))))

(event Custom|Take%20Beer
  (Variables|Default|GetBeer
    (:then
      _)
    (:else
      (bind _returnvalue (Game|SpawnActorfromClass "/Game/Blueprints/Items/BP_Beer.BP_Beer_C" (Transformation|GetSocketTransform (Variables|Character|GetMesh) "LeftHandSocket" "RTS_World") "Undefined" "MultiplyWithRoot" 0 0))
      (Variables|Default|SetBeer _returnvalue)))
  (Transformation|AttachComponentToComponent (Variables|Default|GetBeer) (Variables|Character|GetMesh) "LeftHandSocket" "SnapToTarget" "SnapToTarget" "KeepWorld" true))

(event EventTalkwithObject
  (Utilities|FlowControl|DoOnce false
    (:Completed
      (EventDispatchers|AssignOnActionDuringDialogue (Variables|Default|GetBP_DialogueComponent) (delegate Custom|OnAction_Event))
      (EventDispatchers|AssignOnDialogueEnded (Variables|Default|GetBP_DialogueComponent) (delegate Custom|OnDialogueEnded_Event))
      (bind _dialoguecomponent (Default|ConstructDialogue (Variables|Default|GetBP_DialogueComponent) "ch1_customer2" "/Game/Dialogue/Chapter1_Dialogue.Chapter1_Dialogue" true true))
      (Default|ShowDialogue _dialoguecomponent (Variables|Default|GetPlayerRef) self))))

(event EventBeginPlay
  (|CallParentFunction)
  (bind _returnvalue (Actor|GetActorOfClass "/Game/Blueprints/Chapters/BP_Chapter1SupermarketManager.BP_Chapter1SupermarketManager_C"))
  (Variables|Default|SetChapter1Manager _returnvalue)
  (if (== (Variables|/Game/System/HwyGameInstance.HwyGameInstance_C|GetCurrentChapter (Variables|Default|GetGame%20Instance%20Ref)) 1)
    (Rendering|SetVisibility (Variables|Character|GetMesh) true false)
    (else
      (Rendering|SetVisibility (Variables|Character|GetMesh) false false))))

(fn ConstructionScript
  (|CallParentFunction))