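; Customer Andy on the main map, who starts hidden without collision and runs a one-shot story conversation when talked to.
; In Chapter 2, dialogue events play a cash-register sound and send him home via level sequence carrying the milk, followed by another dialogue that triggers the manager's PlayWindah.
; Otherwise, his Chapter 7 dialogue leads to muted ambience, a black fade and an animated WBP_Semu screen that finishes the chapter.
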(event Custom|GoHome
  (bind (_level_sequence_actor _level_sequence) (CallFunction|PlayGoHomeSequence))
  (EventDispatchers|BindEventtoOnFinished _level_sequence (delegate Custom|OnCostumerFinishedShopping)))

(event Custom|OnDialogueEnded_Event_0
  (Default|PlayWindah (Variables|Default|GetChapter%20Manager)))

(event Custom|OnAction_Event
  (Audio|PlaySound2D "/Game/Sounds/sfx_kaching.sfx_kaching" 1.0 1.0 0.0 0 0))

(event Custom|OnDialogueEnded_Event_1
  (bind _bp_fadescreencomponent (Variables|Default|GetBP_FadeScreenComponent))
  (Audio|PlaySound2D "/Game/Sounds/sfx_creepy-whossh.sfx_creepy-whossh" 1.0 1.0 0.0 0 0)
  (Default|SetAmbienceVolume (Variables|/Game/Blueprints/Chapters/BP_Chapter7AManager.BP_Chapter7AManager_C|GetAmbience (Variables|Default|GetChapter7%20manager)) 0.0)
  (Utilities|FlowControl|Delay 4.0)
  (Default|ShowBlackScreen _bp_fadescreencomponent 3.0 (Variables|Default|GetPlayerRef))
  (EventDispatchers|AssignOnBlackScreenFinished _bp_fadescreencomponent (delegate Custom|OnBlackScreenFinished_Event)))

(event Custom|OnDialogueEnded_Event
  (EventDispatchers|UnbindEventfromOnDialogueEnded (Variables|Default|GetBP_DialogueComponent) (delegate Custom|OnDialogueEnded_Event))
  (Utilities|FlowControl|Delay 1.0)
  (CallFunction|GoHome)
  (bind _returnvalue (Actor|GetActorOfClass "/Game/Blueprints/EventItems/BP_Milk.BP_Milk_C"))
  (bind _output_get (Variables|Default|SetStuff _returnvalue))
  (Transformation|AttachComponentToComponent _output_get (Variables|Character|GetMesh) "RightHandSocket" "SnapToTarget" "SnapToTarget" "KeepWorld" false)
  (Utilities|FlowControl|Delay 1e+01)
  (bind _dialoguecomponent (Default|ConstructDialogue (Variables|Default|GetBP_DialogueComponent) "ch2_akhir2ini" "/Game/Dialogue/Chapter2_Dialogue.Chapter2_Dialogue" true true))
  (Default|ShowDialogue _dialoguecomponent (Variables|Default|GetPlayerRef) self)
  (EventDispatchers|AssignOnDialogueEnded _dialoguecomponent (delegate Custom|OnDialogueEnded_Event_0)))

(event Custom|OnCostumerFinishedShopping
  (Actor|DestroyActor (stale Custom|GoHome _level_sequence_actor))
  (Actor|DestroyActor)
  (Actor|DestroyActor (Variables|Default|GetStuff)))

(event Custom|OnBlackScreenFinished_Event
  (bind _returnvalue (UserInterface|CreateWidget "/Game/Blueprints/Widgets/WBP_Semu.WBP_Semu_C"))
  (UserInterface|Viewport|AddtoViewport _returnvalue 0)
  (UserInterface|Animation|PlayAnimation _returnvalue (Variables|/Game/Blueprints/Widgets/WBP_Semu.WBP_Semu_C|GetShowingSemu _returnvalue) 0.0 1 "Forward" 1.0 false)
  (Class|UserWidget|BindtoAnimationFinished _returnvalue (Variables|/Game/Blueprints/Widgets/WBP_Semu.WBP_Semu_C|GetShowingSemu _returnvalue) (delegate Custom|Return%20to%20menu)))

(event Custom|Return%20to%20menu
  (Class|UserWidget|UnbindfromAnimationFinished (stale Custom|OnBlackScreenFinished_Event _returnvalue) (Variables|/Game/Blueprints/Widgets/WBP_Semu.WBP_Semu_C|GetShowingSemu (stale Custom|OnBlackScreenFinished_Event _returnvalue)) (delegate Custom|Return%20to%20menu))
  (Default|OnChapterFinishedEvent (Variables|Default|GetChapter7%20manager))
  (Utilities|FlowControl|DelayUntilNextTick)
  (Widget|RemovefromParent (stale Custom|OnBlackScreenFinished_Event _returnvalue)))

(event EventTalkwithObject
  (bind _bp_dialoguecomponent (Variables|Default|GetBP_DialogueComponent))
  (if (== (Variables|/Game/System/HwyGameInstance.HwyGameInstance_C|GetCurrentChapter (Variables|Default|GetGame%20Instance%20Ref)) 2)
    (Utilities|FlowControl|DoOnce false
      (:Completed
        (EventDispatchers|AssignOnActionDuringDialogue _bp_dialoguecomponent (delegate Custom|OnAction_Event))
        (EventDispatchers|AssignOnDialogueEnded _bp_dialoguecomponent (delegate Custom|OnDialogueEnded_Event))
        (bind _dialoguecomponent (Default|ConstructDialogue _bp_dialoguecomponent "ch2_andy" "/Game/Dialogue/Chapter2_Dialogue.Chapter2_Dialogue" true true))
        (Default|ShowDialogue _dialoguecomponent (Variables|Default|GetPlayerRef) self)))
    (else
      (Utilities|FlowControl|DoOnce false
        (:Completed
          (bind _dialoguecomponent_2 (Default|ConstructDialogue (Variables|Default|GetBP_DialogueComponent) "ch7_andy" "/Game/Dialogue/Chapter7_Dialogue.Chapter7_Dialogue" true true))
          (Default|ShowDialogue _dialoguecomponent_2 (Variables|Default|GetPlayerRef) self)
          (EventDispatchers|AssignOnDialogueEnded _dialoguecomponent_2 (delegate Custom|OnDialogueEnded_Event_1)))))))

(event EventBeginPlay
  (|CallParentFunction)
  (bind _returnvalue (Actor|GetActorOfClass "/Game/Blueprints/Chapters/BP_Chapter2SupermarketManager.BP_Chapter2SupermarketManager_C"))
  (Variables|Default|SetChapter%20Manager _returnvalue)
  (Rendering|SetVisibility (Variables|Character|GetMesh) false false)
  (Collision|SetActorEnableCollision false))

(fn ConstructionScript
  (|CallParentFunction))