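; Customer character Windah for the Chapter 2 supermarket, visible only in chapter 2 or 0, who buys a food item from the player.
; A level sequence plays the purchase approach, then the item (Nasi, spawned as nachos in the hand by TakeAction) snaps to the drop area.
; A one-time talk runs dialogue whose actions trigger a kaching sound and dancing.
; Afterwards Windah takes the item home, and a follow-up hunger dialogue hands off to the manager's Mikey sequence.
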(event Custom|Start%20Sequence%20Customer%20Windah
  ;[0.15 0.15 0.15 0.5 72] Start Sequence
  (bind (_outactor _returnvalue) (Sequencer|Player|CreateLevelSequencePlayer "/Game/Animation/Anim_CustomerBuyingFromLeft.Anim_CustomerBuyingFromLeft"))
  (Class|LevelSequenceActor|AddBinding _outactor (|GetSequenceBinding) self false)
  (EventDispatchers|AssignOnFinished _returnvalue (delegate Custom|OnFinished_Event))
  (Sequencer|Player|Play _returnvalue :!class /Script/MovieScene.MovieSceneSequencePlayer))

(event Custom|OnDialogueEnded_Event_0
  (Default|PlayMikeySequence (Variables|Default|GetChapter2Manager))
  (bind _nasi (Variables|Default|GetNasi)
    (:then
      (Actor|DestroyActor _nasi))
    (:else)))

(event Custom|OnAction_Event
  (Variables|Default|GetIs%20Char%20Dancing?
    (:then
      (Variables|Default|SetIs%20Dancing true))
    (:else
      (Audio|PlaySound2D "/Game/Sounds/sfx_kaching.sfx_kaching" 1.0 1.0 0.0 0 0)
      (Variables|Default|SetIs%20Char%20Dancing? true))))

(event Custom|OnFinished_Event
  ;[0.15 0.15 0.15 0.5 72] Start Sequence
  (bind _returnvalue (Actor|GetActorOfClass "/Game/Blueprints/Levels/Area_DropStuff.Area_DropStuff_C"))
  (bind _output_get (Variables|Default|SetArea_Drop _returnvalue))
  (Transformation|AttachComponentToComponent (Variables|Default|GetNasi) (Variables|/Game/Blueprints/ModularItems/BP_SpawnLocation.BP_SpawnLocation_C|GetDefaultSceneRoot _output_get) "" "SnapToTarget" "SnapToTarget" "KeepWorld" true))

(event Custom|OnDialogueEnded_Event
  (EventDispatchers|UnbindallEventsfromOnDialogueEnded (Variables|Default|GetBP_DialogueComponent))
  (Variables|Default|SetIs%20Dancing false)
  (Utilities|FlowControl|Delay 2.0)
  (Transformation|DetachFromActor (Variables|Default|GetNasi) "KeepWorld" "KeepWorld" "KeepWorld")
  (CallFunction|TakeAction)
  (Utilities|FlowControl|DelayUntilNextTick)
  (CallFunction|PlayGoHomeSequence)
  (Utilities|FlowControl|Delay 5.0)
  (bind _dialoguecomponent (Default|ConstructDialogue (Variables|Default|GetBP_DialogueComponent) "ch2_hungry" "/Game/Dialogue/Chapter2_Dialogue.Chapter2_Dialogue" true true))
  (Default|ShowDialogue _dialoguecomponent (Variables|Default|GetPlayerRef) self)
  (EventDispatchers|AssignOnDialogueEnded _dialoguecomponent (delegate Custom|OnDialogueEnded_Event_0)))

(event EventTakeAction
  (Variables|Default|GetNasi
    (:then
      _)
    (:else
      (bind _returnvalue (Game|SpawnActorfromClass "/Game/Blueprints/ModularItems/BP_PropertyItem.BP_PropertyItem_C" (Transformation|GetSocketTransform (Variables|Character|GetMesh) "RightHandSocket" "RTS_World") "Undefined" "MultiplyWithRoot" 0 0))
      (Components|StaticMesh|SetStaticMesh (Variables|/Game/Blueprints/ModularItems/BP_PropertyItem.BP_PropertyItem_C|GetProperty%20Item _returnvalue) "/Game/Convenience_Store/Product_Meshes/SM_Nachos_01.SM_Nachos_01")
      (Collision|SetCollisionEnabled (Variables|/Game/Blueprints/ModularItems/BP_PropertyItem.BP_PropertyItem_C|GetProperty%20Item _returnvalue) "NoCollision")
      (Variables|Default|SetNasi _returnvalue)))
  (Transformation|AttachComponentToComponent (Variables|Default|GetNasi) (Variables|Character|GetMesh) "RightHandSocket" "SnapToTarget" "SnapToTarget" "KeepWorld" true))

(event EventTalkwithObject
  (bind _bp_dialoguecomponent (Variables|Default|GetBP_DialogueComponent))
  (Utilities|FlowControl|DoOnce false
    (:Completed
      (EventDispatchers|AssignOnActionDuringDialogue _bp_dialoguecomponent (delegate Custom|OnAction_Event))
      (EventDispatchers|AssignOnDialogueEnded _bp_dialoguecomponent (delegate Custom|OnDialogueEnded_Event))
      (bind _dialoguecomponent (Default|ConstructDialogue _bp_dialoguecomponent "ch2_windah" "/Game/Dialogue/Chapter2_Dialogue.Chapter2_Dialogue" true true))
      (Default|ShowDialogue _dialoguecomponent (Variables|Default|GetPlayerRef) self))))

(event EventBeginPlay
  (bind _game_instance_ref (Variables|Default|GetGame%20Instance%20Ref))
  (bind _currentchapter (Variables|/Game/System/HwyGameInstance.HwyGameInstance_C|GetCurrentChapter _game_instance_ref))
  (|CallParentFunction)
  (bind _returnvalue (Actor|GetActorOfClass "/Game/Blueprints/Chapters/BP_Chapter2SupermarketManager.BP_Chapter2SupermarketManager_C"))
  (Variables|Default|SetChapter2Manager _returnvalue)
  (if (or (== _currentchapter 2) (== _currentchapter 0))
    (Rendering|SetVisibility (Variables|Character|GetMesh) true false)
    (else
      (Rendering|SetVisibility (Variables|Character|GetMesh) false false))))

(fn ConstructionScript
  (|CallParentFunction))