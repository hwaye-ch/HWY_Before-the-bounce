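; Crawling "Mom" chase enemy that stages a scripted reveal, pursues the player, and triggers game over on contact.
; BeginPlay plays a long-shot camera intro with a jumpscare sting, shows a "RUN" prompt, enables player running and panic, then starts the chase after a delay.
; Pawn sensing drives AI MoveTo toward the player.
; Sphere overlap switches to a close-up child-actor camera with spotlight and sounds before calling game over.
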(event OnComponentBeginOverlap(Sphere)
  (params (OverlappedComponent :type Primitive%20Component%20Object%20Reference) (OtherActor :type Actor%20Object%20Reference) (OtherComp :type Primitive%20Component%20Object%20Reference) (OtherBodyIndex :type Integer) (bFromSweep :type Boolean) (SweepResult :type Hit%20Result%20Structure%20%28by%20ref%29))
  (Variables|Default|GetIsChasing
    (:then
      (if (== OtherActor (Variables|Default|GetTargetPlayer))
        (Transformation|SetRelativeRotation (Variables|Character|GetMesh) (Math|Rotator|MakeRotator 0.0 0.0 -9e+01) false false)
        (Variables|Default|SetIsEnd true)
        (Default|InitializeLevelCamera (Variables|Default|GetClose%20Camera) (Variables|Default|GetTargetPlayer) 0.1 false)
        (Rendering|SetVisibility (Variables|Default|GetSpotLight) true true)
        (Widget|RemovefromParent (Variables|Default|GetWidget))
        (Audio|Components|Audio|Stop (Variables|Default|GetAudio))
        (Audio|PlaySound2D "/Game/Sounds/sfx_croak.sfx_croak" 1.0 1.0 0.0 0 0)
        (Audio|Components|Audio|Stop (Variables|Default|GetBackground%20music))
        (Audio|PlaySound2D "/Game/Sounds/sfx_jumpscare2.sfx_jumpscare2" 1.0 1.0 0.0 0 0)
        (Utilities|FlowControl|Delay 2.0)
        (Default|SetGameOver (Variables|Default|GetTargetPlayer) 8 "NewEnumerator2" true)))
    (:else)))

(event OnSeePawn(PawnSensing)
  (params (Pawn :type Pawn%20Object%20Reference))
  (Variables|Default|GetIsChasing
    (:then
      (AI|AIMoveTo self "0, 0, 0" (Variables|Default|GetTargetPlayer) 1.0 false))
    (:else)))

(event Custom|Destroy
  (Audio|Components|Audio|FadeOut (Variables|Default|GetBackground%20music) 2.0 0.0 "Linear" :!class /Script/Engine.AudioComponent)
  (Utilities|FlowControl|Delay 2.0)
  (Actor|DestroyActor))

(event EventBeginPlay
  (Transformation|SetRelativeRotation (Variables|Character|GetMesh) (Math|Rotator|MakeRotator 0.0 0.0 -9e+01) false false)
  (bind _asbp_first_person_character (Utilities|Casting|CastToBP_FirstPersonCharacter (Game|GetPlayerCharacter 0)))
  (Variables|Default|SetTargetPlayer _asbp_first_person_character)
  (Utilities|FlowControl|Delay 1.0)
  (bind _asbp_level_camera (Utilities|Casting|CastToBP_LevelCamera (Variables|/Script/Engine.ChildActorComponent|GetChildActor (Variables|Default|GetLongCamera))))
  (bind _output_get (Variables|Default|SetLong%20Camera _asbp_level_camera))
  (Default|InitializeLevelCamera _output_get (Variables|Default|GetTargetPlayer) 0.1 false)
  (Utilities|FlowControl|Sequence
    (:then_0
      (Utilities|FlowControl|Delay 2.0)
      (Utilities|FlowControl|Sequence
        (:then_0
          (Default|EndLevelCamera (Variables|Default|GetLong%20Camera))
          (Utilities|FlowControl|Delay (Variables|Default|GetDelayBeforeChase))
          (Variables|Default|SetIsChasing true)
          (Variables|Default|SetIsCrawling true)
          (Transformation|SetRelativeRotation (Variables|Character|GetMesh) (Math|Rotator|MakeRotator 9e+01 0.0 -9e+01) false false)
          (bind _asbp_level_camera_2 (Utilities|Casting|CastToBP_LevelCamera (Variables|/Script/Engine.ChildActorComponent|GetChildActor (Variables|Default|GetChildActor))))
          (Variables|Default|SetClose%20Camera _asbp_level_camera_2))
        (:then_1
          (bind _returnvalue (UserInterface|CreateWidget "/Game/Blueprints/Widgets/WBP_Mission.WBP_Mission_C" 0 "RUN"))
          (bind _output_get_2 (Variables|Default|SetWidget _returnvalue))
          (UserInterface|Viewport|AddtoViewport _output_get_2 0)
          (Utilities|FlowControl|Sequence
            (:then_0
              (Utilities|FlowControl|Delay 3.0)
              (Widget|RemovefromParent _output_get_2))
            (:then_1
              (Variables|/Game/FirstPerson/Blueprints/BP_FirstPersonCharacter.BP_FirstPersonCharacter_C|SetCan%20Run? (Variables|Default|GetTargetPlayer) true)
              (Audio|Components|Audio|Play (Variables|Default|GetBackground%20music) 0.0)
              (Variables|/Game/FirstPerson/Blueprints/BP_FirstPersonCharacter.BP_FirstPersonCharacter_C|SetIsPanic (Variables|Default|GetTargetPlayer) true))))))
    (:then_1
      (Audio|SpawnSound2D "/Game/Sounds/sfx_piano_jumpscare.sfx_piano_jumpscare" 1.0 1.0 0.0 0))))

(fn ConstructionScript)