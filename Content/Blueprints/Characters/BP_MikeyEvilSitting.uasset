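; Seated evil Mikey character that, when talked to, runs the nightmare chapter's closing sequence and credits.
; It plays the Michael dialogue with movement and look blocked, then starts a long fade-out and plays a maniac sound.
; After the audio ends, it fires and unbinds BP_ChapterNightmare's finish event, then removes the fade if valid and shows the credit scene.
; When the credits animation finishes, it sets the current chapter to 9 and teleports to another map.
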(event Custom|OnDialogueEnded_Event
  (Default|FadeOut (Variables|Default|GetBP_FadeScreenComponent) 6e+01 (Variables|Default|GetPlayerRef))
  (Utilities|FlowControl|Delay 4.0)
  (bind _returnvalue (Audio|SpawnSound2D "/Game/Sounds/sfx_maniac.sfx_maniac" 1.0 1.0 0.0 0))
  (EventDispatchers|AssignOnAudioFinished _returnvalue (delegate Custom|OnAudioFinished_Event)))

(event Custom|OnAudioFinished_Event
  (bind _chapternightmare (Variables|Default|GetChapterNightmare))
  (Utilities|FlowControl|Delay 1e+01)
  (Default|CallOnChapterFinished _chapternightmare)
  (Utilities|FlowControl|DelayUntilNextTick)
  (EventDispatchers|UnbindallEventsfromOnChapterFinished _chapternightmare)
  (bind _fadeoutwidget (Variables|/Game/Blueprints/Components/BP_FadeScreenComponent.BP_FadeScreenComponent_C|GetFadeOutWidget (Variables|Default|GetBP_FadeScreenComponent))
    (:then
      (Widget|RemovefromParent _fadeoutwidget)
      (Utilities|FlowControl|Delay 2.0)
      (bind _returnvalue (UserInterface|CreateWidget "/Game/Blueprints/Widgets/WBP_CreditScene.WBP_CreditScene_C"))
      (UserInterface|Viewport|AddtoViewport _returnvalue 0)
      (UserInterface|Animation|PlayAnimation _returnvalue (Variables|/Game/Blueprints/Widgets/WBP_CreditScene.WBP_CreditScene_C|GetPlayCreditScene _returnvalue) 0.0 1 "Forward" 1.0 false)
      (Class|UserWidget|BindtoAnimationFinished _returnvalue (Variables|/Game/Blueprints/Widgets/WBP_CreditScene.WBP_CreditScene_C|GetPlayCreditScene _returnvalue) (delegate Custom|On%20Finished%20animation)))
    (:else)))

(event Custom|On%20Finished%20animation
  (bind _game_instance_ref (Variables|Default|GetGame%20Instance%20Ref))
  (Class|UserWidget|UnbindfromAnimationFinished (stale Custom|OnAudioFinished_Event _returnvalue) (Variables|/Game/Blueprints/Widgets/WBP_CreditScene.WBP_CreditScene_C|GetPlayCreditScene (stale Custom|OnAudioFinished_Event _returnvalue)) (delegate Custom|On%20Finished%20animation))
  (Variables|/Game/System/HwyGameInstance.HwyGameInstance_C|SetCurrentChapter _game_instance_ref 9)
  (Default|CallTeleporttoMap _game_instance_ref "NewEnumerator0"))

(event EventBeginPlay
  (|CallParentFunction)
  (bind _returnvalue (Actor|GetActorOfClass "/Game/Blueprints/Chapters/BP_ChapterNightmare.BP_ChapterNightmare_C"))
  (Variables|Default|SetChapterNightmare _returnvalue))

(event EventTalkwithObject
  (bind _dialoguecomponent (Default|ConstructDialogue (Variables|Default|GetBP_DialogueComponent) "ch7_michael" "/Game/Dialogue/Chapter7_Dialogue.Chapter7_Dialogue" true true))
  (Default|ShowDialogue _dialoguecomponent (Variables|Default|GetPlayerRef) self)
  (EventDispatchers|AssignOnDialogueEnded _dialoguecomponent (delegate Custom|OnDialogueEnded_Event)))

(fn ConstructionScript
  (|CallParentFunction))