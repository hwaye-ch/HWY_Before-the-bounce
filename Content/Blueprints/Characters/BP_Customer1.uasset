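; BP_Customer1 is the first Chapter 1 supermarket customer, visible and moved to its spawn area only in that chapter.
; Talking to it, once the event is ready, runs a one-time movement-locking dialogue with a cash-register sound on its action.
; When dialogue ends, it plays a go-home sequence with a soda can attached to its hand and has the chapter manager start Customer 2's sequence.
; The finished sequence destroys customer and can.
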(event Custom|GoHome
  (bind (_level_sequence_actor _level_sequence) (CallFunction|PlayGoHomeSequence))
  (EventDispatchers|BindEventtoOnFinished _level_sequence (delegate Custom|OnCostumerFinishedShopping))
  (Utilities|FlowControl|DoOnce false
    (:Completed
      (Default|PlayCustomer2Sequence (Variables|Default|GetChapter%20Manager)))))

(event Custom|OnAction_Event
  (Audio|PlaySound2D "/Game/Sounds/sfx_kaching.sfx_kaching" 1.0 1.0 0.0 0 0))

(event Custom|OnDialogueEnded_Event
  (Utilities|FlowControl|Delay 1.0)
  (CallFunction|GoHome)
  (bind _returnvalue (Actor|GetActorOfClass "/Game/Blueprints/EventItems/BP_SodaCan.BP_SodaCan_C"))
  (bind _output_get (Variables|Default|SetStuff _returnvalue))
  (Transformation|AttachComponentToComponent _output_get (Variables|Character|GetMesh) "RightHandSocket" "SnapToTarget" "SnapToTarget" "KeepWorld" false))

(event Custom|OnCostumerFinishedShopping
  (Actor|DestroyActor (stale Custom|GoHome _level_sequence_actor))
  (Actor|DestroyActor)
  (Actor|DestroyActor (Variables|Default|GetStuff)))

(event EventTalkwithObject
  (bind _bp_dialoguecomponent (Variables|Default|GetBP_DialogueComponent))
  (Variables|Default|GetIsEventReady?
    (:then
      (Utilities|FlowControl|DoOnce false
        (:Completed
          (EventDispatchers|AssignOnActionDuringDialogue _bp_dialoguecomponent (delegate Custom|OnAction_Event))
          (EventDispatchers|AssignOnDialogueEnded _bp_dialoguecomponent (delegate Custom|OnDialogueEnded_Event))
          (bind _dialoguecomponent (Default|ConstructDialogue _bp_dialoguecomponent "ch1_customer" "/Game/Dialogue/Chapter1_Dialogue.Chapter1_Dialogue" true true))
          (Default|ShowDialogue _dialoguecomponent (Variables|Default|GetPlayerRef) self))))
    (:else)))

(event EventBeginPlay
  (|CallParentFunction)
  (bind _returnvalue (Actor|GetActorOfClass "/Game/Blueprints/Chapters/BP_Chapter1SupermarketManager.BP_Chapter1SupermarketManager_C"))
  (Variables|Default|SetChapter%20Manager _returnvalue)
  (if (== (Variables|/Game/System/HwyGameInstance.HwyGameInstance_C|GetCurrentChapter (Variables|Default|GetGame%20Instance%20Ref)) 1)
    (Rendering|SetVisibility (Variables|Character|GetMesh) true false)
    (bind _returnvalue_2 (Actor|GetActorOfClass "/Game/Blueprints/Levels/SpawnArea_Customer1.SpawnArea_Customer1_C"))
    (Transformation|SetActorLocationAndRotation self (.location (Transformation|GetActorTransform _returnvalue_2)) (.rotation (Transformation|GetActorTransform _returnvalue_2)) false true)
    (else
      (Rendering|SetVisibility (Variables|Character|GetMesh) false false))))

(fn ConstructionScript
  (|CallParentFunction))