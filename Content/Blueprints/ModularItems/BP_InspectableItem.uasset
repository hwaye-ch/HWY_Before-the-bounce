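; Interactable item that the first-person player can pick up to inspect and rotate.
; Interact toggles inspection, locking player movement and look, hiding the world mesh and spawning a copy of its own class at the player's InspectablePosition.
; Look input rotates that copy.
; Interacting again destroys the copy, reveals the original, restores player control and calls ReturnObject.
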(event Input|EnhancedActionEvents|EnhancedInputActionIA_Look
  (params (ActionValue :type Vector%202D%20Structure) (ElapsedSeconds :type Float%20%28double-precision%29) (TriggeredSeconds :type Float%20%28double-precision%29) (InputAction :type Input%20Action%20Object%20Reference :default "/Game/FirstPerson/Input/Actions/IA_Look.IA_Look"))
  (if (Variables|Default|GetCanInspect?)
    (Transformation|AddLocalRotation (Variables|/Script/Engine.Actor|GetRootComponent (Variables|Default|GetInspectableObject)) (Math|Rotator|MakeRotator 0.0 (* (.y ActionValue) 0.4) (* (.x ActionValue) 0.4)) false false)))

(event EventInteract
  (params (PlayerRef :type BP%20First%20Person%20Character%20Object%20Reference))
  (bind _returnvalue (Game|GetPlayerController 0))
  (Variables|Default|SetPlayerRef PlayerRef)
  (CallFunction|InspectObject)
  (if (Variables|Default|GetCanInspect?)
    (Utilities|FlowControl|Sequence
      (:then_0
        (goto _label Reset))
      (:then_1
        (Variables|Default|SetCanInspect? false)
        (Variables|/Game/FirstPerson/Blueprints/BP_FirstPersonCharacter.BP_FirstPersonCharacter_C|SetActiveInspectableItem (Variables|Default|GetPlayerRef) 0)
        (Variables|/Game/FirstPerson/Blueprints/BP_FirstPersonCharacter.BP_FirstPersonCharacter_C|SetIsInspecting (Variables|Default|GetPlayerRef) false)
        (Pawn|Components|CharacterMovement|SetMovementMode (Variables|/Script/Engine.Character|GetCharacterMovement (Game|GetPlayerCharacter 0)) "MOVE_Walking" 0)
        (Variables|/Script/Engine.PlayerController|SetbShowMouseCursor _returnvalue false)
        (Input|ResetIgnoreLookInput _returnvalue)
        (Input|SetInputModeGameOnly _returnvalue false)
        (Actor|DestroyActor (Variables|Default|GetInspectableObject))
        (Rendering|SetVisibility (Variables|Default|GetInspectableItem) true true)
        (CallFunction|ReturnObject)))
    (else
      (Input|EnableInput (Game|GetPlayerController 0))
      (Utilities|FlowControl|DoOnce false :!label _label
        (:Completed
          (Variables|/Script/Engine.PlayerController|SetbShowMouseCursor (Game|GetPlayerController 0) false)
          (Variables|Default|SetCanInspect? true)
          (Variables|/Game/FirstPerson/Blueprints/BP_FirstPersonCharacter.BP_FirstPersonCharacter_C|SetActiveInspectableItem (Variables|Default|GetPlayerRef) self)
          (Variables|/Game/FirstPerson/Blueprints/BP_FirstPersonCharacter.BP_FirstPersonCharacter_C|SetIsInspecting (Variables|Default|GetPlayerRef) true)
          (Default|DisableMovementandLook (Variables|Default|GetPlayerRef))
          (bind _returnvalue_2 (Game|SpawnActorfromClass (Utilities|GetClass self) (Math|Transform|MakeTransform (.location (Transformation|GetWorldTransform (Variables|/Game/FirstPerson/Blueprints/BP_FirstPersonCharacter.BP_FirstPersonCharacter_C|GetInspectable%20Position (Variables|Default|GetPlayerRef)))) (.rotation (Transformation|GetWorldTransform (Variables|/Game/FirstPerson/Blueprints/BP_FirstPersonCharacter.BP_FirstPersonCharacter_C|GetInspectable%20Position (Variables|Default|GetPlayerRef)))) (Variables|/Script/Engine.SceneComponent|GetRelativeScale3D (Variables|Default|GetInspectableItem))) "Undefined" "MultiplyWithRoot" 0 false 0))
          (bind _output_get (Variables|Default|SetInspectableObject _returnvalue_2))
          (Default|SetCue _output_get false)
          (Rendering|SetVisibility (Variables|Default|GetInspectableItem) false true)
          (CallFunction|InspectObject))))))

(event EventBeginPlay
  (bind _inspectableitem (Variables|Default|GetInspectableItem))
  (Variables|Default|SetOriginal%20Location (Transformation|GetWorldLocation _inspectableitem))
  (Variables|Default|SetOriginal%20Rotation (Transformation|GetWorldRotation _inspectableitem))
  (bind _asbp_first_person_character (Utilities|Casting|CastToBP_FirstPersonCharacter (Game|GetPlayerCharacter 0)))
  (Variables|Default|SetPlayerRef _asbp_first_person_character))

(fn ConstructionScript)