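; Interactable modular door that swings open or shut, plays a locked sound, or calls a peek event.
; Interact checks the disable, peek, lock and in-motion states, then plays or reverses a timeline that lerps door yaw, with OpenForward selecting the angle.
; SetDoorClosed shuts it through a separate timeline, and BeginPlay reveals optional peephole meshes.
; StartPeeking and InteractDoor are empty hooks here.
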(event Custom|Start%20Peeking)

(event Custom|Set%20Door%20Closed
  (Variables|Default|GetIsDoorOpened
    (:then
      (bind _door_alpha (Timeline|Timeline PlayFromStart)
        (:Update
          (Transformation|SetRelativeRotation (Variables|Default|GetDoor) (Math|Rotator|MakeRotator 0.0 0.0 (Math|Float|Lerp (Variables|Default|GetYawValue) 0.0 _door_alpha)) false false)
          (Variables|Default|SetIsDoorOpened false))
        (:Finished
          (Variables|Default|SetIsOpening false))))
    (:else)))

(event EventBeginPlay
  (if (Variables|Default|GetShowPeepHole)
    (Rendering|SetVisibility (Variables|Default|GetSphere) true false)
    (Rendering|SetVisibility (Variables|Default|GetStaticMesh) true false)))

(event EventInteract
  (params (PlayerRef :type BP%20First%20Person%20Character%20Object%20Reference))
  (bind _returnvalue (Transformation|GetActorLocation))
  (Variables|Default|SetPlayer%20Pref PlayerRef)
  ;[0.15 0.15 0.15 0.5] v1.2.2
  (Variables|Default|GetDisable%20Interaction?
    (:then)
    (:else
      (if (Variables|Default|GetIsPeekMode)
        (CallFunction|StartPeeking)
        (elif (Variables|Default|GetIsLocked)
          (Audio|SpawnSoundatLocation "/Game/Sounds/sfx_locked-door.sfx_locked-door" (Transformation|GetActorLocation) "0, 0, 0" 1.0 1.0 0.0 "/Game/Sounds/BasketballBounce/SA_ProximitySound.SA_ProximitySound" 0)
          (elif (not (Variables|Default|GetIsOpening))
            (Variables|Default|SetIsOpening true)
            (CallFunction|InteractDoor (Variables|Default|GetIsDoorOpened))
            (if (Variables|Default|GetOpenForward)
              (Variables|Default|SetYawValue (Variables|Default|GetOpenBackwardValue))
              (else
                (Variables|Default|SetYawValue (Variables|Default|GetOpenForwardValue))))
            (bind _output_get (Variables|Default|SetIsDoorOpened (not (Variables|Default|GetIsDoorOpened))))
            (if _output_get
              (Audio|PlaySoundatLocation "/Game/Sounds/sfx_door_opened.sfx_door_opened" _returnvalue "0, 0, 0" 1.0 1.0 0.0 "/Game/Sounds/BasketballBounce/SA_ProximitySound.SA_ProximitySound" 0 0 0)
              (bind _door_alpha (Timeline|TL_Doors PlayFromStart)
                (:Update
                  (Transformation|SetRelativeRotation (Variables|Default|GetDoor) (Math|Rotator|MakeRotator 0.0 0.0 (Math|Float|Lerp 0.0 (Variables|Default|GetYawValue) _door_alpha)) false false))
                (:Finished
                  (Variables|Default|SetIsOpening false)))
              (else
                (Audio|PlaySoundatLocation "/Game/Sounds/sfx_door_closed.sfx_door_closed" _returnvalue "0, 0, 0" 1.0 1.0 0.0 "/Game/Sounds/BasketballBounce/SA_ProximitySound.SA_ProximitySound" 0 0 0)
                (Timeline|TL_Doors Reverse)))))))))

(fn ConstructionScript)

(fn InteractDoor
  (params (Open :type Boolean))
  (return))