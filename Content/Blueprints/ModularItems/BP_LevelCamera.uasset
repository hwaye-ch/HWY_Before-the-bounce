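; BP_LevelCamera is a placeable camera that temporarily replaces the first-person player's view, with blended transitions in and out.
; While active it registers as the player's override camera and disables normal movement and look, restoring both on exit.
; It offers optional clamped yaw/pitch look, a forward interaction trace and access to its post-process settings.
; Chromatic aberration can be set instantly or faded through a timeline.
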(event Custom|Set%20Look
  (params (Enabled? :type Boolean))
  (Variables|Default|SetIsLookEnabled? Enabled?))

(event Custom|Look%20Through%20Level%20Camera
  (params (Yaw :type Float%20%28double-precision%29) (Pitch :type Float%20%28double-precision%29))
  (Variables|Default|GetIsLookEnabled?
    (:then
      (Transformation|SetRelativeRotation (Variables|Default|GetCamera) (|CollapseGraph Yaw Pitch) false false))
    (:else)))

(event Custom|Initialize%20Level%20Camera
  (params (Player%20Ref :type BP%20First%20Person%20Character%20Object%20Reference) (Blend%20Time :type Float%20%28double-precision%29))
  (Variables|Default|SetPlayer%20Ref Player%20Ref)
  (bind _output_get (Variables|Default|SetBlend%20Time Blend%20Time))
  (Game|Player|SetViewTargetwithBlend (Game|GetPlayerController 0) self _output_get "VTBlend_Linear" 0.0 false)
  (Variables|/Game/FirstPerson/Blueprints/BP_FirstPersonCharacter.BP_FirstPersonCharacter_C|SetIsViewingThroughLevelCam? (Variables|Default|GetPlayer%20Ref) true)
  (Variables|/Game/FirstPerson/Blueprints/BP_FirstPersonCharacter.BP_FirstPersonCharacter_C|SetOverridedCamera (Variables|Default|GetPlayer%20Ref) self)
  (Default|DisableMovementandLook (Variables|Default|GetPlayer%20Ref)))

(event Custom|End%20Level%20Camera
  (Variables|/Game/FirstPerson/Blueprints/BP_FirstPersonCharacter.BP_FirstPersonCharacter_C|SetIsViewingThroughLevelCam? (Variables|Default|GetPlayer%20Ref) false)
  (Game|Player|SetViewTargetwithBlend (Game|GetPlayerController 0) (Variables|Default|GetPlayer%20Ref) (Variables|Default|GetBlend%20Time) "VTBlend_Linear" 0.0 false)
  (Variables|/Game/FirstPerson/Blueprints/BP_FirstPersonCharacter.BP_FirstPersonCharacter_C|SetOverridedCamera (Variables|Default|GetPlayer%20Ref) 0)
  (Default|EnableLookandMovement (Variables|Default|GetPlayer%20Ref)))

(event EventBeginPlay
  (bind _asbp_first_person_character (Utilities|Casting|CastToBP_FirstPersonCharacter (Game|GetPlayerCharacter 0)))
  (Variables|Default|SetPlayer%20Ref _asbp_first_person_character))

(event Custom|Set%20Chromatic%20Abberation%20to%20Camera
  (params (Activate? :type Boolean) (Intensity :type Float%20%28double-precision%29) (Instance? :type Boolean))
  (if Activate?
    (if Instance?
      (bind _structout (Utilities|Struct|SetmembersinPostProcessSettings (Variables|/Script/Engine.CameraComponent|GetPostProcessSettings (Variables|Default|GetCamera)) Intensity))
      (Variables|/Script/Engine.CameraComponent|SetPostProcessSettings (Variables|Default|GetCamera) _structout)
      (else
        (bind _newtrack_0 (Timeline|Timeline PlayFromStart)
          (:Update
            (bind _structout_2 (Utilities|Struct|SetmembersinPostProcessSettings (Variables|/Script/Engine.CameraComponent|GetPostProcessSettings (Variables|Default|GetCamera)) (Math|Float|Lerp (Variables|Default|GetCurrent%20Intensity) Intensity _newtrack_0)))
            (Variables|/Script/Engine.CameraComponent|SetPostProcessSettings (Variables|Default|GetCamera) _structout_2))
          (:Finished
            (Variables|Default|SetCurrent%20Intensity Intensity)))))
    (else
      (Variables|Default|SetCurrent%20Intensity 0.0)
      (Timeline|Timeline Reverse))))

(fn ConstructionScript
  (|CallParentFunction))

(fn GetCameraTrace
  (bind _camera (Variables|Default|GetCamera))
  (bind _returnvalue (Transformation|GetWorldLocation _camera))
  (return _returnvalue (+ (* (Math|Vector|GetForwardVector _camera) (Variables|Default|GetMaxInteractRange)) _returnvalue)))

(fn GetCameraPostProcessSetting
  (return (Variables|/Script/Engine.CameraComponent|GetPostProcessSettings (Variables|Default|GetCamera))))