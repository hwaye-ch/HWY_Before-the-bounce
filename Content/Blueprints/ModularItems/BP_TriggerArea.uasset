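; Modular trigger volume that fires OnOverlapTriggerMessage when the first-person player overlaps its CollisionBox, paired with a toggleable BarrierBox.
; A DoOnce and the IsDeactivated check gate the overlap, and ActivateOverlapTrigger re-arms both, also running at BeginPlay for DebugTrigger.
; The CollisionBox is destroyed after firing unless PreserveTrigger is set.
; SetCollisionSetting switches barrier collision, applied at BeginPlay from EnableCollision.
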(event OnComponentBeginOverlap(CollisionBox)
  (params (OverlappedComponent :type Primitive%20Component%20Object%20Reference) (OtherActor :type Actor%20Object%20Reference) (OtherComp :type Primitive%20Component%20Object%20Reference) (OtherBodyIndex :type Integer) (bFromSweep :type Boolean) (SweepResult :type Hit%20Result%20Structure%20%28by%20ref%29))
  (bind _asbp_first_person_character (Utilities|Casting|CastToBP_FirstPersonCharacter OtherActor))
  (Utilities|FlowControl|DoOnce true
    (:Completed
      (Variables|Default|SetPlayerRef _asbp_first_person_character)
      (Variables|Default|GetIs%20Deactivated?
        (:then)
        (:else
          (Class|BPITrigger|OnOverlapTrigger(Message) self)
          (if (not (Variables|Default|GetPreserve%20Trigger?))
            (Components|DestroyComponent (Variables|Default|GetCollisionBox))))))))

(event Custom|Activate%20Overlap%20Trigger
  (Variables|Default|SetIs%20Deactivated? false)
  (Utilities|FlowControl|DoOnce true) ; enters at Reset
)

(event Custom|Set%20Collision%20Setting
  (params (IsActive :type Boolean))
  (bind _output_get (Variables|Default|SetEnableCollision IsActive))
  (if _output_get
    (Collision|SetCollisionEnabled (Variables|Default|GetBarrierBox) "QueryAndPhysics")
    (else
      (Collision|SetCollisionEnabled (Variables|Default|GetBarrierBox) "NoCollision"))))

(event EventBeginPlay
  (Utilities|FlowControl|Sequence
    (:then_0
      (bind _ashwy_game_instance (Utilities|Casting|CastToHwyGameInstance (Game|GetGameInstance)))
      (Variables|Default|SetGame%20Instance%20Ref _ashwy_game_instance))
    (:then_1
      (CallFunction|SetCollisionSetting (Variables|Default|GetEnableCollision))
      (Variables|Default|GetDebug%20Trigger
        (:then
          (CallFunction|ActivateOverlapTrigger))
        (:else)))))

(fn ConstructionScript)