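; Chapter manager for the main menu that runs the startup flow from splash screen to menu.
; InitializeGame shows WBP_SplashScreen and binds the end of its animation to ShowMenu.
; ShowMenu swaps the splash for WBP_MainMenu, passing itself to the widget, then enables the cursor and Game and UI input.
; A helper function fetches localized text by data table and keyword through BPTextRelatedComponent.
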(event Custom|InitializeGame
  (bind _returnvalue (UserInterface|CreateWidget "/Game/Blueprints/Widgets/WBP_SplashScreen.WBP_SplashScreen_C"))
  (UserInterface|Viewport|AddtoViewport _returnvalue 0)
  (UserInterface|Animation|PlayAnimation _returnvalue (Variables|/Game/Blueprints/Widgets/WBP_SplashScreen.WBP_SplashScreen_C|GetSplashAnimation _returnvalue) 0.0 1 "Forward" 1.0 false)
  (Class|UserWidget|BindtoAnimationFinished _returnvalue (Variables|/Game/Blueprints/Widgets/WBP_SplashScreen.WBP_SplashScreen_C|GetSplashAnimation _returnvalue) (delegate Custom|Show%20Menu)))

(event Custom|Show%20Menu
  (bind _returnvalue (Game|GetPlayerController 0))
  (Widget|RemovefromParent (stale Custom|InitializeGame _returnvalue))
  (bind _returnvalue_2 (UserInterface|CreateWidget "/Game/Blueprints/Widgets/WBP_MainMenu.WBP_MainMenu_C" 0 self))
  (Default|InitializeWidget _returnvalue_2)
  (UserInterface|Viewport|AddtoViewport _returnvalue_2 0)
  (Variables|/Script/Engine.PlayerController|SetbShowMouseCursor _returnvalue true)
  (Input|SetInputModeGameandUI _returnvalue _returnvalue_2 "DoNotLock" true false))

(event EventBeginPlay
  (|CallParentFunction) ; This node is disabled and will not be called.\nDrag off pins to build functionality.
)

(fn ConstructionScript
  (|CallParentFunction))

(fn ExtractTextforLocalization
  (params (DataTable :type Data%20Table%20Object%20Reference) (Keyword :type Name))
  (bind _extracted_text (Default|ExtractText (Variables|Default|GetBP_TextRelatedComponent) DataTable Keyword))
  (return _extracted_text))