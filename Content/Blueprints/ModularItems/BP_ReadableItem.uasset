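; BP_ReadableItem is an interactable item that the player can read and dismiss.
; Interact toggles the player's IsReading flag and calls ReadItem or DismissItem.
; Reading shows a description widget from BPReadableComponent, plays its animation, locks movement and look, and registers the active item.
; Dismissal plays the closing animation, removes the widget after a delay and restores control, while SetInteraction sets collision and visibility.
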(event Custom|Set%20Collision
  (params (Enabled? :type Boolean))
  (if Enabled?
    (Collision|SetCollisionEnabled (Variables|Default|GetReadableItem) "QueryAndPhysics")
    (else
      (Collision|SetCollisionEnabled (Variables|Default|GetReadableItem) "NoCollision"))))

(event Custom|Set%20Interaction
  (params (Can%20Interact? :type Boolean) (Visible? :type Boolean))
  (bind _output_get (Variables|Default|SetCanInteract? Can%20Interact?))
  (CallFunction|SetCollision _output_get)
  (Rendering|SetVisibility (Variables|Default|GetReadableItem) Visible? false))

(event EventInteract
  (params (PlayerRef :type BP%20First%20Person%20Character%20Object%20Reference))
  (bind _output_get (Variables|Default|SetPlayer%20Ref PlayerRef))
  (bind _isreading (Variables|/Game/FirstPerson/Blueprints/BP_FirstPersonCharacter.BP_FirstPersonCharacter_C|GetIsReading _output_get)
    (:then
      (|DismissItem))
    (:else
      (|ReadItem)))
  (Variables|/Game/FirstPerson/Blueprints/BP_FirstPersonCharacter.BP_FirstPersonCharacter_C|SetIsReading (Variables|Default|GetPlayer%20Ref) (not _isreading)))

(fn ConstructionScript)