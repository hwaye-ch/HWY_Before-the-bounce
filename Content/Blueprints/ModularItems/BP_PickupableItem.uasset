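; Pickupable physics item that the player can pick up and throw through Interact.
; Pickup disables physics and collision and snaps the Pickupable component to the player's PickupPosition, gated by CanInteract.
; Throwing detaches it, restores physics, applies a forward velocity impulse scaled by the player's ThrowForce and clears the held-item state.
; Helper events show, hide or destroy the item, and construction sets initial visibility from HidePhysic.
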(event Custom|Destroy%20Item
  (Utilities|FlowControl|Delay 0.01)
  (Actor|DestroyActor))

(event Custom|Throw%20Object
  (bind _playerref (Variables|Default|GetPlayerRef))
  ;[0.15 0.15 0.15 0.5] Throw Object
  (Collision|SetCollisionEnabled (Variables|Default|GetPickupable) "QueryAndPhysics")
  (Transformation|DetachFromComponent (Variables|Default|GetPickupable) "KeepWorld" "KeepWorld" "KeepWorld" true)
  (Physics|SetSimulatePhysics (Variables|Default|GetPickupable) true)
  (Physics|AddImpulse (Variables|Default|GetPickupable) (* (Transformation|GetActorForwardVector _playerref) (Variables|/Game/FirstPerson/Blueprints/BP_FirstPersonCharacter.BP_FirstPersonCharacter_C|GetThrowForce _playerref)) "None" true)
  (Variables|/Game/FirstPerson/Blueprints/BP_FirstPersonCharacter.BP_FirstPersonCharacter_C|SetIsHoldingItem (Variables|Default|GetPlayerRef) false)
  (Utilities|FlowControl|Sequence
    (:then_0
      (Variables|/Game/FirstPerson/Blueprints/BP_FirstPersonCharacter.BP_FirstPersonCharacter_C|SetItemPicked (Variables|Default|GetPlayerRef) 0))
    (:then_1
      (CallFunction|ThrowObject))))

(event Custom|Show%20Item
  (Rendering|SetVisibility (Variables|Default|GetPickupable) true false)
  (Collision|SetCollisionEnabled (Variables|Default|GetPickupable) "QueryAndPhysics"))

(event Custom|Hide%20Item
  (Rendering|SetVisibility (Variables|Default|GetPickupable) false false)
  (Collision|SetCollisionEnabled (Variables|Default|GetPickupable) "NoCollision"))

(event EventInteract
  (params (PlayerRef :type BP%20First%20Person%20Character%20Object%20Reference))
  ;[0.15 0.15 0.15 0.5] Pick up Object
  (bind _output_get (Variables|Default|SetPlayerRef PlayerRef))
  (Variables|/Game/FirstPerson/Blueprints/BP_FirstPersonCharacter.BP_FirstPersonCharacter_C|GetIsHoldingItem _output_get
    (:then
      (CallFunction|ThrowObject))
    (:else
      (if (Variables|Default|GetCanInteract?)
        (Physics|SetSimulatePhysics (Variables|Default|GetPickupable) false)
        (Utilities|FlowControl|DelayUntilNextTick)
        (Collision|SetCollisionEnabled (Variables|Default|GetPickupable) "NoCollision")
        (Transformation|AttachComponentToComponent (Variables|Default|GetPickupable) (Variables|/Game/FirstPerson/Blueprints/BP_FirstPersonCharacter.BP_FirstPersonCharacter_C|GetPickupPosition (Variables|Default|GetPlayerRef)) "None" "SnapToTarget" "SnapToTarget" "KeepWorld" true)
        (Variables|/Game/FirstPerson/Blueprints/BP_FirstPersonCharacter.BP_FirstPersonCharacter_C|SetItemPicked (Variables|Default|GetPlayerRef) self)
        (Variables|/Game/FirstPerson/Blueprints/BP_FirstPersonCharacter.BP_FirstPersonCharacter_C|SetIsHoldingItem (Variables|Default|GetPlayerRef) true)
        (CallFunction|PickupObject)
        (else
          (Development|PrintString "Item is not ready to interact"))))))

(fn ConstructionScript
  (Rendering|SetVisibility (Variables|Default|GetPickupable) (not (Variables|Default|GetHide%20Physic?)) true))