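; BP_BaseCustomer is a base customer actor that tracks whether it is walking and can play a go-home cinematic when it finishes shopping.
; SetState stores the walking flag, while TakeAction is left as an empty event.
; PlayGoHomeSequence creates a player for the finished-shopping Level Sequence, binds this customer into it at runtime, plays it and returns the sequence actor and player.
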(event Custom|Take%20Action)

(event Custom|Set%20State
  (params (Walking? :type Boolean))
  (Variables|Default|SetIsWalking Walking?))

(event EventBeginPlay
  (|CallParentFunction))

(fn ConstructionScript
  (|CallParentFunction))

(fn PlayGoHomeSequence
  (bind (_outactor _returnvalue) (Sequencer|Player|CreateLevelSequencePlayer "/Game/Animation/Anim_CustomerFinishedShopping.Anim_CustomerFinishedShopping"))
  (Class|LevelSequenceActor|AddBinding _outactor (|GetSequenceBinding) self false)
  (Sequencer|Player|Play _returnvalue :!class /Script/MovieScene.MovieSceneSequencePlayer)
  (return _outactor _returnvalue))