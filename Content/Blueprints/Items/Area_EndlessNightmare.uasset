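; Self-replicating level block for the endless nightmare chapter, chaining copies of itself as the player advances.
; One-shot player triggers spawn the next block at the Arrow, enable that block's Wall, and destroy the current block.
; Each triggered spawn passes both blocks to BP_ChapterNightmare's SpawnStuff.
; InitializeNightmare separately spawns a block with its Wall hidden and non-colliding.
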(event OnComponentBeginOverlap(Spawn)
  (params (OverlappedComponent :type Primitive%20Component%20Object%20Reference) (OtherActor :type Actor%20Object%20Reference) (OtherComp :type Primitive%20Component%20Object%20Reference) (OtherBodyIndex :type Integer) (bFromSweep :type Boolean) (SweepResult :type Hit%20Result%20Structure%20%28by%20ref%29))
  (Utilities|Casting|CastToBP_FirstPersonCharacter OtherActor)
  (Utilities|FlowControl|DoOnce false
    (:Completed
      (bind _new_block (CallFunction|SpawnBlock))
      (bind _output_get (Variables|Default|SetNew%20Spawned%20Area _new_block))
      (Default|SpawnStuff (Variables|Default|GetChapterManager) _output_get self)
      (Development|PrintString "Spawn"))))

(event OnComponentBeginOverlap(Destroy)
  (params (OverlappedComponent :type Primitive%20Component%20Object%20Reference) (OtherActor :type Actor%20Object%20Reference) (OtherComp :type Primitive%20Component%20Object%20Reference) (OtherBodyIndex :type Integer) (bFromSweep :type Boolean) (SweepResult :type Hit%20Result%20Structure%20%28by%20ref%29))
  (Utilities|Casting|CastToBP_FirstPersonCharacter OtherActor)
  (Utilities|FlowControl|DoOnce false
    (:Completed
      (Actor|DestroyActor)
      (Development|PrintString "Destroy"))))

(event OnComponentBeginOverlap(WallBuilder)
  (params (OverlappedComponent :type Primitive%20Component%20Object%20Reference) (OtherActor :type Actor%20Object%20Reference) (OtherComp :type Primitive%20Component%20Object%20Reference) (OtherBodyIndex :type Integer) (bFromSweep :type Boolean) (SweepResult :type Hit%20Result%20Structure%20%28by%20ref%29))
  (Utilities|Casting|CastToBP_FirstPersonCharacter OtherActor)
  (Utilities|FlowControl|DoOnce false
    (:Completed
      (bind _new_spawned_area (Variables|Default|GetNew%20Spawned%20Area)
        (:then
          (Rendering|SetVisibility (Variables|Area_EndlessNightmare_C|GetWall _new_spawned_area) true false)
          (Collision|SetCollisionEnabled (Variables|Area_EndlessNightmare_C|GetWall _new_spawned_area) "QueryAndPhysics")
          (Development|PrintString "Wall Built"))
        (:else)))))

(event Custom|Initialize%20Nightmare
  (bind _new_block (CallFunction|SpawnBlock))
  (Rendering|SetVisibility (Variables|Area_EndlessNightmare_C|GetWall _new_block) false true)
  (Collision|SetCollisionEnabled (Variables|Area_EndlessNightmare_C|GetWall _new_block) "NoCollision"))

(event EventBeginPlay
  (bind _returnvalue (Actor|GetActorOfClass "/Game/Blueprints/Chapters/BP_ChapterNightmare.BP_ChapterNightmare_C"))
  (Variables|Default|SetChapterManager _returnvalue))

(fn ConstructionScript)

(fn SpawnBlock
  (bind _returnvalue (Game|SpawnActorfromClass "Area_EndlessNightmare_C" (Transformation|GetWorldTransform (Variables|Default|GetArrow)) "Undefined" "MultiplyWithRoot" 0 (Game|GetPlayerCharacter 0)))
  (return _returnvalue))