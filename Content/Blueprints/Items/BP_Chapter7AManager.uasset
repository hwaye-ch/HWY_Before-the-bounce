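; Chapter 7A manager that runs the chapter's scripted story flow, from bench intro to post-credit jumpscare.
; Initialization prepares props, door, triggers and ambience, then chains fades, dialogue, rain and a player teleport through delegates.
; Counting stored sequences unlocks the window camera event with a mission prompt.
; After credits, Tick watches the player's hit actor to reveal Andy, using a timeline to turn the bench camera toward his head.
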(event OnActionDuringDialogue(BP_DialogueComponent)
  (Utilities|FlowControl|Delay 2.0)
  (CallFunction|PlayThunder))

(event Custom|Initialize%20Chapter%207A
  (bind _bp_fadescreencomponent (Variables|Default|GetBP_FadeScreenComponent))
  (Utilities|FlowControl|Sequence
    (:then_0
      (bind _outactors (Actor|GetAllActorswithTag "mikey"))
      (for _array_element _outactors
        (Rendering|SetActorHiddenInGame _array_element (not (Variables|Default|GetStuff%20Visible?)))
        (if (Actor|ActorHasTag _array_element "lampu")
          (bind _asceiling_lamp (Utilities|Casting|CastToCeilingLamp _array_element))
          (Default|TurntheLight _asceiling_lamp true))))
    (:then_1
      (bind _mikey_s_door (Variables|Default|GetMikey's%20Door)
        (:then
          (Variables|/Game/Blueprints/ModularItems/BP_InteractableDoor.BP_InteractableDoor_C|SetIsLocked _mikey_s_door false)
          (Variables|/Game/Blueprints/EventItems/BP_MikeysDoor.BP_MikeysDoor_C|SetIsIntroChapter7 _mikey_s_door true)
          (Variables|/Game/Blueprints/ModularItems/BP_InteractableDoor.BP_InteractableDoor_C|SetIsLocked _mikey_s_door false)
          (bind _returnvalue (Actor|GetActorOfClass "/Game/Blueprints/Levels/Trigger_StartGoodEnding.Trigger_StartGoodEnding_C"))
          (bind _output_get (Variables|Default|SetTrigger%20Good%20Ending _returnvalue))
          (Default|ActivateOverlapTrigger _output_get)
          (bind _ambience (Variables|Default|GetAmbience)
            (:then
              (Default|SpawnNightAmbience _ambience 0.1))
            (:else)))
        (:else)))
    (:then_2
      (EventDispatchers|BindEventtoStoreSequenceState (delegate Custom|StoreSequenceState_Event)))
    (:then_3
      (bind _trigger_stairs (Variables|Default|GetTrigger%20Stairs)
        (:then
          (Default|ActivateOverlapTrigger _trigger_stairs))
        (:else)))
    (:then_4
      (Default|BlackScreenThenFadein _bp_fadescreencomponent (Variables|Default|GetPlayer%20Ref) 5.0)
      (EventDispatchers|AssignOnFadein _bp_fadescreencomponent (delegate Custom|OnFadeIn_Event)))
    (:then_5
      (bind _bench (Variables|Default|GetBench)
        (:then
          (Default|InitializeLevelCamera (Variables|/Game/Blueprints/EventItems/BP_ParkBench.BP_ParkBench_C|GetBench%20Camera _bench) (Variables|Default|GetPlayer%20Ref) 0.0))
        (:else)))
    (:then_6
      (EventDispatchers|BindEventtoOnChapterFinished (delegate Custom|On%20Chapter%20Finished_Event)))))

(event Custom|Start%20Thunder%20and%20Rain
  (Utilities|FlowControl|Sequence
    (:then_0
      (CallFunction|PlayThunder)
      (Utilities|FlowControl|Delay 1e+01)
      (CallFunction|PlayRain))
    (:then_1
      (Utilities|FlowControl|Delay 10.1)
      (CallFunction|PlayRain))))

(event Custom|Play%20Credit%20Scene
  (bind _returnvalue (UserInterface|CreateWidget "/Game/Blueprints/Widgets/WBP_CreditScene.WBP_CreditScene_C"))
  (UserInterface|Viewport|AddtoViewport _returnvalue 0)
  (UserInterface|Animation|PlayAnimation _returnvalue (Variables|/Game/Blueprints/Widgets/WBP_CreditScene.WBP_CreditScene_C|GetPlayCreditScene _returnvalue) 0.0 1 "Forward" 1.0 false)
  (Class|UserWidget|BindtoAnimationFinished _returnvalue (Variables|/Game/Blueprints/Widgets/WBP_CreditScene.WBP_CreditScene_C|GetPlayCreditScene _returnvalue) (delegate Custom|Play%20Post-credit%20Scene)))

(event Custom|Play%20Rain
  (bind _returnvalue (Actor|GetActorOfClass "/Game/Blueprints/Levels/BP_AmbienceSoundModifier.BP_AmbienceSoundModifier_C"))
  (Variables|/Game/Blueprints/Levels/BP_AmbienceSoundModifier.BP_AmbienceSoundModifier_C|SetIsRaining? _returnvalue true)
  (Default|StartRain _returnvalue)
  (bind _returnvalue_2 (Actor|GetActorOfClass "/Game/EasyRain/Blueprints/BP_EasyRain.BP_EasyRain_C"))
  (Rendering|SetVisibility (Variables|/Game/EasyRain/Blueprints/BP_EasyRain.BP_EasyRain_C|GetrainBP _returnvalue_2) true true))

(event Custom|StoreSequenceState_Event
  (Math|Integer|IncrementInt (Variables|Default|GetSequenceCount)
    (:%20%20
      (Development|PrintString "Sequence Stored")
      (if (== (Variables|Default|GetSequenceCount) (Variables|Default|GetSequenceTotal))
        (Utilities|FlowControl|Delay 3.0)
        (Development|PrintString "Sequences Done! Activate the Window")
        (bind _returnvalue (Actor|GetActorOfClass "/Game/Blueprints/LevelCameras/BP_WindowCamera.BP_WindowCamera_C"))
        (Variables|/Game/Blueprints/LevelCameras/BP_WindowCamera.BP_WindowCamera_C|SetIsEventReady? _returnvalue true)
        (Default|SetCue _returnvalue true)
        (bind _returnvalue_2 (UserInterface|CreateWidget "/Game/Blueprints/Widgets/WBP_Mission.WBP_Mission_C" 0 "Look at the Window"))
        (UserInterface|Viewport|AddtoViewport _returnvalue_2 0)
        (Utilities|FlowControl|Delay 1e+01)
        (Widget|RemovefromParent _returnvalue_2)))))

(event Custom|CustomEvent
  (bind _bp_fadescreencomponent (Variables|Default|GetBP_FadeScreenComponent))
  (EventDispatchers|UnbindEventfromOnDialogueEnded (stale Custom|OnDialogueEnded_Event _dialoguecomponent) (delegate Custom|CustomEvent))
  (Default|FadeEvent _bp_fadescreencomponent 5.0 (Variables|Default|GetPlayer%20Ref) 2.0)
  (EventDispatchers|AssignOnFadeEventFinished _bp_fadescreencomponent (delegate Custom|OnFadeEventFinished_Event)))

(event Custom|Play%20Thunder
  (Audio|SpawnSound2D "/Game/Sounds/sfx_thunder.sfx_thunder" 1.0 1.0 0.0 0))

(event Custom|Play%20Post-credit%20Scene
  (Widget|RemovefromParent (stale Custom|Play%20Credit%20Scene _returnvalue))
  (Default|Fadein (Variables|Default|GetBP_FadeScreenComponent) (Variables|Default|GetPlayer%20Ref))
  (bind _court_bench_camera (Variables|Default|GetCourt%20Bench%20Camera)
    (:then
      (Default|InitializeLevelCamera _court_bench_camera (Variables|Default|GetPlayer%20Ref) 0.0)
      (Collision|SetActorEnableCollision (Variables|Default|GetAndy) false)
      (Default|SetAmbienceVolume (Variables|Default|GetAmbience) 0.2)
      (Utilities|FlowControl|Delay 1.0)
      (Variables|Default|SetIs%20Post%20Credit%20Scene%20Ready? true))
    (:else)))

(event Custom|OnDialogueEnded_Event
  (EventDispatchers|UnbindEventfromOnDialogueEnded (stale Custom|OnFadeIn_Event _dialoguecomponent) (delegate Custom|OnDialogueEnded_Event))
  (Utilities|FlowControl|Delay 1e+01)
  (CallFunction|PlayRain)
  (Utilities|FlowControl|Delay 3.0)
  (bind _dialoguecomponent (Default|ConstructDialogue (Variables|Default|GetBP_DialogueComponent) "ch7_rain" "/Game/Dialogue/Chapter7_Dialogue.Chapter7_Dialogue" true true))
  (Default|ShowDialogue _dialoguecomponent (Variables|Default|GetPlayer%20Ref) self)
  (EventDispatchers|AssignOnDialogueEnded _dialoguecomponent (delegate Custom|CustomEvent)))

(event Custom|On%20Chapter%20Finished_Event
  (Default|BacktoMainMenu (Variables|Default|GetPlayer%20Ref)))

(event Custom|OnFadeEventFinished_Event
  (bind _player_ref (Variables|Default|GetPlayer%20Ref))
  (bind _spawn_area_taman (Variables|Default|GetSpawn%20Area%20Taman)
    (:then
      (Transformation|SetActorLocation _player_ref (Transformation|GetActorLocation _spawn_area_taman) false true)
      (Pawn|SetControlRotation (Game|GetPlayerController 0) (Math|Rotator|FindLookatRotation (Transformation|GetActorLocation _player_ref) (Transformation|GetActorLocation _spawn_area_taman)))
      (Default|EndLevelCamera (Variables|/Game/Blueprints/EventItems/BP_ParkBench.BP_ParkBench_C|GetBench%20Camera (Variables|Default|GetBench))))
    (:else)))

(event Custom|OnFadeIn_Event
  (Utilities|FlowControl|Delay 5.0)
  (bind _dialoguecomponent (Default|ConstructDialogue (Variables|Default|GetBP_DialogueComponent) "ch7_relieve" "/Game/Dialogue/Chapter7_Dialogue.Chapter7_Dialogue" true true))
  (Default|ShowDialogue _dialoguecomponent (Variables|Default|GetPlayer%20Ref) self)
  (EventDispatchers|AssignOnDialogueEnded _dialoguecomponent (delegate Custom|OnDialogueEnded_Event)))

(event EventBeginPlay
  (|CallParentFunction))

(event EventTick
  (params (DeltaSeconds :type Float%20%28single-precision%29))
  (bind _andy (Variables|Default|GetAndy))
  (bind _court_bench_camera (Variables|Default|GetCourt%20Bench%20Camera))
  (bind _camera (Variables|/Game/Blueprints/ModularItems/BP_LevelCamera.BP_LevelCamera_C|GetCamera _court_bench_camera))
  (Variables|Default|GetIs%20Post%20Credit%20Scene%20Ready?
    (:then
      (bind _hit_actor (Variables|/Game/FirstPerson/Blueprints/BP_FirstPersonCharacter.BP_FirstPersonCharacter_C|GetHit%20Actor (Variables|Default|GetPlayer%20Ref))
        (:then
          (if (Actor|ActorHasTag _hit_actor "trigger_andy")
            (Utilities|FlowControl|DoOnce false
              (:Completed
                (Utilities|FlowControl|Delay 1.0)
                (Default|SetLook (Variables|Default|GetCourt%20Bench%20Camera) false)
                (Rendering|SetVisibility (Variables|/Script/Engine.Character|GetMesh (Variables|Default|GetAndy)) true false)
                (Collision|SetActorEnableCollision _andy true)
                (Audio|PlaySound2D "/Game/Sounds/sfx_piano_jumpscare.sfx_piano_jumpscare" 1.0 1.0 0.0 0 0)
                (bind _newtrack_0 (Timeline|Timeline Play)
                  (:Update
                    (Transformation|SetWorldRotation _camera (Math|Rotator|Lerp(Rotator) (Transformation|GetWorldRotation _camera) (Math|Rotator|FindLookatRotation (Transformation|GetWorldLocation _camera) (Transformation|GetSocketLocation (Variables|/Script/Engine.Character|GetMesh _andy) "head")) _newtrack_0) false false))
                  (:Finished
                    (Default|SetLook (Variables|Default|GetCourt%20Bench%20Camera) true)))))))
        (:else)))
    (:else)))

(fn ConstructionScript)