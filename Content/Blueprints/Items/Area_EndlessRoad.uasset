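; Road segment actor that builds an endless road for the BP_BusMoveEndlessly bus by spawning copies of itself.
; PlayEvent sets IsMoving, spawns the next segment and calls Execute on the bus found at BeginPlay.
; The bus overlapping Spawner also triggers spawning, limited by DoOnce to one segment and positioned by a collapsed graph.
; The bus overlapping Destroyer removes the current segment.
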(event OnComponentBeginOverlap(Spawner)
  (params (OverlappedComponent :type Primitive%20Component%20Object%20Reference) (OtherActor :type Actor%20Object%20Reference) (OtherComp :type Primitive%20Component%20Object%20Reference) (OtherBodyIndex :type Integer) (bFromSweep :type Boolean) (SweepResult :type Hit%20Result%20Structure%20%28by%20ref%29))
  (if (== OtherActor (Variables|Default|GetBus))
    (CallFunction|SpawnRoad)))

(event OnComponentBeginOverlap(Destroyer)
  (params (OverlappedComponent :type Primitive%20Component%20Object%20Reference) (OtherActor :type Actor%20Object%20Reference) (OtherComp :type Primitive%20Component%20Object%20Reference) (OtherBodyIndex :type Integer) (bFromSweep :type Boolean) (SweepResult :type Hit%20Result%20Structure%20%28by%20ref%29))
  (if (== OtherActor (Variables|Default|GetBus))
    (Actor|DestroyActor)
    (Development|PrintString "Destroy Road")))

(event Custom|Spawn%20Road
  (bind (_returnvalue _rotation) (|CollapseGraph))
  (Utilities|FlowControl|DoOnce false
    (:Completed
      (Game|SpawnActorfromClass "Area_EndlessRoad_C" (Math|Transform|MakeTransform _returnvalue _rotation "1.000000,1.000000,1.000000") "Undefined" "MultiplyWithRoot" 0 0)
      (Development|PrintString "Spawn New Road"))))

(event Custom|Play%20Event
  (Variables|Default|SetIsMoving true)
  (CallFunction|SpawnRoad)
  (bind _bus (Variables|Default|GetBus)
    (:then
      (Default|Execute _bus))
    (:else)))

(event EventBeginPlay
  (|CallParentFunction)
  (bind _returnvalue (Actor|GetActorOfClass "/Game/Blueprints/EventItems/BP_BusMoveEndlessly.BP_BusMoveEndlessly_C"))
  (Variables|Default|SetBus _returnvalue))

(fn ConstructionScript
  (|CallParentFunction))