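; BP_Mikey_Sick is the Mikey character, a talkable NPC whose appearance changes by chapter.
; Chapter setup events swap mesh and anim Blueprint and show him, with chapter 2 adding a crutch and building his dialogue from a data table.
; TalkwithObject starts that dialogue when a code is set.
; Dialogue handlers toggle idle/talk, and ending also unblocks a barrier, though it calls the parent's Started handler instead of Ended.
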(event Custom|Setup%20event%20for%20chapter%202
  (Default|ConstructDialogue (Variables|Default|GetBP_DialogueComponent) "ch2_ryan1" "/Game/Dialogue/Chapter2_Dialogue.Chapter2_Dialogue" true true)
  (Components|SkeletalMesh|SetSkeletalMeshAsset (Variables|Character|GetMesh) "/Game/Objects/Mikey/MikeySick/Mikey_sick.Mikey_sick")
  (Components|SkeletalMesh|SetAnimInstanceClass (Variables|Character|GetMesh) "/Game/Blueprints/Characters/ABP_MikeySick.ABP_MikeySick_C")
  (CallFunction|SetMikeyVisibility true)
  (Rendering|SetVisibility (Variables|Default|GetCrutch) true false))

(event Custom|Setup%20event%20for%20chapter%201
  (Components|SkeletalMesh|SetSkeletalMeshAsset (Variables|Character|GetMesh) "/Game/Objects/Mikey/Michael.Michael")
  (Components|SkeletalMesh|SetAnimInstanceClass (Variables|Character|GetMesh) "/Game/Blueprints/Characters/ABP_Mikey.ABP_Mikey_C")
  (CallFunction|SetMikeyVisibility true))

(event Custom|Set%20Mikey%20Visibility
  (params (Visible? :type Boolean))
  (Rendering|SetVisibility (Variables|Character|GetMesh) Visible? false))

(event EventBeginPlay
  (|CallParentFunction))

(event EventHandleDialogueStarted
  (|CallParentFunction)
  (Development|PrintString "Start Dialogue wih Mikey")
  (Default|CallToggleIdleandTalk true))

(event EventHandleDialogueEnded
  (|CallParentFunction)
  (Development|PrintString "End Dialogue with Mikey")
  (Default|CallUnblockBarrier)
  (Default|CallToggleIdleandTalk false))

(event EventTalkwithObject
  (bind _bp_dialoguecomponent (Variables|Default|GetBP_DialogueComponent))
  (if (!= (Variables|/Game/Blueprints/Components/BP_DialogueComponent.BP_DialogueComponent_C|GetDialogueCode (Variables|Default|GetBP_DialogueComponent)) "")
    (Default|CallOnDialogStarted _bp_dialoguecomponent)
    (Class|BPIDialogue|ShowDialogue(Message) _bp_dialoguecomponent (Variables|Default|GetPlayerRef) self)))

(fn ConstructionScript
  (|CallParentFunction))