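; Janitor NPC that catches the player in a scripted Chapter 3 scene and also carries a Chapter 1 greeting.
; An Enabler's events move it to a spawn-area actor behind the player or start the encounter, which freezes the player, shows dialogue and triggers laptop activation.
; Dialogue start and end handlers toggle idle/talk, with the end handler also firing a delayed, one-time after-caught monologue.
; Helper events set mesh visibility and relocation.
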(event Custom|Move%20Janitor%20Behind%20Player
  (bind _returnvalue (Actor|GetActorOfClass "/Game/Blueprints/Levels/SpawnArea_Janitor208.SpawnArea_Janitor208_C"))
  (CallFunction|MoveJanitortoASpawnArea _returnvalue))

(event Custom|Interact%20With%20Janitor
  (params (Player%20Pref :type BP%20First%20Person%20Character%20Object%20Reference))
  (bind _bp_dialoguecomponent (Variables|Default|GetBP_DialogueComponent))
  (Variables|Default|SetPlayer%20Pref Player%20Pref)
  (Default|DisableMovementandLook (Variables|Default|GetPlayer%20Pref))
  (Utilities|FlowControl|Delay 3.0)
  (Default|CallOnDialogStarted _bp_dialoguecomponent)
  (bind _dialoguecomponent (Default|ConstructDialogue _bp_dialoguecomponent "ch3_janiryan1" "/Game/Dialogue/Chapter3_Dialogue.Chapter3_Dialogue" true true))
  (Default|ShowDialogue _dialoguecomponent (Variables|Default|GetPlayer%20Pref) self)
  (Default|CallActivateLaptop)
  (Variables|Default|SetAfterCaught? true))

(event Custom|Set%20default%20action%20for%20Janitor
  (Default|ConstructDialogue (Variables|Default|GetBP_DialogueComponent) "ch1_janitor_greeting" "/Game/Dialogue/Chapter1_Dialogue.Chapter1_Dialogue" false false)
  (CallFunction|SetJanitorVisibility true))

(event Custom|Set%20Janitor%20Visibility
  (params (Visible? :type Boolean))
  (Rendering|SetVisibility (Variables|Character|GetMesh) Visible? false))

(event EventTalkwithObject)

(event EventHandleDialogueStarted
  (|CallParentFunction)
  (Development|PrintString "Start Dialogue wih Janitor")
  (Default|CallToggleIdleandTalk true))

(event EventHandleDialogueEnded
  (|CallParentFunction)
  (Development|PrintString "End Dialogue with Janitor")
  (Default|CallToggleIdleandTalk false)
  (Variables|Default|GetAfterCaught?
    (:then
      (Utilities|FlowControl|DoOnce false
        (:Completed
          (Utilities|FlowControl|Delay 3.0)
          (bind _returnvalue (Actor|GetActorOfClass "/Game/Blueprints/Levels/Monologue_AfterPeekingMichaelsRoom.Monologue_AfterPeekingMichaelsRoom_C"))
          (Default|DisplayDialogueAfterBeingCaughtbyJanitor _returnvalue))))
    (:else)))

(event EventBeginPlay
  (bind _enabler (Variables|Default|GetEnabler))
  (|CallParentFunction)
  (Utilities|IsValid _enabler
    (:Is%20Valid
      (EventDispatchers|BindEventtoMoveJanitor _enabler (delegate Custom|Move%20Janitor%20Behind%20Player))
      (EventDispatchers|BindEventtoTalktoJanitor _enabler (delegate Custom|Interact%20With%20Janitor)))))

(event Custom|Move%20Janitor%20to%20a%20spawn%20area
  (params (SpawnLocation :type BP%20Spawn%20Location%20Object%20Reference))
  (bind _returnvalue (Transformation|GetActorTransform SpawnLocation))
  (Transformation|SetActorLocationAndRotation (.location _returnvalue) (.rotation _returnvalue)))

(fn ConstructionScript
  (|CallParentFunction))